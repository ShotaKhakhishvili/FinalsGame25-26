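; BP_CombatNPC is a combat NPC that starts with a preset skill loadout and can choose abilities at random by weight.
; On BeginPlay it feeds its ability tree component points, then unlocks a base skill and two elementals, each with its own set of skill nodes.
; FRandomAbilityIndex sums the Abilities weights, rolls within that total and returns the entry where the running sum reaches the roll, falling back to the last.
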(event EventBeginPlay
  (bind _ac_abilitytree (Variables|Default|GetAC_AbilityTree))
  (bind _ac_abilitytree_2 (Variables|Default|GetAC_AbilityTree))
  (bind _ac_abilitytree_3 (Variables|Default|GetAC_AbilityTree))
  (Utilities|FlowControl|Sequence
    (:then_0
      (Default|AddAbilityPoint _ac_abilitytree_3 10)
      (Default|UnlockNode _ac_abilitytree_3 "/Game/ThirdPerson/Ability/Tree/DA_Skill_D1.DA_Skill_D1"))
    (:then_1
      (Default|UnlockElemental _ac_abilitytree "NewEnumerator0")
      (Default|UnlockNode _ac_abilitytree "/Game/ThirdPerson/Ability/Tree/DA_Skill_F1.DA_Skill_F1")
      (Default|UnlockNode _ac_abilitytree "/Game/ThirdPerson/Ability/Tree/DA_Skill_F2.DA_Skill_F2")
      (Default|UnlockNode _ac_abilitytree "/Game/ThirdPerson/Ability/Tree/DA_Skill_F3.DA_Skill_F3")
      (Default|UnlockNode _ac_abilitytree "/Game/ThirdPerson/Ability/Tree/DA_Skill_F4.DA_Skill_F4"))
    (:then_2
      (Default|UnlockElemental _ac_abilitytree_2 "NewEnumerator1")
      (Default|UnlockNode _ac_abilitytree_2 "/Game/ThirdPerson/Ability/Tree/DA_Skill_E1.DA_Skill_E1")
      (Default|UnlockNode _ac_abilitytree_2 "/Game/ThirdPerson/Ability/Tree/DA_Skill_E2.DA_Skill_E2")
      (Default|UnlockNode _ac_abilitytree_2 "/Game/ThirdPerson/Ability/Tree/DA_Skill_E3.DA_Skill_E3")
      (Default|UnlockNode _ac_abilitytree_2 "/Game/ThirdPerson/Ability/Tree/DA_Skill_E4.DA_Skill_E4"))))

(event Collision|EventActorBeginOverlap
  (params (OtherActor :type Actor%20Object%20Reference)))

(event EventTick
  (params (DeltaSeconds :type Float%20%28single-precision%29)))

(fn ConstructionScript
  (|CallParentFunction))

(fn FRandomAbilityIndex
  (bind _abilities (Variables|Default|GetAbilities))
  (bind _returnvalue (Utilities|Array|LastIndex _abilities))
  (for _array_element (Variables|Default|GetAbilities)
    (LocalVariables|SetTotalWeights (+ (LocalVariables|GetTotalWeights) (.Weight (Utilities|Struct|BreakS_NPCAbilityData _array_element)))))
  (LocalVariables|SetRandomFloat (Math|Random|RandomFloatinRange 0.0 (LocalVariables|GetTotalWeights)))
  (for (_array_element_2 _array_index) (Variables|Default|GetAbilities)
    (bind _output_get (LocalVariables|SetAcc (+ (LocalVariables|GetAcc) (.Weight (Utilities|Struct|BreakS_NPCAbilityData _array_element_2)))))
    (if (>= _output_get (LocalVariables|GetRandomFloat))
      (return _array_index _array_element_2)))
  (return _returnvalue (Utilities|Array|Get(acopy) _abilities _returnvalue)))