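; AI controller for combat NPCs that runs their behavior tree and drives ability-based attacks on the player.
; A looping timer picks a random ability when distance leaves its switch range or repeat uses max out, otherwise executes it off cooldown.
; Execution halts movement through the blackboard until a delayed cleanup after ability end.
; Perception updates player blackboard keys, with a Tick countdown ending the chase after sight is lost.
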(event OnTargetPerceptionUpdated(AIPerception)
  (params (Actor :type Actor%20Object%20Reference) (Stimulus :type AI%20Stimulus%20Structure))
  ;[0 0 0 0.5] Perception Update For Player
  ;;[0.15 0.15 0.15 0.5] Checking If Its Really The Player And The Sight Condition For It
  (if (== Actor (Variables|Default|GetPlayerCharacter))
    (if (.bSuccessfullySensed (Utilities|Struct|BreakAIStimulus Stimulus))
      ;;[0.15 0.15 0.15 0.5] If Player Just Got Seen
      (AI|Components|Blackboard|SetValueasObject (AI|GetBlackboard 0) (Utilities|Name|MakeLiteralName "Player") (Variables|Default|GetPlayerCharacter))
      (Variables|Default|SetPlayerInvestigationTIme_Left (Variables|Default|GetPlayerInvestigationTIme))
      (Variables|Default|SetPlayesSeen true)
      (AI|Components|Blackboard|SetValueasBool (AI|GetBlackboard 0) (Utilities|Name|MakeLiteralName "ShouldChasePlayer") true)
      (else
        ;;[0.15 0.15 0.15 0.5] If Player Is Not Seen Anymore
        (AI|Components|Blackboard|SetValueasObject (AI|GetBlackboard 0) (Utilities|Name|MakeLiteralName "Player") 0)
        ;;;[0.15 0.15 0.15 0.5] Get Ready For The Investigation part
        (AI|Components|Blackboard|SetValueasVector (AI|GetBlackboard 0) (Utilities|Name|MakeLiteralName "LastPlayerPos") (Transformation|GetActorLocation (Variables|Default|GetPlayerCharacter)))
        (Variables|Default|SetPlayesSeen false)))))

(event Custom|AbilityUpdate
  (bind _pawnlocation (CallFunction|FGetPawnLocation))
  (bind _currabilitydata (Variables|Default|GetCurrAbilityData))
  (bind _playercharacter (Variables|Default|GetPlayerCharacter))
  (bind (_switchoutrange_min _switchoutrange_max) (Utilities|Struct|BreakS_NPCAbilityData _currabilitydata))
  (bind _returnvalue (Transformation|GetActorLocation _playercharacter))
  (bind _returnvalue_2 (+ _pawnlocation "0.000000,0.000000,50.000000"))
  (bind _returnvalue_3 (+ _returnvalue "0.000000,0.000000,50.000000"))
  ;[0 0 0 0.5] Refreshing The Ability Behaviour Every 0.1 Seconds
  ;;[0.15 0.15 0.15 0.5] Check If We Need To Switch An Ability
  (if (or (< (CallFunction|FDisttoPlayer) _switchoutrange_min) (> (CallFunction|FDisttoPlayer) _switchoutrange_max))
    (CallFunction|FSwitchAbility)
    (else
      ;;[0.15 0.15 0.15 0.5] If Ability Stays The Same, Check The Cooldown
      (bind _passed (Default|CheckCooldown (Variables|/Game/ThirdPerson/Blueprints/BP_BaseCharacter.BP_BaseCharacter_C|GetAC_AbilitySystem (Variables|Default|GetControlledPawn)) (Variables|Default|GetCurrAbility)))
      (Development|PrintString (Utilities|String|ToString(Boolean) _passed))
      (if _passed
        ;;[0.15 0.15 0.15 0.5] If Cooldown Is Fine, Trace By Channel And Spawn THe Ability To Execute It
        (bind _outhit (Collision|LineTraceByChannel _returnvalue_2 _returnvalue_3 "TraceTypeQuery1" false 0 "None"))
        (bind _returnvalue_4 (Game|SpawnActorfromClass (Variables|/Game/ThirdPerson/Ability/Abilities/PDA_SpecialAbility.PDA_SpecialAbility_C|GetLogicClass (Variables|Default|GetCurrAbility)) (CallFunction|FGetPawnTransform) "Undefined" "MultiplyWithRoot" 0 (Variables|Default|GetCurrAbility) 0))
        (bind _output_get (Variables|Default|SetCurrAbiltyLogic _returnvalue_4))
        (Default|ExecuteAbility (Variables|/Game/ThirdPerson/Blueprints/BP_BaseCharacter.BP_BaseCharacter_C|GetAC_AbilitySystem (Variables|Default|GetControlledPawn)) (Variables|Default|GetCurrAbility) _output_get _outhit (Math|Vector|Normalize (- _returnvalue_3 _returnvalue_2)))
        ;;[0.15 0.15 0.15 0.5] Stop Any Walking Movement
        (Utilities|MSetShouldMove false)
        ;;[0.15 0.15 0.15 0.5] Check For The Consequtive Executions. If Reaches Its Limit, We Switch The Ability
        (bind _result (Math|Integer|IncrementInt (Variables|Default|GetConsequtiveExec))
          (:%20%20
            (if (>= _result (.MaxConsequtiveUse (Utilities|Struct|BreakS_NPCAbilityData (Variables|Default|GetCurrAbilityData))))
              (CallFunction|FSwitchAbility))))))))

(event Custom|OnAbilityEnd_Event
  ;[0.15 0.15 0.15 0.5] Destroying The Ability Logic Actor And Accessing Movement When The Ability Ends
  (Utilities|FlowControl|Delay 4.0)
  (bind _currabiltylogic (Variables|Default|GetCurrAbiltyLogic)
    (:then
      (Actor|DestroyActor _currabiltylogic)
      (Utilities|MSetShouldMove true))
    (:else)))

(event EventBeginPlay
  ;[0 0 0 0.5] Initializations, Bindings
  (bind _asbp_base_character (Utilities|Casting|CastToBP_BaseCharacter (Game|Player|GetPlayerPawn 0)))
  (Variables|Default|SetPlayerCharacter _asbp_base_character)
  (bind _asbp_combat_npc (Utilities|Casting|CastToBP_CombatNPC (Pawn|GetControlledPawn)))
  (Variables|Default|SetControlledPawn _asbp_combat_npc)
  (Utilities|Time|SetTimerbyEvent (delegate Custom|AbilityUpdate) 0.1 true)
  (EventDispatchers|AssignOnAbilityEnd (Variables|/Game/ThirdPerson/Blueprints/BP_BaseCharacter.BP_BaseCharacter_C|GetAC_AbilitySystem (Variables|Default|GetControlledPawn)) (delegate Custom|OnAbilityEnd_Event))
  (AI|RunBehaviorTree "/Game/Shota/Blueprints/NPCs/BT_CombatNPC.BT_CombatNPC")
  (Utilities|MSetShouldMove true)
  (Utilities|FlowControl|DelayUntilNextTick)
  (Default|ChangeElement (Variables|/Game/ThirdPerson/Blueprints/BP_BaseCharacter.BP_BaseCharacter_C|GetAC_AbilitySystem (Variables|Default|GetControlledPawn)) "NewEnumerator0")
  (CallFunction|FSwitchAbility))

(event EventTick
  (params (DeltaSeconds :type Float%20%28single-precision%29))
  ;[0 0 0 0.5] Update The Countdown Of Player Not Being Seen On Each Tick. If It Reaches Zero, The NPC Should Stop Looking For The Player.
  (if (not (Variables|Default|GetPlayesSeen))
    (bind _output_get (Variables|Default|SetPlayerInvestigationTIme_Left (- (Variables|Default|GetPlayerInvestigationTIme_Left) DeltaSeconds)))
    (if (<= _output_get 0.0)
      (AI|Components|Blackboard|SetValueasBool (AI|GetBlackboard 0) (Utilities|Name|MakeLiteralName "ShouldChasePlayer") false))))

(fn ConstructionScript)

(fn FDisttoPlayer
  (return (Math|Vector|Distance(Vector) (CallFunction|FGetPawnLocation) (Transformation|GetActorLocation (Variables|Default|GetPlayerCharacter)))))

(fn FSwitchAbility
  (bind _controlledpawn (Variables|Default|GetControlledPawn))
  (bind _ac_abilitysystem (Variables|/Game/ThirdPerson/Blueprints/BP_BaseCharacter.BP_BaseCharacter_C|GetAC_AbilitySystem _controlledpawn))
  (bind (_defaultability _abilitydata) (Default|FGetRandomAbility _ac_abilitysystem))
  (Development|PrintString (Utilities|String|Append (Utilities|GetDisplayName _defaultability) "ads"))
  (Variables|Default|SetCurrAbility _defaultability)
  (Variables|Default|SetCurrAbilityData _abilitydata)
  (Variables|Default|SetConsequtiveExec 0)
  (AI|Components|Blackboard|SetValueasFloat (AI|GetBlackboard 0) (Utilities|Name|MakeLiteralName "AttackAcceptableRange") (Utilities|Struct|BreakS_NPCAbilityData (Variables|Default|GetCurrAbilityData)))
  (return))

(fn FGetPawnLocation
  (return (Transformation|GetActorLocation (Variables|Default|GetControlledPawn))))

(fn FGetPawnTransform
  (return (Transformation|GetActorTransform (Variables|Default|GetControlledPawn))))