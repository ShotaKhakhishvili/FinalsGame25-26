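; Base arrow projectile that launches with charge-scaled speed and gravity, with effects and sounds chosen by element and overcharge state.
; Shoot adds a ProjectileMovementComponent at runtime and attaches a trail.
; The first overlap with a non-instigator destroys that component, reports the hit and plays impact effects.
; Arrows hide on characters and attach to other surfaces, pushing and staggering staggerable characters or nudging physics bodies.
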(event OnComponentBeginOverlap(Collider)
  (params (OverlappedComponent :type Primitive%20Component%20Object%20Reference) (OtherActor :type Actor%20Object%20Reference) (OtherComp :type Primitive%20Component%20Object%20Reference) (OtherBodyIndex :type Integer) (bFromSweep :type Boolean) (SweepResult :type Hit%20Result%20Structure%20%28by%20ref%29))
  (if (and (!= OtherActor (Game|GetInstigator)) (not (Variables|Default|GetIsHit)))
    (bind _projectilemovementcomponent (Variables|Default|GetProjectileMovementComponent)
      (:then
        (Components|DestroyComponent _projectilemovementcomponent)
        (Collision|SetCollisionEnabled (Variables|Default|GetCollider) "NoCollision")
        (CallFunction|AttachArrow SweepResult)
        (Variables|Default|SetIsHit true)
        (Default|CallOnHit SweepResult self (Variables|Default|GetChargeLevel) (Variables|Default|GetDirection) (Variables|Default|GetElemental))
        (CallFunction|ApplyHitForce SweepResult)
        (CallFunction|AttachEffect (.HitEffect (Utilities|GetVfx)))
        (Utilities|FlowControl|Delay 0.25)
        (bind _traileffectref (Variables|Default|GetTrailEffectRef)
          (:then
            (Components|Activation|Deactivate _traileffectref)
            (Utilities|FlowControl|Delay 0.5)
            (Components|DestroyComponent _traileffectref))
          (:else)))
      (:else))))

(event Custom|Shoot
  (params (Direction :type Vector) (Strength :type Float%20%28double-precision%29))
  (bind _output_get (Variables|Default|SetChargeLevel Strength))
  (CallFunction|DoShoot Direction _output_get)
  (bind _resulteffect (CallFunction|AttachEffect (.TrailEffect (Utilities|GetVfx))))
  (Variables|Default|SetTrailEffectRef _resulteffect)
  (Collision|SetCollisionEnabled (Variables|Default|GetCollider) "QueryAndPhysics")
  (Utilities|FlowControl|Delay 0.2)
  (CallFunction|DisableMainEffect))

(event Custom|ApplyHitForce
  (params (HitResult :type Hit%20Result%20Structure))
  (bind (_bblockinghit _binitialoverlap _time _distance _location _impactpoint _normal _impactnormal _physmat _hitactor _hitcomponent) (Collision|BreakHitResult HitResult))
  (bind _velocity (Variables|Default|GetVelocity))
  (bind _returnvalue (/ _velocity 16))
  (bind _asbp_base_character (Utilities|Casting|CastToBP_BaseCharacter _hitactor)
    (:then
      (if (Variables|/Game/Saba/Blueprints/Characters/BP_BaseCharacter.BP_BaseCharacter_C|GetCanStagger _asbp_base_character)
        (Physics|AddImpulse (Variables|/Script/Engine.Character|GetCharacterMovement _asbp_base_character) _returnvalue true)
        (Utilities|FlowControl|Delay 0.1)
        (Default|Stagger _asbp_base_character (Math|Vector|NegateVector _returnvalue))))
    (:CastFailed
      (if (Physics|IsSimulatingPhysics _hitcomponent "None")
        (Physics|AddImpulse _hitcomponent _returnvalue "None" true)))))

(event Custom|AttachArrow
  (params (HitResult :type Hit%20Result%20Structure))
  (bind (_bblockinghit _binitialoverlap _time _distance _location _impactpoint _normal _impactnormal _physmat _hitactor _hitcomponent) (Collision|BreakHitResult HitResult))
  (Utilities|IsValid _hitactor
    (:Is%20Valid
      (Utilities|Casting|CastToBP_BaseCharacter _hitactor
        (:then
          (Development|SetHiddeninGame (Variables|Default|GetStaticMesh) true true))
        (:CastFailed
          (Transformation|AttachComponentToComponent _hitcomponent "None" "KeepWorld" "KeepWorld" "KeepWorld" true :!label _label))))
    (:Is%20Not%20Valid
      (goto _label))))

(event Custom|PlayHitSound
  (params (HitResult :type Hit%20Result%20Structure) (Weapon :type BP%20Weapon%20Object%20Reference) (Charge :type Float%20%28double-precision%29) (Direction :type Vector) (Elemental :type E_ElementalType%20Enum :default "NewEnumerator0"))
  (bind (_bblockinghit _binitialoverlap _time _distance _location _impactpoint _normal _impactnormal _physmat _hitactor) (Collision|BreakHitResult HitResult))
  (bind _shootsfx_ref (Variables|Default|GetShootSfx%20Ref)
    (:then
      (Audio|Components|Audio|FadeOut _shootsfx_ref 0.1 0.0 "Linear" :!class /Script/Engine.AudioComponent)
      (Audio|Components|Audio|StopDelayed _shootsfx_ref 0.1)
      (Utilities|Casting|CastToBP_BaseCharacter _hitactor
        (:then
          (Audio|PlaySoundatLocation (.HitSfx (Utilities|GetSfx)) _location "0, 0, 0" 1.0 1.0 0.0 "/Game/Saba/SFX/AbilityAttenuation.AbilityAttenuation" 0 0 0))
        (:CastFailed
          (Audio|PlaySoundatLocation (Variables|Default|GetDefaultHitSfx) _location "0, 0, 0" 1.0 1.0 0.0 "/Game/Saba/SFX/AbilityAttenuation.AbilityAttenuation" 0 0 0))))
    (:else)))

(event EventBeginPlay
  (Collision|SetCollisionEnabled (Variables|Default|GetCollider) "NoCollision")
  (CallFunction|UpdateMainEffect)
  (EventDispatchers|BindEventtoOnHit (delegate Custom|PlayHitSound)))

(event EventWeaponCharged
  (params (Chraged :type Boolean))
  (|CallParentFunction Chraged)
  (if (Variables|Default|GetIsOvercharge)
    (CallFunction|UpdateMainEffect)))

(event EventChangeElement
  (params (ElementType :type E_ElementalType%20Enum :default "NewEnumerator0"))
  (|CallParentFunction ElementType)
  (CallFunction|UpdateMainEffect))

(fn ConstructionScript)

(fn DoShoot
  (params (Direction :type Vector) (Strength :type Float%20%28double-precision%29))
  (bind _output_get (Variables|Default|SetDirection Direction))
  (bind _returnvalue (AddComponent|AddProjectileMovementComponent))
  (bind _output_get_2 (Variables|Default|SetProjectileMovementComponent _returnvalue))
  (bind _output_get_3 (Variables|/Script/Engine.MovementComponent|SetVelocity _output_get_2 (* _output_get (Math|Float|Lerp (Variables|Default|GetMinSpeed) (Variables|Default|GetMaxSpeed) Strength))))
  (Variables|Default|SetVelocity _output_get_3)
  (Variables|/Script/Engine.ProjectileMovementComponent|SetProjectileGravityScale _output_get_2 (Math|Float|Lerp (Variables|Default|GetMaxGravityScale) (Variables|Default|GetMinGravityScale) Strength))
  (Actor|SetLifeSpan 15.0)
  (bind _returnvalue_2 (Audio|SpawnSoundAttached (Variables|Default|GetShootSfx) (Variables|Default|GetEffectLocation) "None" "0, 0, 0" "0, 0, 0" "KeepRelativeOffset" true 1.0 1.0 0.0 "/Game/Saba/SFX/AbilityAttenuation.AbilityAttenuation" 0))
  (Variables|Default|SetShootSfx%20Ref _returnvalue_2))

(fn UpdateMainEffect
  (CallFunction|DisableMainEffect)
  (bind _resulteffect (CallFunction|AttachEffect (.MainEffect (Utilities|GetVfx))))
  (Variables|Default|SetMainEffectRef _resulteffect)
  (bind _returnvalue (Audio|SpawnSoundAttached (.MainSfx (Utilities|GetSfx)) (Variables|Default|GetEffectLocation) "None" "0, 0, 0" "0, 0, 0" "KeepRelativeOffset" true 1.0 1.0 0.0 "/Game/Saba/SFX/AbilityAttenuation.AbilityAttenuation" 0))
  (Utilities|IsValid _returnvalue
    (:Is%20Valid
      (bind _output_get (Variables|Default|SetMainSfx%20Ref _returnvalue))
      (Audio|Components|Audio|FadeIn _output_get 0.25 1.0 0.0 "Linear" :!class /Script/Engine.AudioComponent))))

(fn DisableMainEffect
  (bind _maineffectref (Variables|Default|GetMainEffectRef)
    (:then
      (Components|Activation|Deactivate _maineffectref))
    (:else
      _))
  (bind _mainsfx_ref (Variables|Default|GetMainSfx%20Ref)
    (:then
      (Audio|Components|Audio|FadeOut _mainsfx_ref 0.5 0.0 "Linear" :!class /Script/Engine.AudioComponent)
      (Audio|Components|Audio|StopDelayed _mainsfx_ref 0.5)
      (Variables|Default|SetMainEffectRef 0))
    (:else)))

(fn AttachEffect
  (params (Effect :type Niagara%20System%20Object%20Reference))
  (bind _returnvalue (Niagara|SpawnSystemAttached Effect (Variables|Default|GetEffectLocation) "None" "0, 0, 0" "0, 0, 0" "KeepRelativeOffset" false))
  (Utilities|IsValid _returnvalue
    (:Is%20Valid
      (Class|NiagaraComponent|SetAutoDestroy _returnvalue true))
    (:Is%20Not%20Valid
      _))
  (return _returnvalue))