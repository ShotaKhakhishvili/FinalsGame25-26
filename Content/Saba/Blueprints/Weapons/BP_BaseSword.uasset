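; Base sword weapon Blueprint with elemental and overcharge-dependent VFX and SFX for its blade, swing trail and hits.
; Collider overlaps skip the instigator, cap hits per actor until collision is disabled, then broadcast OnHit with charge, direction and element.
; Hits push and stagger characters that allow it or impulse physics objects, then fade the trail.
; Element changes and overcharging rebuild the main effect; GetSwordMainMesh returns nothing here, presumably for child overrides.
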(event OnComponentBeginOverlap(Collider)
  (params (OverlappedComponent :type Primitive%20Component%20Object%20Reference) (OtherActor :type Actor%20Object%20Reference) (OtherComp :type Primitive%20Component%20Object%20Reference) (OtherBodyIndex :type Integer) (bFromSweep :type Boolean) (SweepResult :type Hit%20Result%20Structure%20%28by%20ref%29))
  (bind _result (CallFunction|TryHitActor OtherActor))
  (if _result
    (bind _direction (CallFunction|CalculateAttackDirection OtherActor))
    (Default|CallOnHit SweepResult self (Variables|Default|GetChargeLevel) _direction (Variables|Default|GetElemental))
    (CallFunction|ApplyHitForce SweepResult _direction)
    (CallFunction|AttachHitEffect (.HitEffect (Utilities|GetVfx)))
    (Utilities|FlowControl|Delay 0.25)
    (bind _traileffectref (Variables|Default|GetTrailEffectRef)
      (:then
        (Components|Activation|Deactivate _traileffectref)
        (Utilities|FlowControl|Delay 0.5)
        (bind _traileffectref_2 (Variables|Default|GetTrailEffectRef)
          (:then
            (Components|DestroyComponent _traileffectref_2))
          (:else)))
      (:else))))

(event Custom|Attack
  (params (Strength :type Float%20%28double-precision%29))
  (Variables|Default|SetChargeLevel Strength)
  (bind _resulteffect (CallFunction|AttachTrailEffect (.TrailEffect (Utilities|GetVfx))))
  (Variables|Default|SetTrailEffectRef _resulteffect))

(event Custom|ApplyHitForce
  (params (HitResult :type Hit%20Result%20Structure) (Direction :type Vector))
  (bind (_bblockinghit _binitialoverlap _time _distance _location _impactpoint _normal _impactnormal _physmat _hitactor _hitcomponent) (Collision|BreakHitResult HitResult))
  (bind _staggerpower (Variables|Default|GetStaggerPower))
  (bind _returnvalue (* Direction _staggerpower))
  (Utilities|IsValid _hitactor
    (:Is%20Valid
      (bind _asbp_base_character (Utilities|Casting|CastToBP_BaseCharacter _hitactor)
        (:then
          (if (Variables|/Game/Saba/Blueprints/Characters/BP_BaseCharacter.BP_BaseCharacter_C|GetCanStagger _asbp_base_character)
            (Physics|AddImpulse (Variables|/Script/Engine.Character|GetCharacterMovement _asbp_base_character) _returnvalue true)
            (Utilities|FlowControl|Delay 0.1)
            (Default|Stagger _asbp_base_character (Math|Vector|NegateVector Direction))))
        (:CastFailed
          (if (Physics|IsSimulatingPhysics _hitcomponent "None") :!label _label
            (Physics|AddImpulse _hitcomponent _returnvalue "None" true)))))
    (:Is%20Not%20Valid
      (goto _label))))

(event Custom|PlayHitSound
  (params (HitResult :type Hit%20Result%20Structure) (Weapon :type BP%20Weapon%20Object%20Reference) (Charge :type Float%20%28double-precision%29) (Direction :type Vector) (Elemental :type E_ElementalType%20Enum :default "NewEnumerator0"))
  (bind (_bblockinghit _binitialoverlap _time _distance _location _impactpoint _normal _impactnormal _physmat _hitactor) (Collision|BreakHitResult HitResult))
  (Utilities|Casting|CastToBP_BaseCharacter _hitactor
    (:then
      (Audio|PlaySoundatLocation (.HitSfx (Utilities|GetSfx)) _location "0, 0, 0" 1.0 1.0 0.0 "/Game/Saba/SFX/AbilityAttenuation.AbilityAttenuation" 0 0 0))
    (:CastFailed
      (Audio|PlaySoundatLocation (Variables|Default|GetDefaultHitSfx) _location "0, 0, 0" 1.0 1.0 0.0 "/Game/Saba/SFX/AbilityAttenuation.AbilityAttenuation" 0 0 0))))

(event EventBeginPlay
  (CallFunction|UpdateMainEffect)
  (EventDispatchers|BindEventtoOnHit (delegate Custom|PlayHitSound)))

(event EventWeaponCharged
  (params (Chraged :type Boolean))
  (|CallParentFunction Chraged)
  (if (Variables|Default|GetIsOvercharge)
    (CallFunction|UpdateMainEffect)))

(event EventChangeElement
  (params (ElementType :type E_ElementalType%20Enum :default "NewEnumerator0"))
  (|CallParentFunction ElementType)
  (CallFunction|UpdateMainEffect))

(fn ConstructionScript)

(fn UpdateMainEffect
  (CallFunction|DisableMainEffect)
  (bind _resulteffect (CallFunction|AttachMainEffect (.MainEffect (Utilities|GetVfx))))
  (Variables|Default|SetMainEffectRef _resulteffect)
  (bind _returnvalue (Audio|SpawnSoundAttached (.MainSfx (Utilities|GetSfx)) (Variables|Default|GetEffectLocation) "None" "0, 0, 0" "0, 0, 0" "KeepRelativeOffset" true 1.0 1.0 0.0 "/Game/Saba/SFX/AbilityAttenuation.AbilityAttenuation" 0))
  (Utilities|IsValid _returnvalue
    (:Is%20Valid
      (bind _output_get (Variables|Default|SetMainSfx%20Ref _returnvalue))
      (Audio|Components|Audio|FadeIn _output_get 0.25 1.0 0.0 "Linear" :!class /Script/Engine.AudioComponent))))

(fn DisableMainEffect
  (bind _maineffectref (Variables|Default|GetMainEffectRef)
    (:then
      (Components|DestroyComponent _maineffectref))
    (:else
      _))
  (bind _mainsfx_ref (Variables|Default|GetMainSfx%20Ref)
    (:then
      (Audio|Components|Audio|FadeOut _mainsfx_ref 0.5 0.0 "Linear" :!class /Script/Engine.AudioComponent)
      (Audio|Components|Audio|StopDelayed _mainsfx_ref 0.5)
      (Variables|Default|SetMainEffectRef 0))
    (:else)))

(fn AttachTrailEffect
  (params (Effect :type Niagara%20System%20Object%20Reference))
  (Utilities|FlowControl|Sequence
    (:then_0
      (bind _traileffectref (Variables|Default|GetTrailEffectRef)
        (:then
          (Components|DestroyComponent _traileffectref))
        (:else)))
    (:then_1
      (bind _returnvalue (Niagara|SpawnSystemAttached Effect (Variables|/Script/Engine.Character|GetMesh (Variables|Default|GetCharacter%20Ref)) (Variables|Default|GetCharacter%20Socket) "0, 0, 0" "0, 0, 0" "KeepRelativeOffset" true))
      (return _returnvalue))))

(fn AttachMainEffect
  (params (Effect :type Niagara%20System%20Object%20Reference))
  (bind _mesh (CallFunction|GetSwordMainMesh))
  (Utilities|IsValid _mesh
    (:Is%20Valid
      (bind _returnvalue (Niagara|SpawnSystemAttached Effect _mesh "None" "0, 0, 0" "0, 0, 0" "KeepRelativeOffset" true))
      (return _returnvalue))))

(fn AttachHitEffect
  (params (Effect :type Niagara%20System%20Object%20Reference))
  (bind _returnvalue (Niagara|SpawnSystemAttached Effect (Variables|Default|GetEffectLocation) "None" "0, 0, 0" "0, 0, 0" "KeepRelativeOffset" false))
  (Utilities|IsValid _returnvalue
    (:Is%20Valid
      (Class|NiagaraComponent|SetAutoDestroy _returnvalue true))
    (:Is%20Not%20Valid
      _))
  (return _returnvalue))

(fn CalculateAttackDirection
  (params (HitActor :type Actor%20Object%20Reference))
  (return (Math|Vector|GetUnitDirection(Vector) (Transformation|GetWorldLocation (Variables|/Script/Engine.Actor|GetRootComponent (Variables|Default|GetInstigator))) (Transformation|GetWorldLocation (Variables|/Script/Engine.Actor|GetRootComponent HitActor)))))

(fn EnableCollision
  (Collision|SetCollisionEnabled (Variables|Default|GetCollider) "QueryOnly"))

(fn DisableCollision
  (Collision|SetCollisionEnabled (Variables|Default|GetCollider) "NoCollision")
  (Utilities|Map|Clear (Variables|Default|GetCurrentHits)))

(fn TryHitActor
  (params (Actor :type Actor%20Object%20Reference))
  (bind _currenthits (Variables|Default|GetCurrentHits))
  (bind (_value _returnvalue) (Utilities|Map|Find _currenthits Actor))
  (if (!= (Game|GetInstigator) Actor)
    (if _returnvalue
      (if (>= _value (Variables|Default|GetHitPerAttack))
        (return false)
        (else
          (Utilities|Map|Add (Variables|Default|GetCurrentHits) Actor (+ _value 1))
          (return true)))
      (else
        (Utilities|Map|Add (Variables|Default|GetCurrentHits) Actor 1)
        (return true)))
    (else
      (return false))))

(fn GetSwordMainMesh
  (return 0))