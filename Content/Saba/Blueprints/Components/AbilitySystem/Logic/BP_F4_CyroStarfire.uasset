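; BP_F4_CyroStarfire is the ability logic for Cyro Starfire, an area damage attack that spreads one step out from the impact.
; It spawns a fire effect at the hit location, gathers hits in radius, then runs a second radius query around each of those hits.
; The second-pass results are merged into a set, and each unique character takes fixed HP damage and the ability's status effects before the parent logic runs.
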(fn ConstructionScript)

(fn ExecuteAbilityLogic
  (Niagara|SpawnSystematLocation (Variables|Default|GetFireVfx) (.Location (Collision|BreakHitResult (Variables|Default|GetAbility%20HitResult))))
  (bind _newhits (CallFunction|GetHitCharactersinRadius (Variables|Default|GetAbility%20HitResult)))
  (for _array_element _newhits
    (bind _result (CallFunction|GetHitCharactersinRadius _array_element))
    (Utilities|Set|AddItems (LocalVariables|GetTarget%20Refs) _result))
  (bind _result_2 (Utilities|Set|ToArray (LocalVariables|GetTarget%20Refs)))
  (for _array_element_2 _result_2
    (Default|UpdateStats _array_element_2 -25.0 0.0 0.0 "NewEnumerator0")
    (CallFunction|ApplyEffectstoCharacter _array_element_2 (Variables|/Game/Saba/Blueprints/Components/AbilitySystem/PDA_SpecialAbility.PDA_SpecialAbility_C|GetEffects (Variables|Default|GetAbility%20Ref))))
  (|CallParentFunction))