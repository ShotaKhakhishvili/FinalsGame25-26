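; BP_F3_AzureFrostfire is the ability logic Blueprint for Azure Frostfire, an area-of-effect damage ability.
; On execution it spawns a fire VFX system at the ability's hit location and gathers the characters within a radius of that hit.
; Each character takes a fixed HP loss and receives the status effects defined on the ability reference.
; It then hands off to the parent ability logic.
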(fn ConstructionScript)

(fn ExecuteAbilityLogic
  (Niagara|SpawnSystematLocation (Variables|Default|GetFireVfx) (.Location (Collision|BreakHitResult (Variables|Default|GetAbility%20HitResult))))
  (bind _result (CallFunction|GetHitCharactersinRadius (Variables|Default|GetAbility%20HitResult)))
  (for _array_element _result
    (Default|UpdateStats _array_element -2e+01 0.0 0.0 "NewEnumerator0")
    (CallFunction|ApplyEffectstoCharacter _array_element (Variables|/Game/Saba/Blueprints/Components/AbilitySystem/PDA_SpecialAbility.PDA_SpecialAbility_C|GetEffects (Variables|Default|GetAbility%20Ref))))
  (|CallParentFunction))