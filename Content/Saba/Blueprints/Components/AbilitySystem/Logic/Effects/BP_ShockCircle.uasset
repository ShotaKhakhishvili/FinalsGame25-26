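; Shock circle ability effect that builds a ring of BP_ShockCircleSegment actors around a start location, with a center VFX and sound.
; A delayed loop spawns mirrored segments about every 100 units, sweeping from behind the instigator's aim yaw to the front.
; Downward traces against WorldStatic place each segment on the ground.
; It gathers characters overlapping the segments and, on DestroySparks, removes them, plays an explosion sound and destroys itself.
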(event Custom|SpawnSparks
  (params (InstigatorCharacter :type BP%20Base%20Character%20Object%20Reference) (Radius :type Float%20%28double-precision%29) (StartLocation :type Vector))
  (bind _returnvalue (Math|Float|MultiplybyPi Radius))
  (bind _returnvalue_2 (/ _returnvalue 1e+02))
  (bind _returnvalue_3 (Math|Float|Ceil _returnvalue_2))
  (bind _returnvalue_4 (Niagara|SpawnSystematLocation (Variables|Default|GetSphereVfx) StartLocation))
  (Variables|Default|SetSphereVfx%20Ref _returnvalue_4)
  (bind _index (Utilities|ForLoopwithDelay 0 _returnvalue_3 0.1)
    (:LoopBody
      (CallFunction|SpawnShockSegment _index _returnvalue_3 Radius StartLocation InstigatorCharacter false)
      (if (> _index 0)
        (CallFunction|SpawnShockSegment _index _returnvalue_3 Radius StartLocation InstigatorCharacter true :!label _label)
        (else
          (bind _returnvalue_5 (Audio|SpawnSoundatLocation (Variables|Default|GetSphereSfx) StartLocation "0, 0, 0" 1.0 1.0 0.0 "/Game/Saba/SFX/AbilityAttenuation.AbilityAttenuation" 0))
          (Variables|Components|SetSphereSfx%20Ref _returnvalue_5))))
    (:Completed
      (goto _label))))

(event Custom|SpawnShockSegment
  (params (Index :type Integer) (Count :type Integer) (Radius :type Float%20%28double-precision%29) (Location :type Vector) (InstigatorCharacter :type Pawn%20Object%20Reference) (NegateAngle :type Boolean))
  (bind _returnvalue (Math|Float|SelectFloat -1.0 1.0 NegateAngle))
  (bind (_x _y _z) (Math|Vector|BreakVector Location))
  (bind _returnvalue_2 (Pawn|GetBaseAimRotation InstigatorCharacter))
  (bind _returnvalue_3 (Math|Float|MultiplybyPi Radius))
  (bind _returnvalue_4 (- Count Index))
  (bind _returnvalue_5 (Math|Trig|DegreesToRadians (.yaw _returnvalue_2)))
  (bind _returnvalue_6 (/ _returnvalue_3 Count))
  (bind _returnvalue_7 (/ _returnvalue_6 Radius))
  (bind _returnvalue_8 (* _returnvalue_4 _returnvalue_7 _returnvalue))
  (bind _returnvalue_9 (+ _returnvalue_8 _returnvalue_5))
  (bind _returnvalue_10 (Math|Trig|Cos(Radians) _returnvalue_9))
  (bind _returnvalue_11 (Math|Trig|Sin(Radians) _returnvalue_9))
  (bind _returnvalue_12 (* Radius _returnvalue_11))
  (bind _returnvalue_13 (* Radius _returnvalue_10))
  (bind _returnvalue_14 (+ _x _returnvalue_13))
  (bind _returnvalue_15 (+ _y _returnvalue_12))
  (bind _outhit (Collision|LineTraceForObjects (Math|Vector|MakeVector _returnvalue_14 _returnvalue_15 (+ _z 1.8e+02)) (Math|Vector|MakeVector _returnvalue_14 _returnvalue_15 -1e+04) (Utilities|Array|MakeArray "ObjectTypeQuery1") false (Variables|Default|GetSparks) "None"))
  (bind _returnvalue_16 (Game|SpawnActorfromClass "/Game/Saba/Blueprints/Components/AbilitySystem/Logic/Effects/BP_ShockCircleSegment.BP_ShockCircleSegment_C" (Math|Transform|MakeTransform (.Location (Collision|BreakHitResult _outhit)) "0, 0, 0" "1.000000,1.000000,1.000000") "Undefined" "MultiplyWithRoot" 0 InstigatorCharacter))
  (Utilities|Array|Add (Variables|Default|GetSparks) _returnvalue_16)
  (Variables|Default|SetCurrentSparks (+ (Variables|Default|GetCurrentSparks) 1)))

(event Custom|DestroySparks
  (bind _spheresfx_ref (Variables|Components|GetSphereSfx%20Ref))
  (for _array_element (Variables|Default|GetSparks)
    (Default|DeactivateandDestroy _array_element 0.0))
  (bind _spheresfx_ref_2 (Variables|Components|GetSphereSfx%20Ref)
    (:then
      (Audio|PlaySoundatLocation (Variables|Default|GetExplodeSfx) (Transformation|GetWorldLocation _spheresfx_ref_2) "0, 0, 0" 1.0 1.0 0.0 0 0 0 0)
      (Audio|Components|Audio|Stop _spheresfx_ref)
      (Components|DestroyComponent _spheresfx_ref))
    (:else
      _))
  (Actor|DestroyActor))

(fn ConstructionScript)

(fn GetOverlappingCharacters
  (for _array_element (Variables|Default|GetSparks)
    (for _array_element_2 (Collision|GetOverlappingActors _array_element "/Game/Saba/Blueprints/Characters/BP_BaseCharacter.BP_BaseCharacter_C" :!class /Script/Engine.Actor)
      (Utilities|Set|Add (LocalVariables|GetCharacterSet) _array_element_2)))
  (return (LocalVariables|GetCharacterSet)))