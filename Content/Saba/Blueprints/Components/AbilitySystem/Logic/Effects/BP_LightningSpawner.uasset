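; Short-lived effect actor that draws jagged lightning bolts travelling from a start to an end location, then destroys itself.
; A looping timer advances several parallel bolts along the line over a duration derived from distance and speed.
; Each step spawns a Niagara beam segment and sound per bolt, linking its previous point to a randomly offset new one.
; Jitter peaks mid-path via a cubed falloff, and the final segment snaps to the end.
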(event Custom|Update
  (bind _endlocation (Variables|Default|GetEndLocation))
  (bind _output_get (Variables|Default|SetCurrentTime (+ (Variables|Default|GetCurrentTime) (Variables|Default|GetStep))))
  (if (>= _output_get (Variables|Default|GetFinalDuration))
    (Utilities|Time|ClearandInvalidateTimerbyHandle (stale EventBeginPlay _returnvalue))
    (Actor|DestroyActor)
    (else
      (for (_array_element _array_index) (Variables|Default|GetPreviousLocations)
        (bind _output_get_2 (Variables|Default|SetCurrentLocation (Math|Vector|SelectVector _endlocation (+ (Math|Vector|Lerp(Vector) (Variables|Default|GetStartLocation) _endlocation (/ (Variables|Default|GetCurrentTime) (Variables|Default|GetFinalDuration))) (Math|Vector|MakeVector (Math|Random|RandomFloatinRange (* (* (Math|Float|Power (- 1.0 (Math|Float|Absolute(Float) (- 0.5 (/ (Variables|Default|GetCurrentTime) (Variables|Default|GetFinalDuration))))) 3.0) (* (Variables|Default|GetFinalDuration) (Variables|Default|GetWidth))) -1.0) (* (Math|Float|Power (- 1.0 (Math|Float|Absolute(Float) (- 0.5 (/ (Variables|Default|GetCurrentTime) (Variables|Default|GetFinalDuration))))) 3.0) (* (Variables|Default|GetFinalDuration) (Variables|Default|GetWidth)))) (Math|Random|RandomFloatinRange (* (* (Math|Float|Power (- 1.0 (Math|Float|Absolute(Float) (- 0.5 (/ (Variables|Default|GetCurrentTime) (Variables|Default|GetFinalDuration))))) 3.0) (* (Variables|Default|GetFinalDuration) (Variables|Default|GetWidth))) -1.0) (* (Math|Float|Power (- 1.0 (Math|Float|Absolute(Float) (- 0.5 (/ (Variables|Default|GetCurrentTime) (Variables|Default|GetFinalDuration))))) 3.0) (* (Variables|Default|GetFinalDuration) (Variables|Default|GetWidth)))) (Math|Random|RandomFloatinRange (* (* (Math|Float|Power (- 1.0 (Math|Float|Absolute(Float) (- 0.5 (/ (Variables|Default|GetCurrentTime) (Variables|Default|GetFinalDuration))))) 3.0) (* (Variables|Default|GetFinalDuration) (Variables|Default|GetWidth))) -1.0) (* (Math|Float|Power (- 1.0 (Math|Float|Absolute(Float) (- 0.5 (/ (Variables|Default|GetCurrentTime) (Variables|Default|GetFinalDuration))))) 3.0) (* (Variables|Default|GetFinalDuration) (Variables|Default|GetWidth)))))) (>= (+ (Variables|Default|GetCurrentTime) (Variables|Default|GetStep)) (Variables|Default|GetFinalDuration)))))
        (bind _returnvalue (Niagara|SpawnSystematLocation (Variables|Default|GetLightningVfx) _array_element))
        (Class|NiagaraComponent|SetVariablePosition _returnvalue "BeamEnd" (- _output_get_2 _array_element))
        (Audio|SpawnSoundatLocation (Variables|Default|GetLightningSfx) _array_element "0, 0, 0" 1.0 1.0 0.0 "/Game/Saba/SFX/AbilityAttenuation.AbilityAttenuation" 0)
        (Utilities|Array|SetArrayElem (Variables|Default|GetPreviousLocations) _array_index _output_get_2)))))

(event EventBeginPlay
  (Utilities|Array|Clear (Variables|Default|GetPreviousLocations))
  (for _index (range 1 (Variables|Default|GetLightningCount))
    (Utilities|Array|Add (Variables|Default|GetPreviousLocations) (Variables|Default|GetStartLocation)))
  (Variables|Default|SetCurrentTime 0.0)
  (Variables|Default|SetFinalDuration (/ (Math|Vector|VectorLength (- (Variables|Default|GetEndLocation) (Variables|Default|GetStartLocation))) (Variables|Default|GetSpeed)))
  (bind _returnvalue (Utilities|Time|SetTimerbyEvent (delegate Custom|Update) (Variables|Default|GetStep) true)))

(fn ConstructionScript)