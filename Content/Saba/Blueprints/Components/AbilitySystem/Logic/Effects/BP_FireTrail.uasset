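; BP_FireTrail is an effect actor that lays a trail of BP_FireTrailSegment fires along a direction and later removes them.
; SpawnFires uses a delayed loop to place segments at intervals, snapping each to world-static ground with a downward line trace.
; DestroyFires shuffles the segments, deactivates them in staggered random order, then destroys itself.
; GetOverlappingCharacters gathers the set of characters overlapping any segment.
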(event Custom|SpawnFires
  (params (InstigatorCharacter :type BP%20Base%20Character%20Object%20Reference) (Distance :type Float%20%28double-precision%29) (Direction :type Vector) (HitLocation :type Vector) (StartLocation :type Vector))
  (bind _returnvalue (Math|Conversions|RotationFromXVector Direction))
  (Utilities|ForLoopwithDelay 0 (Math|Float|Ceil (/ Distance 1e+02)) 0.1
    (:LoopBody
      (bind _outhit (Collision|LineTraceForObjects (Math|Vector|MakeVector (.X (Math|Vector|BreakVector (+ StartLocation (* Direction 200 (Variables|Default|GetCurrentFires))))) (.Y (Math|Vector|BreakVector (+ StartLocation (* Direction 200 (Variables|Default|GetCurrentFires))))) (Math|Float|Max(Float) (.Z (Math|Vector|BreakVector HitLocation)) (.Z (Math|Vector|BreakVector (+ StartLocation (* Direction 200 (Variables|Default|GetCurrentFires))))))) (Math|Vector|MakeVector (.X (Math|Vector|BreakVector (+ StartLocation (* Direction 200 (Variables|Default|GetCurrentFires))))) (.Y (Math|Vector|BreakVector (+ StartLocation (* Direction 200 (Variables|Default|GetCurrentFires))))) -1e+04) (Utilities|Array|MakeArray "ObjectTypeQuery1") false (Variables|Default|GetFires) "None"))
      (bind _returnvalue_2 (Game|SpawnActorfromClass "/Game/Saba/Blueprints/Components/AbilitySystem/Logic/Effects/BP_FireTrailSegment.BP_FireTrailSegment_C" (Math|Transform|MakeTransform (.Location (Collision|BreakHitResult _outhit)) (Math|Rotator|MakeRotator (.roll _returnvalue) 0.0 (.yaw _returnvalue)) "1.000000,1.000000,1.000000") "Undefined" "MultiplyWithRoot" 0 InstigatorCharacter))
      (Utilities|Array|Add (Variables|Default|GetFires) _returnvalue_2)
      (Variables|Default|SetCurrentFires (+ (Variables|Default|GetCurrentFires) 1)))))

(event Custom|DestroyFires
  (bind _fires (Variables|Default|GetFires))
  (Utilities|Array|Shuffle _fires)
  (bind _index (Utilities|ForLoopwithDelay 0 (Utilities|Array|Length _fires) 0.1)
    (:LoopBody
      (Default|DeactivateandDestroy (Utilities|Array|Get(acopy) (Variables|Default|GetFires) _index) (Math|Random|RandomFloatinRange 0.2 0.5)))
    (:Completed
      (Actor|DestroyActor))))

(fn ConstructionScript)

(fn GetOverlappingCharacters
  (for _array_element (Variables|Default|GetFires)
    (for _array_element_2 (Collision|GetOverlappingActors _array_element "/Game/Saba/Blueprints/Characters/BP_BaseCharacter.BP_BaseCharacter_C" :!class /Script/Engine.Actor)
      (Utilities|Set|Add (LocalVariables|GetCharacterSet) _array_element_2)))
  (return (LocalVariables|GetCharacterSet)))