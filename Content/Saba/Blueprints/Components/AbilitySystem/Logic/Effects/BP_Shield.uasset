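; BP_Shield is an ability-effect shield actor that absorbs a set number of hits before breaking.
; SetupShield sets the hit count, and each sphere overlap spawns a hit effect at the impact and decrements it.
; The remaining count selects one of three color and spawn-rate tiers for the Niagara effect and dynamic material.
; Dropping below zero plays a tinted destroy effect, fires ShieldDestroyed and destroys the actor.
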(event OnComponentBeginOverlap(Sphere)
  (params (OverlappedComponent :type Primitive%20Component%20Object%20Reference) (OtherActor :type Actor%20Object%20Reference) (OtherComp :type Primitive%20Component%20Object%20Reference) (OtherBodyIndex :type Integer) (bFromSweep :type Boolean) (SweepResult :type Hit%20Result%20Structure%20%28by%20ref%29))
  (bind (_bblockinghit _binitialoverlap _time _distance _location _impactpoint _normal _impactnormal) (Collision|BreakHitResult SweepResult))
  (bind _returnvalue (Niagara|SpawnSystematLocation (Variables|Components|GetHitVfx) _impactpoint (Math|Rotator|MakeRotfromZ _impactnormal)))
  (Niagara|SetNiagaraVariable(LinearColor) _returnvalue "Color" (.Color (Utilities|State)))
  (CallFunction|DamageShield))

(event Custom|DamageShield
  (bind _output_get (Variables|Default|SetDamageCount (Utilities|Decrement (Variables|Default|GetDamageCount))))
  (if (< _output_get 0)
    (CallFunction|DestroyShield)
    (else
      (CallFunction|UpdateShield))))

(event Custom|SetupShield
  (params (Count :type Integer))
  (Variables|Default|SetDamageCount Count)
  (CallFunction|UpdateShield))

(event Custom|UpdateShield
  (bind (_color _spawn_rate) (Utilities|State))
  (bind _shieldvfx (Variables|Default|GetShieldVfx))
  (Niagara|SetNiagaraVariable(Float) _shieldvfx "SpawnRate" _spawn_rate)
  (Niagara|SetNiagaraVariable(LinearColor) _shieldvfx "Color" _color)
  (Rendering|Material|SetVectorParameterValue (Variables|Components|GetMainMaterialInstance) "Base_Color" _color :!class /Script/Engine.MaterialInstanceDynamic))

(event Custom|DestroyShield
  (bind _returnvalue (Niagara|SpawnSystematLocation (Variables|Components|GetDestroyVfx) (Transformation|GetWorldLocation (Variables|Default|GetDestroyLocation)) "0, 0, 0" "1.000000,1.000000,1.000000" false))
  (Niagara|SetNiagaraVariable(LinearColor) _returnvalue "Color" (.Color (Utilities|State)))
  (Default|CallShieldDestroyed)
  (Actor|DestroyActor))

(fn ConstructionScript
  (bind _returnvalue (Rendering|Material|CreateDynamicMaterialInstance (Variables|Default|GetMesh) 0 "/Game/Saba/Materials/M_Shield.M_Shield" "None" :!class /Script/Engine.PrimitiveComponent))
  (Variables|Components|SetMainMaterialInstance _returnvalue))