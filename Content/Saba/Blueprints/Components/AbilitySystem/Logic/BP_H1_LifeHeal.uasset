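; Healing ability logic for the Life Heal ability, which restores health to the instigating character.
; On execution it plays the ability's montage on the instigator's mesh and attaches a healing VFX.
; After a short delay it sends a stats update with a fixed HP amount and elemental type to the instigator.
; The parent ability logic runs only when the montage completes.
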(event EventExecuteAbilityLogic
  (Animation|Montage|PlayMontage (Variables|/Script/Engine.Character|GetMesh (Variables|Default|GetAbility%20Instigator)) (Variables|/Game/Saba/Blueprints/Components/AbilitySystem/PDA_SpecialAbility.PDA_SpecialAbility_C|GetAnimation (Variables|Default|GetAbility%20Ref))
    (:then
      (Niagara|SpawnSystemAttached (Variables|Default|GetHealingVfx) (Variables|/Script/Engine.Character|GetMesh (Variables|Default|GetAbility%20Instigator)) "None" "0, 0, 0" "0, 0, 0" "KeepRelativeOffset" true)
      (Utilities|FlowControl|Delay 1.0)
      (Class|BPICharacter|UpdateStats(Message) (Variables|Default|GetAbility%20Instigator) 3e+01 0.0 0.0 "NewEnumerator3"))
    (:OnCompleted
      (|CallParentFunction))))

(fn ConstructionScript)