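; Ability logic for the E2 Faraday Cage, an area shock that damages characters around the caster over time.
; Execution locks the caster's movement during the ability montage and spawns a BP_ShockCircle that emits sparks at the ability radius.
; A looping timer damages and applies the ability's status effects to overlapping characters except the caster.
; After a fixed delay it clears the sparks and timer and destroys itself.
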(event Custom|DamageCharacters
  (bind _character_refs (Default|GetOverlappingCharacters (Variables|Default|GetShockCircle)))
  (bind _result (Utilities|Set|ToArray _character_refs))
  (for _array_element _result
    (Utilities|IsValid _array_element
      (:Is%20Valid
        (if (!= _array_element (Variables|Default|GetAbility%20Instigator))
          (Default|UpdateStats _array_element -2.0 0.0 0.0 "NewEnumerator0")
          (CallFunction|ApplyEffectstoCharacter _array_element (Variables|/Game/Saba/Blueprints/Components/AbilitySystem/PDA_SpecialAbility.PDA_SpecialAbility_C|GetEffects (Variables|Default|GetAbility%20Ref))))))))

(event EventExecuteAbilityLogic
  (bind _ability_instigator (Variables|Default|GetAbility%20Instigator))
  (bind _ability_instigator_2 (Variables|Default|GetAbility%20Instigator))
  (Class|BPICharacter|ToggleMovement(Message) _ability_instigator_2 false)
  (Animation|Montage|PlayMontage (Variables|/Script/Engine.Character|GetMesh _ability_instigator_2) (Variables|/Game/Saba/Blueprints/Components/AbilitySystem/PDA_SpecialAbility.PDA_SpecialAbility_C|GetAnimation (Variables|Default|GetAbility%20Ref))
    (:then
      (bind _returnvalue (Game|SpawnActorfromClass "/Game/Saba/Blueprints/Components/AbilitySystem/Logic/Effects/BP_ShockCircle.BP_ShockCircle_C" (Math|Transform|MakeTransform (Transformation|GetWorldLocation (Variables|/Script/Engine.Character|GetMesh _ability_instigator)) "0, 0, 0" "1.000000,1.000000,1.000000") "Undefined" "MultiplyWithRoot" 0 _ability_instigator))
      (bind _output_get (Variables|Default|SetShockCircle _returnvalue))
      (Default|SpawnSparks _output_get (Variables|Default|GetAbility%20Instigator) (Variables|/Game/Saba/Blueprints/Components/AbilitySystem/PDA_SpecialAbility.PDA_SpecialAbility_C|GetRadius (Variables|Default|GetAbility%20Ref)) (Transformation|GetWorldLocation (Variables|/Script/Engine.Character|GetMesh (Variables|Default|GetAbility%20Instigator))))
      (bind _returnvalue_2 (Utilities|Time|SetTimerbyEvent (delegate Custom|DamageCharacters) 1.0 true true))
      (Variables|Default|SetDamageTimerHandle _returnvalue_2)
      (Utilities|FlowControl|Delay 1e+01)
      (Default|DestroySparks (Variables|Default|GetShockCircle))
      (Utilities|Time|ClearandInvalidateTimerbyHandle (Variables|Default|GetDamageTimerHandle))
      (Actor|DestroyActor))
    (:OnCompleted
      (Class|BPICharacter|ToggleMovement(Message) (Variables|Default|GetAbility%20Instigator) true :!label _label)
      (Default|CallOnAbilityLogicFinish))
    (:OnInterrupted
      (goto _label))))

(fn ConstructionScript)