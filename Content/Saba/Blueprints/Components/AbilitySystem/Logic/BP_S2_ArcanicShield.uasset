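; Ability logic actor for Arcanic Shield, which surrounds the instigator with a destructible BP_Shield.
; It plays the ability montage, then after a delay replaces any attached shield with one scaled from the ability radius, calling parent logic on montage completion.
; Each hit or overlap decrements ShieldHp, destroying shield and logic actor at zero.
; Tick uses a FlipFlop to alternately grow and shrink the shield each frame, making it jitter.
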(event Custom|DestroyPreviousShield
  (for _array_element (Actor|GetAttachedActors (Variables|Default|GetAbility%20Instigator) true false)
    (if (== "/Game/Saba/Blueprints/Components/AbilitySystem/Logic/Effects/BP_Shield.BP_Shield_C" (Utilities|GetClass _array_element))
      (Actor|DestroyActor _array_element))))

(event Custom|ShieldDamaged
  (params (SelfActor :type Actor%20Object%20Reference) (OtherActor :type Actor%20Object%20Reference) (NormalImpulse :type Vector) (Hit :type Hit%20Result%20Structure%20%28by%20ref%29))
  (bind _output_get (Variables|Default|SetShieldHp (Utilities|Decrement (Variables|Default|GetShieldHp))))
  (if (== _output_get 0)
    (CallFunction|DestroyPreviousShield)
    (Actor|DestroyActor)))

(event Custom|ShieldOverlapped
  (params (OverlappedActor :type Actor%20Object%20Reference) (OtherActor :type Actor%20Object%20Reference))
  (bind _output_get (Variables|Default|SetShieldHp (Utilities|Decrement (Variables|Default|GetShieldHp))))
  (if (== _output_get 0)
    (CallFunction|DestroyPreviousShield)
    (Actor|DestroyActor)))

(event EventTick
  (params (DeltaSeconds :type Float%20%28single-precision%29))
  (bind _returnvalue (* DeltaSeconds 3.0))
  (bind _shield (Variables|Default|GetShield)
    (:then
      (Utilities|FlowControl|FlipFlop
        (:A
          (Transformation|SetActorScale3D _shield (+ _returnvalue (Transformation|GetActorScale3D _shield))))
        (:B
          (Transformation|SetActorScale3D _shield (- (Transformation|GetActorScale3D _shield) _returnvalue)))))
    (:else)))

(event EventExecuteAbilityLogic
  (bind _ability_ref (Variables|Default|GetAbility%20Ref))
  (bind _radius (Variables|/Game/Saba/Blueprints/Components/AbilitySystem/PDA_SpecialAbility.PDA_SpecialAbility_C|GetRadius _ability_ref))
  (bind _returnvalue (/ _radius 5e+01))
  (Animation|Montage|PlayMontage (Variables|/Script/Engine.Character|GetMesh (Variables|Default|GetAbility%20Instigator)) (Variables|/Game/Saba/Blueprints/Components/AbilitySystem/PDA_SpecialAbility.PDA_SpecialAbility_C|GetAnimation (Variables|Default|GetAbility%20Ref))
    (:then
      (Utilities|FlowControl|Delay 1.0)
      (CallFunction|DestroyPreviousShield)
      (bind _returnvalue_2 (Game|SpawnActorfromClass "/Game/Saba/Blueprints/Components/AbilitySystem/Logic/Effects/BP_Shield.BP_Shield_C" (Math|Transform|MakeTransform "0, 0, 0" "0, 0, 0" "1.000000,1.000000,1.000000") "Undefined" "MultiplyWithRoot" 0 (Variables|Default|GetAbility%20Instigator)))
      (bind _output_get (Variables|Default|SetShield _returnvalue_2))
      (Transformation|AttachActorToActor _output_get (Variables|Default|GetAbility%20Instigator) "None" "KeepRelative" "KeepRelative" "KeepRelative" true)
      (Transformation|SetActorScale3D (Variables|Default|GetShield) (Math|Vector|MakeVector _returnvalue _returnvalue _returnvalue))
      (Collision|BindEventtoOnActorHit (Variables|Default|GetShield) (delegate Custom|ShieldDamaged))
      (Collision|BindEventtoOnActorBeginOverlap (Variables|Default|GetShield) (delegate Custom|ShieldOverlapped)))
    (:OnCompleted
      (|CallParentFunction))))

(fn ConstructionScript)