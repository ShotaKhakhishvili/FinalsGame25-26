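; Ability logic for Scorch Lance, which lays a temporary trail of fire along the attack direction that damages characters caught in it.
; On execution it spawns a BP_FireTrail at the instigator's mesh and passes it the ability radius as trail length, plus the hit location.
; A looping timer drains health and applies the ability's status effects to overlapping characters except the caster, until a delay destroys the fires and clears the timer.
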(event Custom|DamageCharacters
  (bind _character_refs (Default|GetOverlappingCharacters (Variables|Default|GetFireTrail)))
  (bind _result (Utilities|Set|ToArray _character_refs))
  (for _array_element _result
    (Utilities|IsValid _array_element
      (:Is%20Valid
        (if (!= _array_element (Variables|Default|GetAbility%20Instigator))
          (Default|UpdateStats _array_element -2.5 0.0 0.0 "NewEnumerator0")
          (CallFunction|ApplyEffectstoCharacter _array_element (Variables|/Game/Saba/Blueprints/Components/AbilitySystem/PDA_SpecialAbility.PDA_SpecialAbility_C|GetEffects (Variables|Default|GetAbility%20Ref))))))))

(event EventExecuteAbilityLogic
  (bind _ability_instigator (Variables|Default|GetAbility%20Instigator))
  (|CallParentFunction)
  (bind _returnvalue (Game|SpawnActorfromClass "/Game/Saba/Blueprints/Components/AbilitySystem/Logic/Effects/BP_FireTrail.BP_FireTrail_C" (Math|Transform|MakeTransform (Transformation|GetWorldLocation (Variables|/Script/Engine.Character|GetMesh _ability_instigator)) "0, 0, 0" "1.000000,1.000000,1.000000") "Undefined" "MultiplyWithRoot" 0 _ability_instigator))
  (bind _output_get (Variables|Default|SetFireTrail _returnvalue))
  (Default|SpawnFires _output_get (Variables|Default|GetAbility%20Instigator) (Variables|/Game/Saba/Blueprints/Components/AbilitySystem/PDA_SpecialAbility.PDA_SpecialAbility_C|GetRadius (Variables|Default|GetAbility%20Ref)) (Variables|Default|GetAttack%20Direction) (.Location (Collision|BreakHitResult (Variables|Default|GetAbility%20HitResult))) (Transformation|GetWorldLocation (Variables|/Script/Engine.Character|GetMesh (Variables|Default|GetAbility%20Instigator))))
  (bind _returnvalue_2 (Utilities|Time|SetTimerbyEvent (delegate Custom|DamageCharacters) 1.0 true true))
  (Variables|Default|SetDamageTimerHandle _returnvalue_2)
  (Utilities|FlowControl|Delay 1e+01)
  (Default|DestroyFires (Variables|Default|GetFireTrail))
  (Utilities|Time|ClearandInvalidateTimerbyHandle (Variables|Default|GetDamageTimerHandle)))

(fn ConstructionScript)