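; BP_N3_SoulDrain is the Soul Drain ability logic, which steals health from the hit character for the ability instigator.
; On execution it runs the parent logic, resolves the character from the ability hit result and passes both characters to TransferHP with a fixed amount.
; TransferHP validates both characters, then applies damage and healing through UpdateStats, each with its own elemental type and limited by the victim's HP.
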(event Custom|TransferHP
  (params (FromCharacter :type BPI%20Character%20Interface) (ToCharacter :type BPI%20Character%20Interface) (Hp :type Float%20%28double-precision%29))
  (Utilities|IsValid (Utilities|ToObject(Interface) FromCharacter)
    (:Is%20Valid
      (Utilities|IsValid (Utilities|ToObject(Interface) ToCharacter)
        (:Is%20Valid
          (bind _hp (Default|GetStats FromCharacter))
          (Utilities|FlowControl|Sequence
            (:then_0
              (Default|UpdateStats FromCharacter (Utilities|Negate (Math|Float|Min(Float) _hp Hp)) 0.0 0.0 "NewEnumerator2"))
            (:then_1
              (Default|UpdateStats ToCharacter (Math|Float|Min(Float) _hp Hp) 0.0 0.0 "NewEnumerator3"))))))))

(event EventExecuteAbilityLogic
  (|CallParentFunction)
  (bind _result (CallFunction|GetHitCharacter (Variables|Default|GetAbility%20HitResult)))
  (CallFunction|TransferHP _result (Variables|Default|GetAbility%20Instigator) 3e+01))

(fn ConstructionScript)