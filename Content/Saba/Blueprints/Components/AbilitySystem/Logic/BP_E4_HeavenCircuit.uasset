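; BP_E4_HeavenCircuit is the logic for the Heaven Circuit ability, an area attack that deals elemental damage in two stages.
; After the parent logic runs, it gathers the characters within a radius of the ability's hit result.
; A delayed loop damages them one after another in a short stagger, applying the ability's status effects to each.
; When the loop completes, all gathered characters take a heavier hit of the same element at once.
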(event EventExecuteAbilityLogic
  (|CallParentFunction)
  (bind _result (CallFunction|GetHitCharactersinRadius (Variables|Default|GetAbility%20HitResult)))
  (bind _index (Utilities|ForLoopwithDelay 0 (Utilities|Array|Length _result) 0.1)
    (:LoopBody
      (Default|UpdateStats (Utilities|Array|Get(acopy) _result _index) -2e+01 0.0 0.0 "NewEnumerator1")
      (CallFunction|ApplyEffectstoCharacter (Utilities|Array|Get(acopy) _result _index) (Variables|/Game/Saba/Blueprints/Components/AbilitySystem/PDA_SpecialAbility.PDA_SpecialAbility_C|GetEffects (Variables|Default|GetAbility%20Ref))))
    (:Completed
      (for _array_element _result
        (Default|UpdateStats _array_element -3e+01 0.0 0.0 "NewEnumerator1")))))

(fn ConstructionScript)