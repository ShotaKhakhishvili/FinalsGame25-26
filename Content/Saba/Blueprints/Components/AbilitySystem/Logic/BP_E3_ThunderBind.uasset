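; BP_E3_ThunderBind is an ability logic Blueprint for an area lightning attack that chains between characters hit in a radius.
; A delayed loop steps through those characters, applying fixed elemental HP damage and the ability's status effects to each.
; Each hit after the first spawns a BP_LightningSpawner arc from the previous target at randomized heights.
; The parent ability logic runs once the loop completes.
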(event Custom|HitLightning
  (params (From :type BP%20Base%20Character%20Object%20Reference) (To :type BP%20Base%20Character%20Object%20Reference))
  (Game|SpawnActorfromClass "/Game/Saba/Blueprints/Components/AbilitySystem/Logic/Effects/BP_LightningSpawner.BP_LightningSpawner_C" (Math|Transform|MakeTransform "0, 0, 0" "0, 0, 0" "1.000000,1.000000,1.000000") "Undefined" "MultiplyWithRoot" 0 (Variables|Default|GetShockVfx) (Utilities|AddRandomHeight (Transformation|GetWorldLocation (Variables|/Script/Engine.Character|GetMesh From))) (Utilities|AddRandomHeight (Transformation|GetWorldLocation (Variables|/Script/Engine.Character|GetMesh To))) 10 1e+04 2e+02 0))

(event EventExecuteAbilityLogic
  (bind _result (CallFunction|GetHitCharactersinRadius (Variables|Default|GetAbility%20HitResult)))
  (bind _index (Utilities|ForLoopwithDelay 0 (Utilities|Array|Length _result) 0.1)
    (:LoopBody
      (Default|UpdateStats (Utilities|Array|Get(acopy) _result _index) -15.0 0.0 0.0 "NewEnumerator1")
      (CallFunction|ApplyEffectstoCharacter (Utilities|Array|Get(acopy) _result _index) (Variables|/Game/Saba/Blueprints/Components/AbilitySystem/PDA_SpecialAbility.PDA_SpecialAbility_C|GetEffects (Variables|Default|GetAbility%20Ref)))
      (Utilities|IsValid (Variables|Default|GetLastHit)
        (:Is%20Valid
          (CallFunction|HitLightning (Variables|Default|GetLastHit) (Utilities|Array|Get(acopy) _result _index)))
        (:Is%20Not%20Valid
          _))
      (Variables|Default|SetLastHit (Utilities|Array|Get(acopy) _result _index)))
    (:Completed
      (|CallParentFunction))))

(fn ConstructionScript)