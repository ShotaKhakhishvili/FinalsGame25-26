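; Base ability logic actor that stores an ability's data, instigator, weapon and element, then executes it from a hit result and attack direction.
; Execution runs the logic event and spawns attached SFX; the base event signals completion, fades any valid sound and destroys the actor.
; Helpers find characters within the ability radius, putting the hit character first, and apply status effects, routing inversed ones to the instigator.
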(event Custom|ExecuteAbilityLogic
  (bind _ability_ref (Variables|Default|GetAbility%20Ref))
  (bind _sfxfade (Variables|/Game/Saba/Blueprints/Components/AbilitySystem/PDA_SpecialAbility.PDA_SpecialAbility_C|GetSfxFade _ability_ref))
  (Default|CallOnAbilityLogicFinish)
  (bind _sfx_ref (Variables|Default|GetSfx%20Ref)
    (:then
      (Audio|Components|Audio|FadeOut _sfx_ref _sfxfade 0.0 "Linear" :!class /Script/Engine.AudioComponent)
      (Utilities|FlowControl|Delay _sfxfade))
    (:else
      _))
  (Actor|DestroyActor))

(fn ConstructionScript)

(fn TriggerAbility
  (params (Ability%20Ref :type PDA%20Special%20Ability%20Object%20Reference) (Instigator :type BP%20Base%20Character%20Object%20Reference) (Weapon%20Ref :type BP%20Weapon%20Object%20Reference) (Elemental :type E_ElementalType%20Enum :default "NewEnumerator0"))
  (Variables|Default|SetAbility%20Ref Ability%20Ref)
  (Variables|Default|SetAbility%20Instigator Instigator)
  (Variables|Default|SetAbility%20Weapon Weapon%20Ref)
  (Variables|Default|SetAbility%20Elemental Elemental))

(fn ApplyEffectstoCharacter
  (params (Character%20Ref :type BPI%20Character%20Interface) (StatusEffects :type Array%20of%20PDA%20Status%20Effect%20Object%20References))
  (Utilities|IsValid (Utilities|ToObject(Interface) Character%20Ref)
    (:Is%20Valid
      (bind _charactereffects (CallFunction|GetEffectsforCharacter Character%20Ref StatusEffects))
      (for _array_element _charactereffects
        (Default|ApplyStatusEffect Character%20Ref _array_element)))))

(fn GetEffectsforCharacter
  (params (Character%20Ref :type BPI%20Character%20Interface) (StatusEffects :type Array%20of%20PDA%20Status%20Effect%20Object%20References))
  ;[0.15 0.15 0.15 0.5] Filter effects for instigator or target character. Inversed effects will go to the instigator
  (for _array_element StatusEffects
    (if (== (Variables|Default|GetAbility%20Instigator) Character%20Ref)
      (if (Variables|/Game/Saba/Blueprints/Components/StatusEffectSystem/PDA_StatusEffect.PDA_StatusEffect_C|GetInversed _array_element)
        (Utilities|Array|Add (LocalVariables|GetEffects) _array_element :!label _label))
      (elif (not (Variables|/Game/Saba/Blueprints/Components/StatusEffectSystem/PDA_StatusEffect.PDA_StatusEffect_C|GetInversed _array_element))
        (goto _label))))
  (return (LocalVariables|GetEffects)))

(fn GetHitCharactersinRadius
  (params (HitResult :type Hit%20Result%20Structure))
  (bind _location (Utilities|HitLocation HitResult))
  (bind _outhits (Collision|MultiSphereTraceForObjects _location _location (Variables|/Game/Saba/Blueprints/Components/AbilitySystem/PDA_SpecialAbility.PDA_SpecialAbility_C|GetRadius (Variables|Default|GetAbility%20Ref)) (Utilities|Array|MakeArray "ObjectTypeQuery9") false (Utilities|Array|MakeArray (Variables|Default|GetAbility%20Instigator)) "None"))
  (bind _output_get (LocalVariables|SetTargetHits _outhits))
  (for _array_element _output_get
    (bind _asbp_base_character (Utilities|Casting|CastToBP_BaseCharacter (.HitActor (Collision|BreakHitResult _array_element))))
    (Utilities|Set|Add (LocalVariables|GetTarget%20Refs) _asbp_base_character))
  (bind _result (Utilities|Set|ToArray (LocalVariables|GetTarget%20Refs)))
  (bind _result_2 (CallFunction|GetHitCharacter HitResult))
  (Utilities|IsValid _result_2
    (:Is%20Valid
      (Utilities|Array|RemoveItem _result _result_2)
      (Utilities|Array|Insert _result _result_2))
    (:Is%20Not%20Valid
      _))
  (return _result (LocalVariables|GetTargetHits)))

(fn GetHitCharacter
  (params (HitResult :type Hit%20Result%20Structure))
  (bind _asbp_base_character (Utilities|Casting|CastToBP_BaseCharacter (.HitActor (Collision|BreakHitResult HitResult))))
  (return _asbp_base_character))

(fn ExecuteAbility
  (params (HitResult :type Hit%20Result%20Structure) (AttackDirection :type Vector))
  (bind _hitcomponent (Collision|BreakHitResult HitResult))
  (Variables|Default|SetAbility%20HitResult HitResult)
  (Variables|Default|SetAttack%20Direction AttackDirection)
  (CallFunction|ExecuteAbilityLogic)
  (bind _sfx (Variables|/Game/Saba/Blueprints/Components/AbilitySystem/PDA_SpecialAbility.PDA_SpecialAbility_C|GetSfx (Variables|Default|GetAbility%20Ref))
    (:then
      (bind _returnvalue (Audio|SpawnSoundAttached _sfx (Utilities|Select :Index (Variables|/Game/Saba/Blueprints/Components/AbilitySystem/PDA_SpecialAbility.PDA_SpecialAbility_C|GetType (Variables|Default|GetAbility%20Ref)) :NewEnumerator0 0 :NewEnumerator1 _hitcomponent :NewEnumerator4 _hitcomponent :NewEnumerator2 _hitcomponent :NewEnumerator3 (Variables|/Script/Engine.Character|GetMesh (Variables|Default|GetAbility%20Instigator))) "None" "0, 0, 0" "0, 0, 0" "KeepRelativeOffset" true 1.0 1.0 0.0 "/Game/Saba/SFX/AbilityAttenuation.AbilityAttenuation" 0))
      (Variables|Default|SetSfx%20Ref _returnvalue))
    (:else)))