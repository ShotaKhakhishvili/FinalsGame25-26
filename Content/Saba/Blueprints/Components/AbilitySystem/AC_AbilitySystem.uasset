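; Ability system component for BP_BaseCharacter that runs an element-specific ability set with mana costs and per-type cooldowns, ticked down each frame.
; Arming an ability spends mana and spawns its attached logic actor; cast, self and passive abilities execute immediately.
; Others await HitCallback from the armed weapon with sufficient charge, while other weapons trigger the default ability and every character hit takes basic damage.
; Execution starts cooldown; completion clears armed state.
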(event Custom|HitCallback
  (params (HitResult :type Hit%20Result%20Structure) (Weapon :type BP%20Weapon%20Object%20Reference) (Charge :type Float%20%28double-precision%29) (Direction :type Vector) (Elemental :type E_ElementalType%20Enum :default "NewEnumerator0"))
  (bind _defaultability (Variables|Default|GetDefaultAbility))
  (if (== Weapon (Variables|Default|GetArmedAbilityWeapon))
    (if (>= Charge (Variables|/Game/Saba/Blueprints/Components/AbilitySystem/PDA_SpecialAbility.PDA_SpecialAbility_C|GetRequiredCharge (Variables|Default|GetArmedAbility)))
      (CallFunction|ExecuteAbility (Variables|Default|GetArmedAbility) (Variables|Default|GetArmedAbilityLogic) HitResult Direction))
    (else
      ;[0.15 0.15 0.15 0.5 12] Default Ability
      (bind _passed (CallFunction|CheckAbilityAvailable _defaultability))
      (if (and _passed (>= Charge (Variables|/Game/Saba/Blueprints/Components/AbilitySystem/PDA_SpecialAbility.PDA_SpecialAbility_C|GetRequiredCharge (Variables|Default|GetDefaultAbility))))
        (bind _abilitylogic (CallFunction|TriggerAbility _defaultability Weapon Elemental))
        (CallFunction|ExecuteAbility _defaultability _abilitylogic HitResult Direction))))
  ;[0.15 0.15 0.15 0.5 12] Basic Attack
  (bind _hitcharacter_ref (CallFunction|GetHitCharacter HitResult))
  (Utilities|IsValid _hitcharacter_ref
    (:Is%20Valid
      (Class|BPICharacter|UpdateStats(Message) _hitcharacter_ref (* (Variables|/Game/Saba/Blueprints/Weapons/BP_Weapon.BP_Weapon_C|GetBaseDamage Weapon) (- -1.0 Charge)) 0.0 0.0 Elemental))))

(event Custom|ArmAbility
  (params (Ability :type PDA%20Special%20Ability%20Object%20Reference) (Weapon :type BP%20Weapon%20Object%20Reference) (Elemental :type E_ElementalType%20Enum :default "NewEnumerator0"))
  (bind _passed (CallFunction|CheckAbilityAvailable Ability))
  (if _passed
    (bind _output_get (Variables|Default|SetArmedAbilityWeapon Weapon))
    (bind _output_get_2 (Variables|Default|SetArmedAbility Ability))
    (bind _abilitylogic (CallFunction|TriggerAbility _output_get_2 _output_get Elemental))
    (Variables|Default|SetArmedAbilityLogic _abilitylogic)
    (bind _result (CallFunction|IsAwaitingAttack (Variables|Default|GetArmedAbility)))
    (Default|CallOnAbilityStart _result)
    ;[0.15 0.15 0.15 0.5] If ability is self or cast
    (if (or (Variables|/Game/Saba/Blueprints/Components/AbilitySystem/PDA_SpecialAbility.PDA_SpecialAbility_C|GetIsCast (Variables|Default|GetArmedAbility)) (Utilities|Set|Contains (Utilities|Set|MakeSet "NewEnumerator3" "NewEnumerator0") (Variables|/Game/Saba/Blueprints/Components/AbilitySystem/PDA_SpecialAbility.PDA_SpecialAbility_C|GetType (Variables|Default|GetArmedAbility))))
      (CallFunction|ExecuteAbility :Ability (Variables|Default|GetArmedAbility) :AbilityLogic (Variables|Default|GetArmedAbilityLogic)))
    (else
      (Audio|PlaySound2D "/Game/Saba/SFX/Character/SW_CharacterZeroMana.SW_CharacterZeroMana" 1.0 1.0 0.0 0 0))))

(event Custom|ReArmAbility
  (params (Weapon :type BP%20Weapon%20Object%20Reference))
  ;[0.15 0.15 0.15 0.5] If charge is not met, update new arrow/weapon ref
  (Variables|Default|SetArmedAbilityWeapon Weapon))

(event Custom|ExecuteAbility
  (params (Ability :type PDA%20Special%20Ability%20Object%20Reference) (AbilityLogic :type BP%20Ability%20Base%20Logic%20Object%20Reference) (HitResult :type Hit%20Result%20Structure) (AttackDirection :type Vector))
  (EventDispatchers|BindEventtoOnAbilityLogicFinish AbilityLogic (delegate Custom|AbilityFinished))
  (Default|ExecuteAbility AbilityLogic HitResult AttackDirection)
  (CallFunction|ApplyCooldown Ability))

(event Custom|AbilityFinished
  (bind _result (CallFunction|IsAwaitingAttack (stale Custom|ExecuteAbility Ability)))
  (if (or (== (stale Custom|ExecuteAbility Ability) (Variables|Default|GetArmedAbility)) (not (Utilities|IsValid (Variables|Default|GetArmedAbility))))
    (Variables|Default|SetIsAbilityArmed false)
    (Variables|Default|SetArmedAbility 0)
    (Variables|Default|SetArmedAbilityLogic 0)
    (Variables|Default|SetArmedAbilityWeapon 0))
  (Utilities|FlowControl|DelayUntilNextTick)
  (Default|CallOnAbilityEnd _result (CallFunction|FGetCooldownfromType (Variables|/Game/Saba/Blueprints/Components/AbilitySystem/PDA_SpecialAbility.PDA_SpecialAbility_C|GetType (stale Custom|ExecuteAbility Ability))) (Variables|/Game/Saba/Blueprints/Components/AbilitySystem/PDA_SpecialAbility.PDA_SpecialAbility_C|GetType (stale Custom|ExecuteAbility Ability))))

(event EventBeginPlay
  (bind _asbp_base_character (Utilities|Casting|CastToBP_BaseCharacter (Components|GetOwner)))
  (Variables|Default|SetCharacter%20Ref _asbp_base_character))

(event EventChangeElement
  (params (ElementType :type E_ElementalType%20Enum :default "NewEnumerator0"))
  (bind _output_get (Variables|Default|SetElemental ElementType))
  (bind _abilityset (Default|GetAbilitySet (Variables|Default|GetCharacter%20Ref) _output_get))
  (Variables|Default|SetDefaultAbility (.defaultability _abilityset))
  (Variables|Default|SetLightAbility (.ligthability _abilityset))
  (Variables|Default|SetHeavyAbility (.heavyability _abilityset))
  (Variables|Default|SetHpAbility (.hpability _abilityset))
  (Variables|Default|SetShieldAbility (.shieldability _abilityset))
  (for _array_element (.passiveabilities _abilityset)
    (CallFunction|ArmAbility _array_element 0 "NewEnumerator0")))

(event EventTick
  (params (DeltaSeconds :type Float%20%28single-precision%29))
  ;[0.15 0.15 0.15 0.5] Decrease Cooldowns
  (Utilities|FlowControl|Sequence
    (:then_0
      (Utilities|IsValid (Variables|Default|GetLightAbility)
        (:Is%20Valid
          (if (not (< (Variables|Default|GetLightCooldown) 0.0))
            (Variables|Default|SetLightCooldown (Math|Float|Clamp(Float) (- (Variables|Default|GetLightCooldown) DeltaSeconds) 0.0 (Variables|/Game/Saba/Blueprints/Components/AbilitySystem/PDA_SpecialAbility.PDA_SpecialAbility_C|GetCooldown (Variables|Default|GetLightAbility))))))))
    (:then_1
      (Utilities|IsValid (Variables|Default|GetHeavyAbility)
        (:Is%20Valid
          (if (not (< (Variables|Default|GetHeavyCooldown) 0.0))
            (Variables|Default|SetHeavyCooldown (Math|Float|Clamp(Float) (- (Variables|Default|GetHeavyCooldown) DeltaSeconds) 0.0 (Variables|/Game/Saba/Blueprints/Components/AbilitySystem/PDA_SpecialAbility.PDA_SpecialAbility_C|GetCooldown (Variables|Default|GetHeavyAbility))))))))
    (:then_2
      (Utilities|IsValid (Variables|Default|GetHpAbility)
        (:Is%20Valid
          (if (not (< (Variables|Default|GetSelfCooldown) 0.0))
            (Variables|Default|SetSelfCooldown (Math|Float|Clamp(Float) (- (Variables|Default|GetSelfCooldown) DeltaSeconds) 0.0 (Variables|/Game/Saba/Blueprints/Components/AbilitySystem/PDA_SpecialAbility.PDA_SpecialAbility_C|GetCooldown (Variables|Default|GetHpAbility))))))))))

(fn CheckAbilityAvailable
  (params (Ability :type PDA%20Special%20Ability%20Object%20Reference))
  (if (Variables|Default|GetIsAbilityArmed)
    (Development|PrintString (Utilities|String|Append "AAAAAAAAAAAAAAAA" "-------------" (Utilities|GetDisplayName (Variables|Default|GetArmedAbility))))
    (return false)
    (else
      (Utilities|IsValid Ability
        (:Is%20Valid
          (switch Utilities|FlowControl|Switch|SwitchonE_AbilityType (Variables|/Game/Saba/Blueprints/Components/AbilitySystem/PDA_SpecialAbility.PDA_SpecialAbility_C|GetType Ability)
            (:NewEnumerator0
              (LocalVariables|SetResult true :!label _label))
            (:NewEnumerator1
              (LocalVariables|SetResult (<= (Variables|Default|GetLightCooldown) 0.0)))
            (:NewEnumerator4
              (LocalVariables|SetResult (<= (Variables|Default|GetHeavyCooldown) 0.0)))
            (:NewEnumerator2
              (goto _label))
            (:NewEnumerator3
              (LocalVariables|SetResult (<= (Variables|Default|GetSelfCooldown) 0.0))))
          (bind _result (CallFunction|IsEnoughMana Ability))
          (bind _output_get (LocalVariables|SetResult (and (LocalVariables|GetResult) _result)))
          (return _output_get))))))

(fn ApplyCooldown
  (params (Ability :type PDA%20Special%20Ability%20Object%20Reference))
  (bind _cooldown (Variables|/Game/Saba/Blueprints/Components/AbilitySystem/PDA_SpecialAbility.PDA_SpecialAbility_C|GetCooldown Ability))
  (switch Utilities|FlowControl|Switch|SwitchonE_AbilityType (Variables|/Game/Saba/Blueprints/Components/AbilitySystem/PDA_SpecialAbility.PDA_SpecialAbility_C|GetType Ability)
    (:NewEnumerator1
      (Variables|Default|SetLightCooldown (* (Variables|Default|GetCooldownMultiplier) _cooldown)))
    (:NewEnumerator4
      (Variables|Default|SetHeavyCooldown (* (Variables|Default|GetCooldownMultiplier) _cooldown)))
    (:NewEnumerator3
      (Variables|Default|SetSelfCooldown (* (Variables|Default|GetCooldownMultiplier) _cooldown)))))

(fn TriggerAbility
  (params (Ability :type PDA%20Special%20Ability%20Object%20Reference) (Weapon :type BP%20Weapon%20Object%20Reference) (Elemental :type E_ElementalType%20Enum :default "NewEnumerator0"))
  (bind _character_ref (Variables|Default|GetCharacter%20Ref))
  (bind _returnvalue (Game|SpawnActorfromClass (Variables|/Game/Saba/Blueprints/Components/AbilitySystem/PDA_SpecialAbility.PDA_SpecialAbility_C|GetLogicClass Ability) (Math|Transform|MakeTransform "0, 0, 0" "0, 0, 0" "1.000000,1.000000,1.000000") "Undefined" "MultiplyWithRoot" 0 (Variables|Default|GetCharacter%20Ref)))
  (Transformation|AttachActorToActor _returnvalue (Variables|Default|GetCharacter%20Ref) "None" "KeepRelative" "KeepRelative" "KeepRelative" true)
  (Default|TriggerAbility _returnvalue Ability _character_ref Weapon Elemental)
  (Default|UpdateStats _character_ref 0.0 (Utilities|Negate (Variables|/Game/Saba/Blueprints/Components/AbilitySystem/PDA_SpecialAbility.PDA_SpecialAbility_C|GetCost Ability)) 0.0 Elemental)
  (Variables|Default|SetIsAbilityArmed true)
  (return _returnvalue))

(fn GetHitCharacter
  (params (HitResult :type Hit%20Result%20Structure))
  (bind _asbp_base_character (Utilities|Casting|CastToBP_BaseCharacter (.HitActor (Collision|BreakHitResult HitResult)))
    (:then
      (return _asbp_base_character))
    (:CastFailed
      (return 0))))

(fn IsEnoughMana
  (params (Ability :type PDA%20Special%20Ability%20Object%20Reference))
  (bind _mana (Class|BPICharacter|GetStats(Message) (Variables|Default|GetCharacter%20Ref)))
  (return (>= _mana (Variables|/Game/Saba/Blueprints/Components/AbilitySystem/PDA_SpecialAbility.PDA_SpecialAbility_C|GetCost Ability))))

(fn IsAwaitingAttack
  (params (Ability :type PDA%20Special%20Ability%20Object%20Reference))
  (return (and (not (Variables|/Game/Saba/Blueprints/Components/AbilitySystem/PDA_SpecialAbility.PDA_SpecialAbility_C|GetIsCast Ability)) (Utilities|Select :Index (Variables|/Game/Saba/Blueprints/Components/AbilitySystem/PDA_SpecialAbility.PDA_SpecialAbility_C|GetType Ability) :NewEnumerator0 false :NewEnumerator1 true :NewEnumerator4 true :NewEnumerator2 false :NewEnumerator3 false))))

(fn FGetAbilityfromIndex
  (params (AbilityIndex :type Integer))
  (switch int AbilityIndex
    (:Default
      (return (Variables|Default|GetDefaultAbility)))
    (:0
      (return (Variables|Default|GetDefaultAbility)))
    (:1
      (return (Variables|Default|GetLightAbility)))
    (:2
      (return (Variables|Default|GetHeavyAbility)))))

(fn GetArmedAbilityType
  (bind _armedability (Variables|Default|GetArmedAbility)
    (:then
      (return (Variables|/Game/Saba/Blueprints/Components/AbilitySystem/PDA_SpecialAbility.PDA_SpecialAbility_C|GetType _armedability)))
    (:else
      (return "NewEnumerator0"))))

(fn FGetCooldownfromType
  (params (Type :type E_AbilityType%20Enum :default "NewEnumerator0"))
  (return (Utilities|Select :Index Type :NewEnumerator0 0.0 :NewEnumerator1 (Variables|Default|GetLightCooldown) :NewEnumerator4 (Variables|Default|GetHeavyCooldown) :NewEnumerator2 0.0 :NewEnumerator3 (Variables|Default|GetSelfCooldown))))