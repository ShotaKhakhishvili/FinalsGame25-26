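; Actor component that tracks the active element of a BP_BaseCharacter and cycles through that character's available elementals.
; On BeginPlay it caches the owning character and binds to component activation, which steps the selection backward.
; GetNextElement re-reads the character's elemental list, exits if empty, moves the index forward or back with a modulo, then broadcasts OnElementChanged with the new element.
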(event Custom|ActivateComponent
  (params (Component :type Actor%20Component%20Object%20Reference) (bReset :type Boolean))
  (CallFunction|GetNextElement false))

(event EventBeginPlay
  (bind _asbp_character_base (Utilities|Casting|CastToBP_BaseCharacter (Components|GetOwner)))
  (Variables|Default|SetCharacter%20Ref _asbp_character_base)
  (Components|Activation|BindEventtoOnComponentActivated (delegate Custom|ActivateComponent)))

(fn GetNextElement
  (params (Next :type Boolean))
  (Utilities|FlowControl|Sequence
    (:then_0
      ;[0.15 0.15 0.15 0.5] Init local variables
      (LocalVariables|SetInitialElemental (Variables|Default|GetElement))
      (bind _elementals (Default|GetElementals (Variables|Default|GetCharacter%20Ref)))
      (bind _output_get (LocalVariables|SetAvailableElementals _elementals))
      (if (Utilities|Array|IsEmpty _output_get)
        (return)))
    (:then_1
      ;[0.15 0.15 0.15 0.5] Get next elemental index
      (Variables|Default|SetElementIndex (Utilities|Modulo (+ (select Next 1 -1) (Variables|Default|GetElementIndex)) (Utilities|Array|Length (LocalVariables|GetAvailableElementals)))))
    (:then_2
      ;[0.15 0.15 0.15 0.5] Change elemental and trigger event
      (bind _output_get_2 (Variables|Default|SetElement (Utilities|Array|Get(acopy) (LocalVariables|GetAvailableElementals) (Variables|Default|GetElementIndex))))
      (Default|CallOnElementChanged _output_get_2))))