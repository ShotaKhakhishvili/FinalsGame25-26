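; Ability tree component that tracks skill points, unlocked elementals and unlocked skills, using fixed lists of skill data assets filled on BeginPlay.
; Node state derives from gameplay tags: a node's ID marks it unlocked, while prerequisite tags gate spending a point.
; GetAbilitySet builds an element's loadout from unlocked nodes, assigning attack slots by rank, keeping the highest-ranked heavy, HP and shield abilities, and gathering all defence and offence passives.
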(event EventBeginPlay
  (Variables|Default|SetFireAbilities (Utilities|Array|MakeArray "/Game/Saba/Blueprints/Components/AbilityTree/DA_Skill_F1.DA_Skill_F1" "/Game/Saba/Blueprints/Components/AbilityTree/DA_Skill_F2.DA_Skill_F2" "/Game/Saba/Blueprints/Components/AbilityTree/DA_Skill_F3.DA_Skill_F3" "/Game/Saba/Blueprints/Components/AbilityTree/DA_Skill_F4.DA_Skill_F4"))
  (Variables|Default|SetElectroAbilities (Utilities|Array|MakeArray "/Game/Saba/Blueprints/Components/AbilityTree/DA_Skill_E1.DA_Skill_E1" "/Game/Saba/Blueprints/Components/AbilityTree/DA_Skill_E2.DA_Skill_E2" "/Game/Saba/Blueprints/Components/AbilityTree/DA_Skill_E3.DA_Skill_E3" "/Game/Saba/Blueprints/Components/AbilityTree/DA_Skill_E4.DA_Skill_E4"))
  (Variables|Default|SetNecroAbilities (Utilities|Array|MakeArray "/Game/Saba/Blueprints/Components/AbilityTree/DA_Skill_N1.DA_Skill_N1" "/Game/Saba/Blueprints/Components/AbilityTree/DA_Skill_N2.DA_Skill_N2" "/Game/Saba/Blueprints/Components/AbilityTree/DA_Skill_N3.DA_Skill_N3" "/Game/Saba/Blueprints/Components/AbilityTree/DA_Skill_N4.DA_Skill_N4"))
  (Variables|Default|SetHpAbilities (Utilities|Array|MakeArray "/Game/Saba/Blueprints/Components/AbilityTree/DA_Skill_H1.DA_Skill_H1" "/Game/Saba/Blueprints/Components/AbilityTree/DA_Skill_H2.DA_Skill_H2"))
  (Variables|Default|SetShieldAbilities (Utilities|Array|MakeArray "/Game/Saba/Blueprints/Components/AbilityTree/DA_Skill_S1.DA_Skill_S1" "/Game/Saba/Blueprints/Components/AbilityTree/DA_Skill_S2.DA_Skill_S2"))
  (Variables|Default|SetDefenceAbilities (Utilities|Array|MakeArray "/Game/Saba/Blueprints/Components/AbilityTree/DA_Skill_D1.DA_Skill_D1" "/Game/Saba/Blueprints/Components/AbilityTree/DA_Skill_D2.DA_Skill_D2" "/Game/Saba/Blueprints/Components/AbilityTree/DA_Skill_D3.DA_Skill_D3"))
  (Variables|Default|SetOffenceAbilities (Utilities|Array|MakeArray "/Game/Saba/Blueprints/Components/AbilityTree/DA_Skill_O1.DA_Skill_O1" "/Game/Saba/Blueprints/Components/AbilityTree/DA_Skill_O2.DA_Skill_O2")))

(fn GetSkillState
  (params (SkillNode :type PDA%20Skill%20Node%20Object%20Reference))
  (if (GameplayTags|HasTag (Variables|Default|GetUnlockedSkills) (Variables|/Game/Saba/Blueprints/Components/AbilityTree/PDA_SkillNode.PDA_SkillNode_C|GetID SkillNode) true)
    (return "NewEnumerator1")
    (elif (GameplayTags|HasAllTags (Variables|Default|GetUnlockedSkills) (Variables|/Game/Saba/Blueprints/Components/AbilityTree/PDA_SkillNode.PDA_SkillNode_C|GetPrerequisites SkillNode))
      (return "NewEnumerator2")
      (else
        (return "NewEnumerator0")))))

(fn UnlockNode
  (params (SkillNode :type PDA%20Skill%20Node%20Object%20Reference))
  (bind _status (CallFunction|GetSkillState SkillNode))
  (if (Utilities|Enum|Equal(Enum) _status "NewEnumerator2")
    (if (> (Variables|Default|GetAvailablePoints) 0)
      (Variables|Default|SetAvailablePoints (- (Variables|Default|GetAvailablePoints) 1))
      (GameplayTags|AddGameplayTag (Variables|Default|GetUnlockedSkills) (Variables|/Game/Saba/Blueprints/Components/AbilityTree/PDA_SkillNode.PDA_SkillNode_C|GetID SkillNode) :!class /Script/GameplayTags.BlueprintGameplayTagLibrary)
      (return true)
      (else
        (return false)))
    (else
      (return false))))

(fn AddAbilityPoint
  (params (Points :type Integer))
  (Variables|Default|SetAvailablePoints (+ Points (Variables|Default|GetAvailablePoints))))

(fn UnlockElemental
  (params (Elemental :type E_ElementalType%20Enum :default "NewEnumerator0"))
  (if (not (Utilities|Array|ContainsItem (Variables|Default|GetUnlockedElementals) Elemental))
    (Utilities|Array|Add (Variables|Default|GetUnlockedElementals) Elemental)))

(fn GetAbilitySet
  (params (Elemental :type E_ElementalType%20Enum :default "NewEnumerator0"))
  (Utilities|FlowControl|Sequence
    (:then_0
      ;[0.15 0.15 0.15 0.5] Elementals
      (for _array_element (Utilities|Select :Index Elemental :NewEnumerator0 (Variables|Default|GetFireAbilities) :NewEnumerator1 (Variables|Default|GetElectroAbilities) :NewEnumerator2 (Variables|Default|GetNecroAbilities) :NewEnumerator3 0)
        (bind _unlocked (CallFunction|IsAbilityUnlocked _array_element))
        (if _unlocked
          (switch int (Variables|/Game/Saba/Blueprints/Components/AbilitySystem/PDA_SpecialAbility.PDA_SpecialAbility_C|GetRank (Variables|/Game/Saba/Blueprints/Components/AbilityTree/PDA_SkillNode.PDA_SkillNode_C|GetAbility%20Ref _array_element))
            (:0
              (LocalVariables|SetDefaultAbility (Variables|/Game/Saba/Blueprints/Components/AbilityTree/PDA_SkillNode.PDA_SkillNode_C|GetAbility%20Ref _array_element)))
            (:1
              (LocalVariables|SetLightAbility (Variables|/Game/Saba/Blueprints/Components/AbilityTree/PDA_SkillNode.PDA_SkillNode_C|GetAbility%20Ref _array_element)))
            (:2
              (bind _ability (CallFunction|GetHigherAbility (LocalVariables|GetHeavyAbility) (Variables|/Game/Saba/Blueprints/Components/AbilityTree/PDA_SkillNode.PDA_SkillNode_C|GetAbility%20Ref _array_element) :!label _label))
              (LocalVariables|SetHeavyAbility _ability))
            (:3
              (goto _label))))))
    (:then_1
      ;[0.15 0.15 0.15 0.5] Hp
      (for _array_element_2 (Variables|Default|GetHpAbilities)
        (bind _unlocked_2 (CallFunction|IsAbilityUnlocked _array_element_2))
        (if _unlocked_2
          (bind _ability_2 (CallFunction|GetHigherAbility (LocalVariables|GetHpAbility) (Variables|/Game/Saba/Blueprints/Components/AbilityTree/PDA_SkillNode.PDA_SkillNode_C|GetAbility%20Ref _array_element_2)))
          (LocalVariables|SetHpAbility _ability_2))))
    (:then_2
      ;[0.15 0.15 0.15 0.5] Shield
      (for _array_element_3 (Variables|Default|GetShieldAbilities)
        (bind _unlocked_3 (CallFunction|IsAbilityUnlocked _array_element_3))
        (if _unlocked_3
          (bind _ability_3 (CallFunction|GetHigherAbility (LocalVariables|GetShieldAbility) (Variables|/Game/Saba/Blueprints/Components/AbilityTree/PDA_SkillNode.PDA_SkillNode_C|GetAbility%20Ref _array_element_3)))
          (LocalVariables|SetShieldAbility _ability_3))))
    (:then_3
      ;[0.15 0.15 0.15 0.5] Passive Defence
      (for _array_element_4 (Variables|Default|GetDefenceAbilities)
        (bind _unlocked_4 (CallFunction|IsAbilityUnlocked _array_element_4))
        (if _unlocked_4
          (Utilities|Array|Add (LocalVariables|GetPassiveAbilities) (Variables|/Game/Saba/Blueprints/Components/AbilityTree/PDA_SkillNode.PDA_SkillNode_C|GetAbility%20Ref _array_element_4)))))
    (:then_4
      ;[0.15 0.15 0.15 0.5] Passive Offence
      (for _array_element_5 (Variables|Default|GetOffenceAbilities)
        (bind _unlocked_5 (CallFunction|IsAbilityUnlocked _array_element_5))
        (if _unlocked_5
          (Utilities|Array|Add (LocalVariables|GetPassiveAbilities) (Variables|/Game/Saba/Blueprints/Components/AbilityTree/PDA_SkillNode.PDA_SkillNode_C|GetAbility%20Ref _array_element_5)))))
    (:then_5
      ;[0.15 0.15 0.15 0.5] Return
      (return (Utilities|Struct|MakeS_AbilitySet (LocalVariables|GetDefaultAbility) (LocalVariables|GetLightAbility) (LocalVariables|GetHeavyAbility) (LocalVariables|GetHpAbility) (LocalVariables|GetShieldAbility) (LocalVariables|GetPassiveAbilities))))))

(fn IsAbilityUnlocked
  (params (SkillNode :type PDA%20Skill%20Node%20Object%20Reference))
  (bind _status (CallFunction|GetSkillState SkillNode))
  (return (Utilities|Enum|Equal(Enum) _status "NewEnumerator1")))

(fn GetHigherAbility
  (params (ExistingAbility :type PDA%20Special%20Ability%20Object%20Reference) (NewAbility :type PDA%20Special%20Ability%20Object%20Reference))
  (Utilities|IsValid ExistingAbility
    (:Is%20Valid
      (if (< (Variables|/Game/Saba/Blueprints/Components/AbilitySystem/PDA_SpecialAbility.PDA_SpecialAbility_C|GetRank ExistingAbility) (Variables|/Game/Saba/Blueprints/Components/AbilitySystem/PDA_SpecialAbility.PDA_SpecialAbility_C|GetRank NewAbility))
        _
        (else
          (return ExistingAbility))))
    (:Is%20Not%20Valid
      _))
  (return NewAbility))