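; Sword weapon component that spawns and attaches the sword to the character and runs its combo and charged attacks.
; An aimed attack with charge plays the charge montage; otherwise a combo starts from the default or aim-specific config.
; Montage notify windows gate jumps to the next combo section and toggle root-motion rotation.
; Weapon hooks set the sword's aim/charge state, enable collision on attack and disable it when attacks end.
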(event Custom|ComboAttack
  (bind (_name _montage) (Utilities|StepSection))
  (bind (_name_2 _montage_2) (Utilities|StepSection))
  ;[0.15 0.15 0.15 0.5] Combo attacking
  ;;[0.15 0.15 0.15 0.5] Is first attack
  (if (== (Variables|Default|GetComboStep) 0)
    (bind _montage_3 (CallFunction|GetComboMontage))
    (Variables|Default|SetCurrentComboConfig _montage_3)
    ;;[0.15 0.15 0.15 0.5] Initial attack
    (Variables|Default|SetComboStep (Utilities|Increment (Variables|Default|GetComboStep)))
    (bind _skeleton (Default|GetActiveSkeleton (Variables|Default|GetCharacter%20Ref)))
    (bind _notifyname (Animation|Montage|PlayMontage _skeleton _montage_2 1.0 0.0 _name_2 false)
      (:OnCompleted
        (CallFunction|ComboEnd :!label _label)
        (CallFunction|DoEndAttack)
        (Default|UpdateMovementSpeed (Variables|Default|GetCharacter%20Ref)))
      (:OnInterrupted
        (goto _label))
      (:OnNotifyBegin
        (switch name _notifyname
          (:ComboWindow
            (CallFunction|OnComboWindow true))
          (:RotateWindow
            (CallFunction|OnRotateWindow true))))
      (:OnNotifyEnd
        (switch name _notifyname
          (:ComboWindow
            (CallFunction|OnComboWindow false)
            (CallFunction|DoEndAttack))
          (:RotateWindow
            (CallFunction|OnRotateWindow false)))))
    (else
      ;;[0.15 0.15 0.15 0.5] Combo attack
      (if (Variables|Default|GetIsComboWindow)
        (Variables|Default|SetComboStep (Utilities|Increment (Variables|Default|GetComboStep)))
        (Ability|Animation|MontageJumptoSection (Components|SkeletalMesh|GetAnimInstance (Variables|/Script/Engine.Character|GetMesh (Variables|Default|GetCharacter%20Ref))) _name _montage)
        (Default|ToggleRootMotionRotation (Variables|Default|GetCharacter%20Ref) false)))))

(event Custom|ComboEnd
  ;[0.15 0.15 0.15 0.5] Combo attacking
  (Variables|Default|SetComboStep 0)
  (Variables|Default|SetIsComboWindow false)
  (Variables|Default|SetCurrentComboConfig 0))

(event Custom|OnRotateWindow
  (params (Open :type Boolean))
  (bind _character_ref (Variables|Default|GetCharacter%20Ref))
  ;[0.15 0.15 0.15 0.5] Combo attacking
  (if Open
    (Default|ToggleRootMotionRotation _character_ref true)
    (else
      (Default|ToggleRootMotionRotation _character_ref false))))

(event Custom|OnComboWindow
  (params (Open :type Boolean))
  ;[0.15 0.15 0.15 0.5] Combo attacking
  (if Open
    (Variables|Default|SetIsComboWindow true)
    (else
      (Variables|Default|SetIsComboWindow false))))

(event Custom|LaunchAttack
  (if (and (> (Variables|/Game/Saba/Blueprints/Weapons/BP_BaseSword.BP_BaseSword_C|GetChargeLevel (Variables|Default|GetSword%20Ref)) 0.0) (Variables|Default|GetIsAiming))
    (bind _skeleton (Default|GetActiveSkeleton (Variables|Default|GetCharacter%20Ref)))
    (Animation|Montage|PlayMontage _skeleton (Variables|Default|GetChargeAttackMontage) 1.0 0.0 "None" false
      (:OnCompleted
        _)
      (:OnInterrupted
        _))
    (CallFunction|DoEndAttack)
    (else
      (CallFunction|ComboAttack))))

(event EventEquipWeapon
  (Utilities|IsValid (Variables|Default|GetSword%20Ref)
    (:Is%20Not%20Valid
      (CallFunction|EquipSword))))

(event EventUnequipWeapon
  (Utilities|IsValid (Variables|Default|GetSword%20Ref)
    (:Is%20Valid
      (CallFunction|UnequipSword))))

(fn EquipSword
  (bind _character_ref (Variables|Default|GetCharacter%20Ref))
  (bind _returnvalue (Game|SpawnActorfromClass (Variables|Default|GetSwordClass) (Math|Transform|MakeTransform "0, 0, 0" "0, 0, 0" "1.000000,1.000000,1.000000") "Undefined" "MultiplyWithRoot" 0 (Variables|Default|GetHitPerAttack) false (Variables|Default|GetTrailSocket) _character_ref _character_ref))
  (bind _output_get (Variables|Default|SetSword%20Ref _returnvalue))
  (bind _skeleton (Default|GetAttachSkeleton (Variables|Default|GetCharacter%20Ref)))
  (Transformation|AttachComponentToComponent _output_get _skeleton (Variables|Default|GetSwordSocket) "SnapToTarget" "SnapToTarget" "SnapToTarget" true)
  (Default|ChangeElement (Variables|Default|GetSword%20Ref) (Variables|Default|GetElement))
  (Default|DisableCollision (Variables|Default|GetSword%20Ref))
  (EventDispatchers|BindEventtoOnHit (Variables|Default|GetSword%20Ref) (EventDispatchers|CreateEvent (Variables|Default|GetCharacter%20Ref) :!event ApplyHit)))

(fn UnequipSword
  (bind _sword_ref (Variables|Default|GetSword%20Ref)
    (:then
      (Actor|DestroyActor _sword_ref))
    (:else)))

(fn DoAttack
  (bind _sword_ref (Variables|Default|GetSword%20Ref)
    (:then
      (Default|EnableCollision _sword_ref)
      (bind _charge (CallFunction|GetChargeLevel))
      (Default|Attack (Variables|Default|GetSword%20Ref) _charge))
    (:else)))

(fn DoEndAttack
  (CallFunction|AttackEnd)
  (bind _sword_ref (Variables|Default|GetSword%20Ref)
    (:then
      (Default|DisableCollision _sword_ref))
    (:else)))

(fn GetComboMontage
  (bind _isaiming (Variables|Default|GetIsAiming))
  (bind _defaultcomboconfig (Variables|Default|GetDefaultComboConfig))
  (bind _alternatecombomontage (Variables|Default|GetAlternateComboMontage))
  (bind _returnvalue (select _isaiming _alternatecombomontage _defaultcomboconfig))
  (return (select (Utilities|IsValid _returnvalue) _returnvalue (Variables|Default|GetDefaultComboConfig))))

(fn WeaponAimStart
  (Variables|/Game/Saba/Blueprints/Weapons/BP_BaseSword.BP_BaseSword_C|SetState (Variables|Default|GetSword%20Ref) "NewEnumerator1")
  (return))

(fn WeaponAimEnd
  (Variables|/Game/Saba/Blueprints/Weapons/BP_BaseSword.BP_BaseSword_C|SetState (Variables|Default|GetSword%20Ref) "NewEnumerator0")
  (return))

(fn WeaponChargeStart
  (Variables|/Game/Saba/Blueprints/Weapons/BP_BaseSword.BP_BaseSword_C|SetState (Variables|Default|GetSword%20Ref) "NewEnumerator2")
  (bind _result (Default|IsChargeVfxAvailable (Variables|Default|GetCharacter%20Ref)))
  (Variables|/Game/Saba/Blueprints/Weapons/BP_Weapon.BP_Weapon_C|SetIsOvercharge (Variables|Default|GetSword%20Ref) _result)
  (return))

(fn WeaponChargeEnd
  (Variables|/Game/Saba/Blueprints/Weapons/BP_BaseSword.BP_BaseSword_C|SetState (Variables|Default|GetSword%20Ref) "NewEnumerator0")
  (return))

(fn WeaponAttackStart
  (CallFunction|DoAttack)
  (return))

(fn WeaponAttackEnd
  (CallFunction|LaunchAttack)
  (return))

(fn GetChargeWeapon
  (return (Variables|Default|GetSword%20Ref)))

(fn GetAttackWeapon
  (return (Variables|Default|GetSword%20Ref)))

(fn CanCharge
  (return (not (Variables|Default|GetIsCharging))))

(fn CanJump
  (return (and (not (Variables|Default|GetIsAttacking)) (or (== (Variables|Default|GetComboStep) 0) (Variables|Default|GetIsComboWindow)))))