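; Base weapon system component for a character, handling the aim, charge and attack cycle and equipping or unequipping on component activation.
; Aiming switches character rotation to follow the controller; a looping timer builds charge time, marking the attack weapon charged at full charge.
; Attacks fire only while charging, and element changes pass to both charge and attack weapons.
; Weapon getters, action hooks and CanCharge are empty stubs, apparently for child components to override.
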(event Custom|ComponentActivated
  (params (Component :type Actor%20Component%20Object%20Reference) (bReset :type Boolean))
  ;[0.15 0.15 0.15 0.5] Init
  (CallFunction|EquipWeapon))

(event Custom|ComponentDeactivated
  (params (Component :type Actor%20Component%20Object%20Reference))
  ;[0.15 0.15 0.15 0.5] Init
  (CallFunction|UnequipWeapon))

(event Custom|IncreaseCharge
  ;[0.15 0.15 0.15 0.5] Charging
  (if (Variables|Default|GetIsAiming)
    (bind _output_get (Variables|Default|SetChargeTime (+ (Variables|Default|GetChargeTime) (Variables|Default|GetChargeTimeIncrement))))
    (Development|PrintString (Utilities|String|ToString(Float) _output_get))
    (bind _chargeweapon (CallFunction|GetChargeWeapon))
    (if (<= (Variables|/Game/Saba/Blueprints/Weapons/BP_Weapon.BP_Weapon_C|GetFullChargeTime _chargeweapon) (Variables|Default|GetChargeTime))
      (bind _attackweapon (CallFunction|GetAttackWeapon))
      (if (not (Variables|/Game/Saba/Blueprints/Weapons/BP_Weapon.BP_Weapon_C|GetIsCharged _attackweapon))
        (Default|WeaponCharged _attackweapon true)))))

(event EventBeginPlay
  ;[0.15 0.15 0.15 0.5] Init
  (bind _asbp_base_character (Utilities|Casting|CastToBP_BaseCharacter (Components|GetOwner)))
  (Variables|Default|SetCharacter%20Ref _asbp_base_character)
  (Variables|Default|SetDefaultRotationRate (Variables|/Script/Engine.CharacterMovementComponent|GetRotationRate (Variables|/Script/Engine.Character|GetCharacterMovement (Variables|Default|GetCharacter%20Ref))))
  (Components|Activation|BindEventtoOnComponentActivated (delegate Custom|ComponentActivated))
  (EventDispatchers|BindEventtoOnComponentDeactivated (delegate Custom|ComponentDeactivated)))

(event EventAimEnd
  (bind _character_ref (Variables|Default|GetCharacter%20Ref))
  (bind _charactermovement (Variables|/Script/Engine.Character|GetCharacterMovement _character_ref))
  ;[0.15 0.15 0.15 0.5] Aiming
  (Variables|Default|SetIsAiming false)
  (Variables|/Script/Engine.CharacterMovementComponent|SetbOrientRotationToMovement _charactermovement true)
  (Variables|/Script/Engine.CharacterMovementComponent|SetbUseControllerDesiredRotation _charactermovement false)
  (Variables|/Script/Engine.CharacterMovementComponent|SetRotationRate _charactermovement (Variables|Default|GetDefaultRotationRate))
  (CallFunction|WeaponAimEnd)
  (CallFunction|ChargeEnd)
  (Default|CallOnAimEnd))

(event EventSetChargeMultiplier
  (params (Multiplier :type Float%20%28double-precision%29))
  ;[0.15 0.15 0.15 0.5] Charging
  (Variables|Default|SetChargeTimeMultiplier Multiplier))

(event EventChangeElement
  (params (ElementType :type E_ElementalType%20Enum :default "NewEnumerator0"))
  ;[0.15 0.15 0.15 0.5] Elemenal
  (Variables|Default|SetElement ElementType)
  (Utilities|FlowControl|Sequence
    (:then_0
      (bind _chargeweapon (CallFunction|GetChargeWeapon))
      (Utilities|IsValid _chargeweapon
        (:Is%20Valid
          (Default|ChangeElement _chargeweapon (Variables|Default|GetElement)))))
    (:then_1
      (bind _attackweapon (CallFunction|GetAttackWeapon))
      (Utilities|IsValid _attackweapon
        (:Is%20Valid
          (Default|ChangeElement _attackweapon (Variables|Default|GetElement)))))))

(event EventAttackEnd
  ;[0.15 0.15 0.15 0.5] Attacking
  (Variables|Default|SetIsAttacking false)
  (if (Variables|Default|GetIsAiming)
    (CallFunction|AimStart)
    (if (Variables|Default|GetIsAwaitingCharge)
      (CallFunction|ChargeStart))))

(event EventAttackStart
  ;[0.15 0.15 0.15 0.5] Attacking
  (if (Variables|Default|GetIsCharging)
    (Variables|Default|SetIsAttacking true)
    (CallFunction|WeaponAttackStart)
    (CallFunction|ChargeEnd)
    (CallFunction|WeaponAttackEnd)))

(event EventChargeEnd
  ;[0.15 0.15 0.15 0.5] Charging
  (Variables|Default|SetIsAwaitingCharge false)
  (Variables|Default|SetIsCharging false)
  (Variables|Default|SetChargeTime 0.0)
  (Utilities|Time|ClearandInvalidateTimerbyHandle (Variables|Default|GetChargeTimer))
  (CallFunction|WeaponChargeEnd)
  (Default|CallOnChargeEnd)
  (bind _attackweapon (CallFunction|GetAttackWeapon))
  (Utilities|IsValid _attackweapon
    (:Is%20Valid
      (Default|WeaponCharged _attackweapon false))))

(event EventChargeStart
  ;[0.15 0.15 0.15 0.5] Charging
  (bind _result (CallFunction|CanCharge))
  (if _result
    (Variables|Default|SetIsAwaitingCharge false)
    (Variables|Default|SetIsCharging true)
    (bind _returnvalue (Utilities|Time|SetTimerbyEvent (delegate Custom|IncreaseCharge) (/ (Variables|Default|GetChargeTimeInterval) (Variables|Default|GetChargeTimeMultiplier)) true))
    (Variables|Default|SetChargeTimer _returnvalue)
    (CallFunction|WeaponChargeStart)
    (Default|CallOnChargeStart)
    (else
      (Variables|Default|SetIsAwaitingCharge true))))

(event EventAimStart
  (bind _character_ref (Variables|Default|GetCharacter%20Ref))
  (bind _charactermovement (Variables|/Script/Engine.Character|GetCharacterMovement _character_ref))
  ;[0.15 0.15 0.15 0.5] Aiming
  (Variables|Default|SetIsAiming true)
  (Variables|/Script/Engine.CharacterMovementComponent|SetbOrientRotationToMovement _charactermovement false)
  (Variables|/Script/Engine.CharacterMovementComponent|SetbUseControllerDesiredRotation _charactermovement true)
  (Variables|/Script/Engine.CharacterMovementComponent|SetRotationRate _charactermovement (Variables|Default|GetAimRotationRate))
  (CallFunction|WeaponAimStart)
  (Default|CallOnAimStart))

(fn GetChargeWeapon
  (return 0))

(fn GetAttackWeapon
  (return 0))

(fn WeaponAttackStart)

(fn WeaponAttackEnd)

(fn WeaponChargeStart)

(fn WeaponChargeEnd)

(fn WeaponAimStart)

(fn WeaponAimEnd)

(fn CanCharge
  (return false))

(fn CanJump
  (return false))

(fn GetChargeLevel
  (bind _chargeweapon (CallFunction|GetChargeWeapon))
  (return (Math|Float|Clamp(Float) (Math|Float|NormalizetoRange (Variables|Default|GetChargeTime) 0.0 (Variables|/Game/Saba/Blueprints/Weapons/BP_Weapon.BP_Weapon_C|GetFullChargeTime _chargeweapon)))))

(fn GetCurrentWeapon
  (bind _attackweapon (CallFunction|GetAttackWeapon))
  (return _attackweapon (Utilities|IsValid _attackweapon)))