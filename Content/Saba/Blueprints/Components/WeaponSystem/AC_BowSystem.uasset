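; Bow weapon component that lets a character equip a bow, aim, charge and shoot elemental arrows.
; It overrides weapon hooks to set the bow's state, spawning a socketed arrow on aim start and destroying it on aim end.
; Attacking launches the arrow toward a camera trace target with charge-based strength and binds its hit event.
; Bow and character shoot montages then play before the attack ends.
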(event Custom|Event%20WeaponAttackEnd
  (Animation|Montage|PlayMontage (Variables|/Game/Saba/Blueprints/Weapons/BP_Bow.BP_Bow_C|GetMesh (Variables|Default|GetBow%20Ref)) (Variables|Default|GetBowShootMontage)
    (:then
      (Animation|Montage|PlayMontage (Variables|/Script/Engine.Character|GetMesh (Variables|Default|GetCharacter%20Ref)) (Variables|Default|GetCharacterShootMontage)
        (:OnCompleted
          _)
        (:OnInterrupted
          _))
      (CallFunction|AttackEnd))))

(event EventEquipWeapon
  (Utilities|IsValid (Variables|Default|GetBow%20Ref)
    (:Is%20Not%20Valid
      (CallFunction|EquipBow))))

(event EventUnequipWeapon
  (Utilities|IsValid (Variables|Default|GetBow%20Ref)
    (:Is%20Valid
      (CallFunction|UnequipBow))))

(fn EquipBow
  (bind _character_ref (Variables|Default|GetCharacter%20Ref))
  (bind _returnvalue (Game|SpawnActorfromClass (Variables|Default|GetBowClass) (Math|Transform|MakeTransform "0, 0, 0" "0, 0, 0" "1.000000,1.000000,1.000000") "Undefined" "MultiplyWithRoot" 0 false (Variables|Default|GetBowSocket) _character_ref _character_ref))
  (bind _output_get (Variables|Default|SetBow%20Ref _returnvalue))
  (Transformation|AttachComponentToComponent _output_get (Variables|/Script/Engine.Character|GetMesh (Variables|Default|GetCharacter%20Ref)) (Variables|Default|GetBowSocket) "SnapToTarget" "SnapToTarget" "SnapToTarget" true))

(fn UnequipBow
  (CallFunction|UnequipArrow)
  (bind _bow_ref (Variables|Default|GetBow%20Ref)
    (:then
      (Actor|DestroyActor _bow_ref))
    (:else)))

(fn EquipArrow
  (bind _character_ref (Variables|Default|GetCharacter%20Ref))
  (Utilities|IsValid (Variables|Default|GetArrow%20Ref)
    (:Is%20Not%20Valid
      (bind _result (Default|IsChargeVfxAvailable (Variables|Default|GetCharacter%20Ref)))
      (bind _returnvalue (Game|SpawnActorfromClass (Variables|Default|GetArrowClass) (Math|Transform|MakeTransform "0, 0, 0" "0, 0, 0" "1.000000,1.000000,1.000000") "Undefined" "MultiplyWithRoot" 0 _result (Variables|Default|GetArrowSocket) _character_ref _character_ref))
      (bind _output_get (Variables|Default|SetArrow%20Ref _returnvalue))
      (Transformation|AttachComponentToComponent _output_get (Variables|/Script/Engine.Character|GetMesh (Variables|Default|GetCharacter%20Ref)) (Variables|Default|GetArrowSocket) "KeepRelative" "KeepRelative" "KeepRelative" true)
      (Default|ChangeElement (Variables|Default|GetArrow%20Ref) (Variables|Default|GetElement)))))

(fn UnequipArrow
  (bind _arrow_ref (Variables|Default|GetArrow%20Ref)
    (:then
      (Actor|DestroyActor _arrow_ref)
      (Variables|Default|SetArrow%20Ref 0))
    (:else)))

(fn ShootArrow
  (bind _arrow_ref (Variables|Default|GetArrow%20Ref)
    (:then
      (Transformation|DetachFromActor _arrow_ref "KeepWorld" "KeepWorld" "KeepWorld")
      (bind _direction (CallFunction|CalculateArrowDirection))
      (bind _charge (CallFunction|GetChargeLevel))
      (Default|Shoot _arrow_ref _direction _charge)
      (EventDispatchers|BindEventtoOnHit (Variables|Default|GetArrow%20Ref) (EventDispatchers|CreateEvent (Variables|Default|GetCharacter%20Ref) :!event ApplyHit))
      (Variables|Default|SetArrow%20Ref 0))
    (:else)))

(fn CalculateArrowDirection
  (bind _character_ref (Variables|Default|GetCharacter%20Ref))
  (bind _returnvalue (Actor|GetComponentbyClass _character_ref "/Script/Engine.CameraComponent"))
  (bind _returnvalue_2 (Transformation|GetWorldLocation _returnvalue))
  (bind (_outhit _returnvalue_3) (Collision|LineTraceByChannel _returnvalue_2 (+ _returnvalue_2 (* (Math|Vector|GetForwardVector _returnvalue) 1e+04)) "TraceTypeQuery1" false 0 "None"))
  (bind _arrow_ref (Variables|Default|GetArrow%20Ref)
    (:then
      (return (Math|Vector|GetUnitDirection(Vector) (Transformation|GetActorLocation _arrow_ref) (Math|Vector|SelectVector (.Location (Collision|BreakHitResult _outhit)) (.TraceEnd (Collision|BreakHitResult _outhit)) _returnvalue_3))))
    (:else)))

(fn WeaponAimStart
  (Variables|/Game/Saba/Blueprints/Weapons/BP_Bow.BP_Bow_C|SetState (Variables|Default|GetBow%20Ref) "NewEnumerator1")
  (CallFunction|EquipArrow)
  (return))

(fn WeaponAimEnd
  (Variables|/Game/Saba/Blueprints/Weapons/BP_Bow.BP_Bow_C|SetState (Variables|Default|GetBow%20Ref) "NewEnumerator0")
  (CallFunction|UnequipArrow)
  (return))

(fn WeaponChargeStart
  (Variables|/Game/Saba/Blueprints/Weapons/BP_Bow.BP_Bow_C|SetState (Variables|Default|GetBow%20Ref) "NewEnumerator2")
  (return))

(fn WeaponChargeEnd
  (Variables|/Game/Saba/Blueprints/Weapons/BP_Bow.BP_Bow_C|SetState (Variables|Default|GetBow%20Ref) "NewEnumerator0")
  (return))

(fn WeaponAttackStart
  (CallFunction|ShootArrow)
  (return))

(fn WeaponAttackEnd
  (CallFunction|EventWeaponAttackEnd)
  (return))

(fn GetChargeWeapon
  (return (Variables|Default|GetBow%20Ref)))

(fn GetAttackWeapon
  (return (Variables|Default|GetArrow%20Ref)))

(fn CanCharge
  (return (Math|Boolean|ANDBoolean (not (Variables|Default|GetIsCharging)) (not (Variables|Default|GetIsAttacking)) (Variables|Default|GetIsAiming))))

(fn CanJump
  (return true))