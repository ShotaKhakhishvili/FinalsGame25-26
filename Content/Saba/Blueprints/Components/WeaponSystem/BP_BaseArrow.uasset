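; BP_BaseArrow is the base arrow projectile of the weapon system, launched with a direction and charge strength.
; Shoot stores the charge, then DoShoot adds a projectile movement component at runtime, scaling speed up from min to max and gravity down from max to min as strength rises.
; Hit broadcasts OnHit with the hit result, weapon, charge, direction and element, which ChangeElement sets.
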(event Custom|Shoot
  (params (Direction :type Vector) (Strength :type Float%20%28double-precision%29))
  (bind _output_get (Variables|Default|SetChargeLevel Strength))
  (CallFunction|DoShoot Direction _output_get))

(event EventBeginPlay)

(event Collision|EventActorBeginOverlap
  (params (OtherActor :type Actor%20Object%20Reference)))

(event EventTick
  (params (DeltaSeconds :type Float%20%28single-precision%29)))

(event Collision|EventHit
  (params (MyComp :type Primitive%20Component%20Object%20Reference) (Other :type Actor%20Object%20Reference) (OtherComp :type Primitive%20Component%20Object%20Reference) (bSelfMoved :type Boolean) (HitLocation :type Vector :default "0, 0, 0") (HitNormal :type Vector :default "0, 0, 0") (NormalImpulse :type Vector :default "0, 0, 0") (Hit :type Hit%20Result%20Structure%20%28by%20ref%29))
  (Default|CallOnHit Hit self (Variables|Default|GetChargeLevel) (Variables|Default|GetDirection) (Variables|Default|GetElemental)))

(event EventChangeElement
  (params (ElementType :type E_ElementalType%20Enum :default "NewEnumerator0"))
  (Variables|Default|SetElemental ElementType))

(fn ConstructionScript)

(fn DoShoot
  (params (Direction :type Vector) (Strength :type Float%20%28double-precision%29))
  (bind _output_get (Variables|Default|SetDirection Direction))
  (bind _returnvalue (AddComponent|AddProjectileMovementComponent))
  (bind _output_get_2 (Variables|Default|SetProjectileMovementComponent _returnvalue))
  (Variables|/Script/Engine.MovementComponent|SetVelocity _output_get_2 (* _output_get (Math|Float|Lerp (Variables|Default|GetMinSpeed) (Variables|Default|GetMaxSpeed) Strength)))
  (Variables|/Script/Engine.ProjectileMovementComponent|SetProjectileGravityScale _output_get_2 (Math|Float|Lerp (Variables|Default|GetMaxGravityScale) (Variables|Default|GetMinGravityScale) Strength)))