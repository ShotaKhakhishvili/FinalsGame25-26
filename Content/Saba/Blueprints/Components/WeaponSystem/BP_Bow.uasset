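; BP_Bow is a bow weapon actor that changes its tint to show its current element.
; The construction script creates a dynamic material instance from MI_Quinn_02_Inst on the mesh's first material slot.
; The ChangeElement event stores the new element and calls ApplyElement, which sets the material's Tint parameter for fire, electro or necro.
; The file holds only this visual switch, with no firing or damage logic.
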(event EventBeginPlay)

(event Collision|EventActorBeginOverlap
  (params (OtherActor :type Actor%20Object%20Reference)))

(event EventTick
  (params (DeltaSeconds :type Float%20%28single-precision%29)))

(event EventChangeElement
  (params (ElementType :type E_ElementalType%20Enum :default "NewEnumerator0"))
  (Variables|Default|SetElement ElementType)
  (CallFunction|ApplyElement))

(fn ConstructionScript
  (bind _returnvalue (Rendering|Material|CreateDynamicMaterialInstance (Variables|Default|GetMesh) 0 "/Game/Saba/Materials/MI_Quinn_02_Inst.MI_Quinn_02_Inst" "None" :!class /Script/Engine.PrimitiveComponent))
  (Variables|Default|SetMainMaterialInstance _returnvalue))

(fn ApplyElement
  (bind _mainmaterialinstance (Variables|Default|GetMainMaterialInstance))
  (Utilities|IsValid (Variables|Default|GetMainMaterialInstance)
    (:Is%20Valid
      (switch Utilities|FlowControl|Switch|SwitchonE_ElementalType (Variables|Default|GetElement)
        (:NewEnumerator0
          (Rendering|Material|SetVectorParameterValue _mainmaterialinstance "Tint" "(R=0.369792,G=0.000000,B=0.012882,A=1.000000)" :!class /Script/Engine.MaterialInstanceDynamic))
        (:NewEnumerator1
          (Rendering|Material|SetVectorParameterValue _mainmaterialinstance "Tint" "(R=0.368616,G=0.369792,B=0.000000,A=1.000000)" :!class /Script/Engine.MaterialInstanceDynamic))
        (:NewEnumerator2
          (Rendering|Material|SetVectorParameterValue _mainmaterialinstance "Tint" "(R=0.018463,G=0.000000,B=0.093750,A=1.000000)" :!class /Script/Engine.MaterialInstanceDynamic))))))