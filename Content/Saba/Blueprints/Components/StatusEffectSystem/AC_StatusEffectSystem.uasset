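; Actor component that manages status effects on a BP_BaseCharacter, both permanent passives and timed effects.
; Applying a new status spawns its logic actor, attaches it to the character and triggers the effect; reapplying a timed one only resets its duration.
; Tick counts timed statuses down and, on expiry, removes them and finishes their logic.
; OnEffectsUpdate broadcasts the current status list whenever a logic is added or removed.
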(event EventBeginPlay
  (bind _asbp_base_character (Utilities|Casting|CastToBP_BaseCharacter (Components|GetOwner)))
  (Variables|Default|SetCharacter%20Ref _asbp_base_character))

(event EventTick
  (params (DeltaSeconds :type Float%20%28single-precision%29))
  (bind _keys (Utilities|Map|Keys (Variables|Default|GetActiveStatuses)))
  (for _array_element _keys
    (if (>= (.Value (Utilities|Map|Find (Variables|Default|GetActiveStatuses) _array_element)) 0.0)
      (Utilities|Map|Add (Variables|Default|GetActiveStatuses) _array_element (- (.Value (Utilities|Map|Find (Variables|Default|GetActiveStatuses) _array_element)) DeltaSeconds))
      (else
        (CallFunction|RemoveStatus _array_element)))))

(fn ApplyStatus
  (params (Status :type PDA%20Status%20Effect%20Object%20Reference))
  (if (Variables|/Game/Saba/Blueprints/Components/StatusEffectSystem/PDA_StatusEffect.PDA_StatusEffect_C|GetPermanent Status)
    ;[0.15 0.15 0.15 0.5] Permanent Statuses (Passive abilities)
    (if (not (Utilities|Set|Contains (Variables|Default|GetPermanentStatuses) Status))
      (Utilities|Set|Add (Variables|Default|GetPermanentStatuses) Status)
      (CallFunction|ExecuteStatus Status))
    (else
      ;[0.15 0.15 0.15 0.5] Timed Statuses
      (LocalVariables|SetStatusAlreadyApplied (Utilities|Map|Contains (Variables|Default|GetActiveStatuses) Status))
      (Utilities|Map|Add (Variables|Default|GetActiveStatuses) Status (Variables|/Game/Saba/Blueprints/Components/StatusEffectSystem/PDA_StatusEffect.PDA_StatusEffect_C|GetDuration Status))
      (if (not (LocalVariables|GetStatusAlreadyApplied))
        (CallFunction|ExecuteStatus Status)))))

(fn ExecuteStatus
  (params (Status :type PDA%20Status%20Effect%20Object%20Reference))
  (bind _returnvalue (Game|SpawnActorfromClass (Variables|/Game/Saba/Blueprints/Components/StatusEffectSystem/PDA_StatusEffect.PDA_StatusEffect_C|GetLogicClass Status) (Math|Transform|MakeTransform "0, 0, 0" "0, 0, 0" "1.000000,1.000000,1.000000") "Undefined" "MultiplyWithRoot" 0 (Variables|Default|GetCharacter%20Ref)))
  (Transformation|AttachActorToActor _returnvalue (Variables|Default|GetCharacter%20Ref) "None" "KeepRelative" "KeepRelative" "KeepRelative" true)
  (Utilities|FlowControl|Sequence
    (:then_0
      (Utilities|Map|Add (Variables|Default|GetStatusLogics) Status _returnvalue))
    (:then_1
      (Default|TriggerEffect _returnvalue Status (Variables|Default|GetCharacter%20Ref))
      (bind _keys (Utilities|Map|Keys (Variables|Default|GetStatusLogics)))
      (Default|CallOnEffectsUpdate _keys))))

(fn RemoveStatus
  (params (Status :type PDA%20Status%20Effect%20Object%20Reference))
  (LocalVariables|SetStatusToRemove Status)
  (Utilities|FlowControl|Sequence
    (:then_0
      (Utilities|Map|Remove (Variables|Default|GetActiveStatuses) (LocalVariables|GetStatusToRemove)))
    (:then_1
      (LocalVariables|SetLogicToRemove (.Value (Utilities|Map|Find (Variables|Default|GetStatusLogics) (LocalVariables|GetStatusToRemove)))))
    (:then_2
      (Utilities|IsValid (LocalVariables|GetLogicToRemove)
        (:Is%20Valid
          (Utilities|Map|Remove (Variables|Default|GetStatusLogics) (LocalVariables|GetStatusToRemove))
          (Default|FinishEffect (LocalVariables|GetLogicToRemove))
          (bind _keys (Utilities|Map|Keys (Variables|Default|GetStatusLogics)))
          (Default|CallOnEffectsUpdate _keys))))))