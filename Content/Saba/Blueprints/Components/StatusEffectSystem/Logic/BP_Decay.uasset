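; BP_Decay is a status effect that damages a character over time and slows it while active.
; On trigger it attaches smoke particles to the character's mesh, caches the max walk speed and halves it.
; Each tick subtracts the effect's value from HP through UpdateStats, tagged with an elemental type.
; On finish it destroys the particles and restores the cached speed, with all three overrides calling their parent versions.
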(fn ConstructionScript)

(fn TriggerEffect
  (params (StatusEffect%20Ref :type PDA%20Status%20Effect%20Object%20Reference) (Character%20Ref :type BP%20Base%20Character%20Object%20Reference))
  (bind _charactermovement (Variables|/Script/Engine.Character|GetCharacterMovement Character%20Ref))
  (|CallParentFunction StatusEffect%20Ref Character%20Ref)
  (bind _returnvalue (Effects|SpawnEmitterAttached "/Game/Saba/Particles/P_Smoke.P_Smoke" (Variables|/Script/Engine.Character|GetMesh (Variables|Default|GetCharacter%20Ref)) "None"))
  (Variables|Default|SetEffectParticles _returnvalue)
  (bind _output_get (Variables|Default|SetInitialSpeed (Variables|/Script/Engine.CharacterMovementComponent|GetMaxWalkSpeed _charactermovement)))
  (Variables|/Script/Engine.CharacterMovementComponent|SetMaxWalkSpeed _charactermovement (/ _output_get 2.0)))

(fn FinishEffect
  (|CallParentFunction)
  (Components|DestroyComponent (Variables|Default|GetEffectParticles))
  (Variables|/Script/Engine.CharacterMovementComponent|SetMaxWalkSpeed (Variables|/Script/Engine.Character|GetCharacterMovement (Variables|Default|GetCharacter%20Ref)) (Variables|Default|GetInitialSpeed)))

(fn TickEffect
  (|CallParentFunction)
  (Default|UpdateStats (Variables|Default|GetCharacter%20Ref) (Utilities|Negate (Variables|/Game/Saba/Blueprints/Components/StatusEffectSystem/PDA_StatusEffect.PDA_StatusEffect_C|GetValue (Variables|Default|GetStatusEffect%20Ref))) 0.0 0.0 "NewEnumerator2"))