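; BP_Burn is a burn status effect in the StatusEffectSystem that deals damage over time to the affected character.
; On trigger it runs the parent logic, attaches the P_Fire emitter to the character's mesh and prints a debug message.
; Each tick lowers the character's Hp by the effect's Value through UpdateStats.
; On finish it destroys the fire particles before calling the parent's finish.
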(fn ConstructionScript)

(fn TriggerEffect
  (params (StatusEffect%20Ref :type PDA%20Status%20Effect%20Object%20Reference) (Character%20Ref :type BP%20Base%20Character%20Object%20Reference))
  (|CallParentFunction StatusEffect%20Ref Character%20Ref)
  (bind _returnvalue (Effects|SpawnEmitterAttached "/Game/Saba/Particles/P_Fire.P_Fire" (Variables|/Script/Engine.Character|GetMesh (Variables|Default|GetCharacter%20Ref)) "None"))
  (Variables|Default|SetFireParticles _returnvalue)
  (Development|PrintString "Burning"))

(fn FinishEffect
  (Components|DestroyComponent (Variables|Default|GetFireParticles))
  (|CallParentFunction))

(fn TickEffect
  (|CallParentFunction)
  (Default|UpdateStats (Variables|Default|GetCharacter%20Ref) (Utilities|Negate (Variables|/Game/Saba/Blueprints/Components/StatusEffectSystem/PDA_StatusEffect.PDA_StatusEffect_C|GetValue (Variables|Default|GetStatusEffect%20Ref))) 0.0 0.0 "NewEnumerator0"))