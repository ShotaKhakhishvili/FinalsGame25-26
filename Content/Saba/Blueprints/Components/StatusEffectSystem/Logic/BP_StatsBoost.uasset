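; Status effect logic Blueprint that boosts a character's maximum HP and Mana when triggered.
; TriggerEffect runs the parent logic, then scales both maximums by the effect's Value as a percentage increase, with HP gaining only three quarters of that rate.
; The scaled amounts go to SetMaxStats and also to UpdateStats with a fixed elemental type.
; No removal or revert logic is defined here.
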(fn ConstructionScript)

(fn TriggerEffect
  (params (StatusEffect%20Ref :type PDA%20Status%20Effect%20Object%20Reference) (Character%20Ref :type BP%20Base%20Character%20Object%20Reference))
  (bind _value (Variables|/Game/Saba/Blueprints/Components/StatusEffectSystem/PDA_StatusEffect.PDA_StatusEffect_C|GetValue (Variables|Default|GetStatusEffect%20Ref)))
  (|CallParentFunction StatusEffect%20Ref Character%20Ref)
  (bind (_hp _mana) (Class|BPICharacter|GetMaxStats(Message) (Variables|Default|GetCharacter%20Ref)))
  (Default|SetMaxStats (Variables|Default|GetCharacter%20Ref) (Utilities|Percent _hp (+ (* _value 0.75) 1e+02)) (Utilities|Percent _mana (+ _value 1e+02)))
  (Default|UpdateStats (Variables|Default|GetCharacter%20Ref) (Utilities|Percent _hp (+ (* _value 0.75) 1e+02)) (Utilities|Percent _mana (+ _value 1e+02)) 0.0 "NewEnumerator3"))