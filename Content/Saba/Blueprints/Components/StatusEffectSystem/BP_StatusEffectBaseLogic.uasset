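; Base actor for status effect logic, providing the lifecycle and periodic timing for an effect on a character.
; TriggerEffect stores the effect and character references, and FinishEffect destroys the actor.
; Tick accumulates delta time and calls the empty TickEffect hook when the effect's Interval is reached, carrying over the remainder and firing at most once per frame.
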(event EventTick
  (params (DeltaSeconds :type Float%20%28single-precision%29))
  (bind _output_get (Variables|Default|SetTickCurrent (+ DeltaSeconds (Variables|Default|GetTickCurrent))))
  (if (>= _output_get (Variables|/Game/Saba/Blueprints/Components/StatusEffectSystem/PDA_StatusEffect.PDA_StatusEffect_C|GetInterval (Variables|Default|GetStatusEffect%20Ref)))
    (Variables|Default|SetTickCurrent (- (Variables|Default|GetTickCurrent) (Variables|/Game/Saba/Blueprints/Components/StatusEffectSystem/PDA_StatusEffect.PDA_StatusEffect_C|GetInterval (Variables|Default|GetStatusEffect%20Ref))))
    (CallFunction|TickEffect)))

(fn ConstructionScript)

(fn TriggerEffect
  (params (StatusEffect%20Ref :type PDA%20Status%20Effect%20Object%20Reference) (Character%20Ref :type BP%20Base%20Character%20Object%20Reference))
  (Variables|Default|SetStatusEffect%20Ref StatusEffect%20Ref)
  (Variables|Default|SetCharacter%20Ref Character%20Ref))

(fn FinishEffect
  (Actor|DestroyActor))

(fn TickEffect)