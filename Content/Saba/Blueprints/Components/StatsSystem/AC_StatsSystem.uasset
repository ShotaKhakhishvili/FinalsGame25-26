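; Stats component that tracks HP, mana, XP and level through three additive events.
; AddHp and AddMana clamp their value between zero and its maximum, then broadcast HP, mana and XP through OnStatUpdate.
; AddXp carries overflow past MaxXp into the next level, handling one level-up per call and broadcasting only when a level is gained.
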(event Custom|AddMana
  (params (ManaOffset :type Float%20%28double-precision%29))
  (Variables|Default|SetMana (Math|Float|Clamp(Float) (+ ManaOffset (Variables|Default|GetMana)) 0.0 (Variables|Default|GetMaxMana)))
  (Default|CallOnStatUpdate (Variables|Default|GetHp) (Variables|Default|GetMana) (Variables|Default|GetXp)))

(event Custom|AddXp
  (params (XpOffset :type Float%20%28double-precision%29))
  (bind _output_get (Variables|Default|SetXp (+ XpOffset (Variables|Default|GetXp))))
  (if (>= _output_get (Variables|Default|GetMaxXp))
    (Variables|Default|SetXp (- (Variables|Default|GetXp) (Variables|Default|GetMaxXp)))
    (Variables|Default|SetLevel (+ (Variables|Default|GetLevel) 1))
    (Default|CallOnStatUpdate (Variables|Default|GetHp) (Variables|Default|GetMana) (Variables|Default|GetXp))))

(event Custom|AddHp
  (params (HpOffset :type Float%20%28double-precision%29))
  (Variables|Default|SetHp (Math|Float|Clamp(Float) (+ HpOffset (Variables|Default|GetHp)) 0.0 (Variables|Default|GetMaxHp)))
  (Default|CallOnStatUpdate (Variables|Default|GetHp) (Variables|Default|GetMana) (Variables|Default|GetXp)))