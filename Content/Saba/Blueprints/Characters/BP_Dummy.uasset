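; BP_Dummy is a dummy character that takes stat updates and falls over when its HP runs out.
; On BeginPlay it runs init, component binding and activation calls, then listens for updates from its stats component (ACStatsSystem).
; UpdateStats defers to the parent, then prints the dummy's name and current HP.
; At zero HP or below, KillCharacter simply rolls the mesh 90 degrees onto its side.
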(event Custom|HandleStatUpdate
  (params (HP :type Float%20%28double-precision%29) (Mana :type Float%20%28double-precision%29) (XP :type Float%20%28double-precision%29))
  (if (<= HP 0.0)
    (CallFunction|KillCharacter)))

(event EventBeginPlay
  (CallFunction|InitParams)
  (CallFunction|BindComponentEvents)
  (CallFunction|ActivateComponents)
  (EventDispatchers|BindEventtoOnStatUpdate (Variables|Default|GetAC_StatsSystem) (delegate Custom|HandleStatUpdate)))

(event EventUpdateStats
  (params (Hp :type Float%20%28double-precision%29) (Mana :type Float%20%28double-precision%29) (Xp :type Float%20%28double-precision%29) (Elemental :type E_ElementalType%20Enum :default "NewEnumerator0"))
  (|CallParentFunction Hp Mana Xp Elemental)
  (Development|PrintString (Utilities|String|Append (Utilities|GetDisplayName self) "  ::  " (Utilities|String|ToString(Float) (Variables|/Game/Saba/Blueprints/Components/StatsSystem/AC_StatsSystem.AC_StatsSystem_C|GetHp (Variables|Default|GetAC_StatsSystem))))))

(event EventKillCharacter
  (bind _mesh (Variables|Character|GetMesh))
  (bind _returnvalue (Transformation|GetWorldRotation _mesh))
  (Transformation|SetWorldRotation _mesh (Math|Rotator|MakeRotator 9e+01 (.pitch _returnvalue) (.yaw _returnvalue)) false false))

(fn ConstructionScript
  (|CallParentFunction))