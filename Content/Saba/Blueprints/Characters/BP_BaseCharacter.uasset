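; Base character that acts as a hub for stats, ability tree, abilities, status effects, elements and switchable weapon systems.
; Forwards attack, aim, charge, ability and switch requests to those components, gated by CanSwitchSetting based on aiming and ability state.
; Component callbacks track the element and ability use, auto-aiming for abilities awaiting an attack.
; Walk speed follows sprint and aim state, with airborne changes deferred until landing.
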(event Custom|UpdateMovementSpeed
  ;[0.15 0.15 0.15 0.5] Character movement controlls
  (bind _speed (CallFunction|CalculateWalkingSpeed))
  (Variables|Default|SetCurrentWalkSpeed _speed)
  ;;[0.15 0.15 0.15 0.5] Only update speed when on the ground to not affect speed midair
  (if (not (AI|Components|NavMovement|IsFalling (Variables|Character|GetCharacterMovement)))
    (CallFunction|DoUpdateMovementSpeed)))

(event Custom|AttackStart
  ;[0.15 0.15 0.15 0.5] Attack/Charge
  (bind _attack (CallFunction|CanSwitchSetting))
  (if _attack
    (Default|AttackStart (Variables|Components|GetActiveWeaponSystem))))

(event Custom|AbilityStartCallback
  (params (AwaitingAttack :type Boolean))
  ;[0.15 0.15 0.15 0.5] Ability execution
  (Variables|Default|SetIsUsingAbility true)
  (if AwaitingAttack
    (CallFunction|AimStart)))

(event Custom|AbilityEndCallback
  (params (AwaitingAttack :type Boolean))
  ;[0.15 0.15 0.15 0.5] Ability execution
  (Variables|Default|SetIsUsingAbility false)
  (if AwaitingAttack
    (CallFunction|AimEnd)))

(event Custom|AimStart
  ;[0.15 0.15 0.15 0.5] Aiming
  (Default|AimStart (Variables|Components|GetActiveWeaponSystem))
  (CallFunction|UpdateMovementSpeed))

(event Custom|AimEnd
  ;[0.15 0.15 0.15 0.5] Aiming
  (Default|AimEnd (Variables|Components|GetActiveWeaponSystem))
  (CallFunction|UpdateMovementSpeed))

(event Custom|AimStartCallback
  ;[0.15 0.15 0.15 0.5] Aiming
  (if (Variables|Default|GetIsUsingAbility)
    (bind _weapon (CallFunction|GetCharacterWeapon))
    (Default|ReArmAbility (Variables|Default|GetAC_AbilitySystem) _weapon)))

(event Custom|AimEndCallback
  ;[0.15 0.15 0.15 0.5] Aiming
)

(event Custom|BindComponentEvents
  ;[0.15 0.15 0.15 0.5] Bind events
  (EventDispatchers|BindEventtoOnAbilityStart (Variables|Default|GetAC_AbilitySystem) (EventDispatchers|CreateEvent :!event Custom|AbilityStartCallback))
  (EventDispatchers|BindEventtoOnAbilityEnd (Variables|Default|GetAC_AbilitySystem) (EventDispatchers|CreateEvent :!event Custom|AbilityEndCallback))
  (EventDispatchers|BindEventtoOnElementChanged (Variables|Default|GetAC_ElementalSystem) (EventDispatchers|CreateEvent :!event ChangeElement))
  (EventDispatchers|BindEventtoOnElementChanged (Variables|Default|GetAC_ElementalSystem) (EventDispatchers|CreateEvent (Variables|Default|GetAC_AbilitySystem) :!event ChangeElement))
  (for _array_element (Variables|Components|GetWeaponSystems)
    (EventDispatchers|BindEventtoOnElementChanged (Variables|Default|GetAC_ElementalSystem) (EventDispatchers|CreateEvent _array_element :!event ChangeElement))
    (EventDispatchers|BindEventtoOnAimStart _array_element (EventDispatchers|CreateEvent :!event Custom|AimStartCallback))
    (EventDispatchers|BindEventtoOnAimEnd _array_element (EventDispatchers|CreateEvent :!event Custom|AimEndCallback))
    (EventDispatchers|BindEventtoOnChargeStart _array_element (EventDispatchers|CreateEvent :!event Custom|ChargeStartCallback))
    (EventDispatchers|BindEventtoOnChargeEnd _array_element (EventDispatchers|CreateEvent :!event Custom|ChargeEndCallback))))

(event Custom|SwitchElemental
  (params (Next :type Boolean))
  ;[0.15 0.15 0.15 0.5] Element change
  (bind _elemental (CallFunction|CanSwitchSetting))
  (if _elemental
    (Default|GetNextElement (Variables|Default|GetAC_ElementalSystem) Next)))

(event Custom|ChargeStart
  ;[0.15 0.15 0.15 0.5] Attack/Charge
  (bind _attack (CallFunction|CanSwitchSetting))
  (if _attack
    (Default|ChargeStart (Variables|Components|GetActiveWeaponSystem))))

(event Custom|Init%20Params
  ;[0.15 0.15 0.15 0.5] Initialize Parameters
  (CallFunction|UpdateStats 1e+02 1e+02 0.0 "NewEnumerator3"))

(event Custom|ToggleSprint
  (params (Sprinting :type Boolean))
  ;[0.15 0.15 0.15 0.5] Character movement controlls
  (Variables|Default|SetIsSprinting Sprinting)
  (CallFunction|UpdateMovementSpeed))

(event Custom|DoUpdateMovementSpeed
  ;[0.15 0.15 0.15 0.5] Character movement controlls
  (Variables|/Script/Engine.CharacterMovementComponent|SetMaxWalkSpeed (Variables|Character|GetCharacterMovement) (Variables|Default|GetCurrentWalkSpeed)))

(event Custom|ChargeEndCallback
  ;[0.15 0.15 0.15 0.5] Aiming
)

(event Custom|ChargeStartCallback
  ;[0.15 0.15 0.15 0.5] Aiming
)

(event Custom|ActivateAbility
  (params (Ability :type PDA%20Special%20Ability%20Object%20Reference))
  ;[0.15 0.15 0.15 0.5] Ability execution
  (bind _ability (CallFunction|CanSwitchSetting))
  (if _ability
    (bind _weapon (CallFunction|GetCharacterWeapon))
    (Default|ArmAbility (Variables|Default|GetAC_AbilitySystem) Ability _weapon (Variables|Default|GetElemental))))

(event EventToggleMovement
  (params (Enabled :type Boolean))
  (bind _returnvalue (Pawn|GetMovementComponent))
  ;[0.15 0.15 0.15 0.5] Character movement controlls
  (if Enabled
    (Components|Activation|Activate _returnvalue false)
    (CallFunction|UpdateMovementSpeed)
    (else
      (Components|Activation|Deactivate _returnvalue))))

(event EventToggleRootMotionRotation
  (params (Enabled :type Boolean))
  ;[0.15 0.15 0.15 0.5] Character movement controlls
  (Variables|/Script/Engine.CharacterMovementComponent|SetbAllowPhysicsRotationDuringAnimRootMotion (Variables|Character|GetCharacterMovement) Enabled))

(event EventActivateComponents
  ;[0.15 0.15 0.15 0.5] Activate Components
  (for _array_element (Utilities|Array|MakeArray (Variables|Default|GetAC_StatsSystem) (Variables|Default|GetAC_AbilityTree) (Variables|Default|GetAC_AbilitySystem) (Variables|Default|GetAC_StatusEffectSystem) (Variables|Default|GetAC_ElementalSystem))
    (Components|Activation|Activate _array_element false)
    (Development|PrintString "Components activated")))

(event EventSetCooldownMultiplier
  (params (CooldownMultiplier :type Float%20%28double-precision%29))
  ;[0.15 0.15 0.15 0.5] Weapon System
  (Variables|/Game/Saba/Blueprints/Components/AbilitySystem/AC_AbilitySystem.AC_AbilitySystem_C|SetCooldownMultiplier (Variables|Default|GetAC_AbilitySystem) CooldownMultiplier))

(event EventSetChargeMultiplier
  (params (ChargeMultiplier :type Float%20%28double-precision%29))
  ;[0.15 0.15 0.15 0.5] Ability execution
  (Default|SetChargeMultiplier (Variables|Components|GetActiveWeaponSystem) ChargeMultiplier))

(event EventUpdateStats
  (params (Hp :type Float%20%28double-precision%29) (Mana :type Float%20%28double-precision%29) (Xp :type Float%20%28double-precision%29) (Elemental :type E_ElementalType%20Enum :default "NewEnumerator0"))
  (Utilities|FlowControl|Sequence
    (:then_0
      (Default|AddHp (Variables|Default|GetAC_StatsSystem) Hp))
    (:then_1
      (Default|AddMana (Variables|Default|GetAC_StatsSystem) Mana))
    (:then_2
      (Default|AddXp (Variables|Default|GetAC_StatsSystem) Xp))))

(event EventLevelUp
  (Default|AddAbilityPoint (Variables|Default|GetAC_AbilityTree) 1))

(event EventKillCharacter
  (Pawn|Components|CharacterMovement|DisableMovement (Variables|Character|GetCharacterMovement))
  (Development|PrintString "Dead"))

(event EventApplyStatusEffect
  (params (Effect :type PDA%20Status%20Effect%20Object%20Reference))
  (Default|ApplyStatus (Variables|Default|GetAC_StatusEffectSystem) Effect))

(event EventApplyHit
  (params (HitResult :type Hit%20Result%20Structure) (Weapon :type BP%20Weapon%20Object%20Reference) (Charge :type Float%20%28double-precision%29) (Direction :type Vector :default "0, 0, 0") (Elemental :type E_ElementalType%20Enum :default "NewEnumerator0"))
  ;[0.15 0.15 0.15 0.5] Ability execution
  (Default|HitCallback (Variables|Default|GetAC_AbilitySystem) HitResult Weapon Charge Direction Elemental))

(event EventBeginPlay
  ;[0.15 0.15 0.15 0.5] Initialize the object
  (CallFunction|InitParams)
  (CallFunction|BindComponentEvents)
  (Default|EquipWeapon (Variables|Components|GetActiveWeaponSystem))
  (CallFunction|ActivateComponents)
  (bind _output_get (Variables|Default|SetDefaultWalkSpeed (Variables|/Script/Engine.CharacterMovementComponent|GetMaxWalkSpeed (Variables|Character|GetCharacterMovement))))
  (Variables|Default|SetMaxWalkSpeed (* _output_get 1.5))
  (Variables|Default|SetAimingWalkSpeed (* _output_get 0.5)))

(event EventSwitchWeaponSystem
  (params (Next :type Boolean))
  ;[0.15 0.15 0.15 0.5] Weapon System
  (bind _weapon (CallFunction|CanSwitchSetting))
  (if _weapon
    (Utilities|FlowControl|Sequence
      (:then_0
        (bind _activeweaponsystem (Variables|Components|GetActiveWeaponSystem)
          (:then
            (Components|Activation|Deactivate _activeweaponsystem))
          (:else)))
      (:then_1
        (bind _output_get (Variables|Components|SetActiveWeaponSystem (Utilities|Array|Get(acopy) (Variables|Components|GetWeaponSystems) (Utilities|Modulo (+ (Math|Integer|SelectInt -1 1 Next) (Utilities|Array|FindItem (Variables|Components|GetWeaponSystems) (Variables|Components|GetActiveWeaponSystem))) (Utilities|Array|Length (Variables|Components|GetWeaponSystems))))))
        (Components|Activation|Activate _output_get true)))))

(event EventChangeElement
  (params (ElementType :type E_ElementalType%20Enum :default "NewEnumerator0"))
  ;[0.15 0.15 0.15 0.5] Element change
  (Variables|Default|SetElemental ElementType))

(event EventSetMaxStats
  (params (Hp :type Float%20%28double-precision%29) (Mana :type Float%20%28double-precision%29))
  (Class|BPICharacter|SetMaxStats(Message) (Variables|Default|GetAC_StatsSystem) Hp Mana))

(event EventOnLanded
  (params (Hit :type Hit%20Result%20Structure%20%28by%20ref%29))
  ;[0.15 0.15 0.15 0.5] Character movement controlls
  (|CallParentFunction Hit)
  (CallFunction|DoUpdateMovementSpeed))

(fn ConstructionScript
  (Variables|Default|SetElemental "NewEnumerator3"))

(fn CanSwitchSetting
  (bind _isusingability (Variables|Default|GetIsUsingAbility))
  (bind _returnvalue (not _isusingability))
  (bind _type (Default|GetArmedAbilityType (Variables|Default|GetAC_AbilitySystem)))
  (bind _activeweaponsystem (Variables|Components|GetActiveWeaponSystem)
    (:then
      (return (and (not (Variables|/Game/Saba/Blueprints/Components/WeaponSystem/AC_BaseWeaponSystem.AC_BaseWeaponSystem_C|GetIsAiming _activeweaponsystem)) _returnvalue) (and (not (Variables|/Game/Saba/Blueprints/Components/WeaponSystem/AC_BaseWeaponSystem.AC_BaseWeaponSystem_C|GetIsAiming _activeweaponsystem)) _returnvalue) (and (not (Variables|/Game/Saba/Blueprints/Components/WeaponSystem/AC_BaseWeaponSystem.AC_BaseWeaponSystem_C|GetIsAiming _activeweaponsystem)) _returnvalue) (not (and _isusingability (Utilities|Enum|Equal(Enum) _type "NewEnumerator3")))))
    (:else
      (return _returnvalue _returnvalue _returnvalue (not (and _isusingability (Utilities|Enum|Equal(Enum) _type "NewEnumerator3")))))))

(fn CalculateWalkingSpeed
  (bind _activeweaponsystem (Variables|Components|GetActiveWeaponSystem))
  (bind _isaiming (Variables|/Game/Saba/Blueprints/Components/WeaponSystem/AC_BaseWeaponSystem.AC_BaseWeaponSystem_C|GetIsAiming _activeweaponsystem))
  (if (Variables|Default|GetIsSprinting)
    (if _isaiming
      _
      (else
        (return (Variables|Default|GetMaxWalkSpeed))))
    (elif _isaiming
      (return (Variables|Default|GetAimingWalkSpeed))
      (else
        _)))
  (return (Variables|Default|GetDefaultWalkSpeed)))

(fn CanMove
  (bind _result (Default|CanJump (Variables|Components|GetActiveWeaponSystem)))
  (return _result))

(fn GetAbilitySet
  (params (Elemental :type E_ElementalType%20Enum :default "NewEnumerator0"))
  (bind _abilityset (Default|GetAbilitySet (Variables|Default|GetAC_AbilityTree) Elemental))
  (return _abilityset))

(fn GetActiveSkeleton
  (return (Variables|Character|GetMesh)))

(fn GetActiveWeaponType
  (return "NewEnumerator0"))

(fn GetCharacterWeapon
  (bind _weapon (Default|GetCurrentWeapon (Variables|Components|GetActiveWeaponSystem)))
  (return _weapon))

(fn GetChargeLevel
  (bind _charge (Default|GetChargeLevel (Variables|Components|GetActiveWeaponSystem)))
  (return _charge))

(fn GetElementals
  (return (Variables|/Game/Saba/Blueprints/Components/AbilityTree/AC_AbilityTree.AC_AbilityTree_C|GetUnlockedElementals (Variables|Default|GetAC_AbilityTree))))

(fn GetFacingDirection
  (return "0, 0, 0" "0, 0, 0"))

(fn GetMaxStats
  (bind _ac_statssystem (Variables|Default|GetAC_StatsSystem))
  (return (Variables|/Game/Saba/Blueprints/Components/StatsSystem/AC_StatsSystem.AC_StatsSystem_C|GetMaxHp _ac_statssystem) (Variables|/Game/Saba/Blueprints/Components/StatsSystem/AC_StatsSystem.AC_StatsSystem_C|GetMaxMana _ac_statssystem)))

(fn GetStats
  (bind _ac_statssystem (Variables|Default|GetAC_StatsSystem))
  (return (Variables|/Game/Saba/Blueprints/Components/StatsSystem/AC_StatsSystem.AC_StatsSystem_C|GetHp _ac_statssystem) (Variables|/Game/Saba/Blueprints/Components/StatsSystem/AC_StatsSystem.AC_StatsSystem_C|GetMana _ac_statssystem) (Variables|/Game/Saba/Blueprints/Components/StatsSystem/AC_StatsSystem.AC_StatsSystem_C|GetXp _ac_statssystem)))

(fn IsChargeVfxAvailable
  (bind _armedability (Variables|/Game/Saba/Blueprints/Components/AbilitySystem/AC_AbilitySystem.AC_AbilitySystem_C|GetArmedAbility (Variables|Default|GetAC_AbilitySystem))
    (:then
      (return (Math|Boolean|ANDBoolean (Variables|Default|GetIsUsingAbility) (> (Variables|/Game/Saba/Blueprints/Components/AbilitySystem/PDA_SpecialAbility.PDA_SpecialAbility_C|GetRequiredCharge _armedability) 0.0) (Utilities|Enum|Equal(Enum) (Variables|/Game/Saba/Blueprints/Components/AbilitySystem/PDA_SpecialAbility.PDA_SpecialAbility_C|GetType _armedability) "NewEnumerator4"))))
    (:else
      (return false))))