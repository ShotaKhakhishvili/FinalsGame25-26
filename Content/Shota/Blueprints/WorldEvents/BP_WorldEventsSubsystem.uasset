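; A world events subsystem that holds the player and world events actor references and tracks real-time delta.
; StartLevel casts the pawn to BP_ThirdPersonCharacter, stores both references, then initializes the actor with the initial events, stopping if the cast fails.
; UpdateRealTime samples GetAccurateRealTime, keeping the previous sample so FGetWorldRealDeltaTime returns a delta independent of game time.
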(event Custom|StartLevel
  (params (PlayerPawn :type Pawn%20Object%20Reference) (WorldEventsActor :type BP%20World%20Events%20Actor%20Object%20Reference) (InitialEvents :type Array%20of%20PDA%20Event%20Definition%20Object%20References))
  (bind _asbp_third_person_character (Utilities|Casting|CastToBP_ThirdPersonCharacter PlayerPawn))
  (Variables|Default|SetPlayer _asbp_third_person_character)
  (bind _output_get (Variables|Default|SetWorldEventsActor WorldEventsActor))
  (Default|Init _output_get InitialEvents))

(event Custom|UpdateRealTime
  (bind (_seconds _partialseconds) (Class|GameplayStatics|GetAccurateRealTime))
  (Variables|Default|SetLastRealTime (Variables|Default|GetCurrentRealishTime))
  (Variables|Default|SetCurrentRealishTime (+ _seconds _partialseconds)))

(fn FGetWorldRealDeltaTime
  (return (- (Variables|Default|GetCurrentRealishTime) (Variables|Default|GetLastRealTime))))