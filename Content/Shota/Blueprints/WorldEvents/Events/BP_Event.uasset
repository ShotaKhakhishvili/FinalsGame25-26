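; BP_Event is a runtime world event that plays a sequence of BP_WorldEventAction objects in order.
; On first execution it duplicates each action from the Event's ActionSequence with itself as outer, keeping runtime instances separate from the source.
; Each action receives the event and WorldEventsActor, and its finish callback advances the index to execute the next.
; It also stores integer actor IDs by tag, merged without duplicates, for lookup.
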(event Custom|BindAdvance
  (EventDispatchers|BindEventtoOnFinished (CallFunction|FGetCurrentAction) (delegate Custom|Advance)))

(event Custom|Advance
  (Math|Integer|IncrementInt (Variables|Default|GetActionIndex)
    (:%20%20
      (CallFunction|FExecuteCurrentAction))))

(fn FAddActorIDs
  (params (Tag :type Name%20%28by%20ref%29) (NewIDs :type Array%20of%20Integers))
  (bind _runtimeactorids (Variables|Default|GetRuntimeActorIDs))
  (bind (_value _returnvalue) (Utilities|Map|Find _runtimeactorids Tag))
  (if _returnvalue
    (LocalVariables|SetResult (Utilities|Struct|BreakS_ArrayOfIntegers _value)))
  (for _array_element NewIDs
    (Utilities|Array|AddUnique (LocalVariables|GetResult) _array_element))
  (Utilities|Map|Add (Variables|Default|GetRuntimeActorIDs) Tag (Utilities|Struct|MakeS_ArrayOfIntegers (LocalVariables|GetResult))))

(fn FGetActorIDs
  (params (Tag :type Name%20%28by%20ref%29))
  (bind _runtimeactorids (Variables|Default|GetRuntimeActorIDs))
  (bind (_value _returnvalue) (Utilities|Map|Find _runtimeactorids Tag))
  (if _returnvalue
    (return (Utilities|Struct|BreakS_ArrayOfIntegers _value))))

(fn FGetCurrentAction
  (return (Utilities|Array|Get(acopy) (Variables|Default|GetRuntimeActionSequence) (Variables|Default|GetActionIndex))))

(fn FExecuteCurrentAction
  (if (Variables|Default|GetInitialized)
    _
    (else
      (CallFunction|FInit)))
  (if (< (Variables|Default|GetActionIndex) (Utilities|Array|Length (Variables|Default|GetRuntimeActionSequence)))
    (CallFunction|BindAdvance)
    (Default|Execute (CallFunction|FGetCurrentAction) self 0 (Variables|Default|GetWorldEventsActor))))

(fn FInit
  (Variables|Default|SetInitialized true)
  (for _array_element (Variables|/Game/Shota/Blueprints/WorldEvents/Events/PDA_EventDefinition.PDA_EventDefinition_C|GetActionSequence (Variables|Default|GetEvent))
    (bind _returnvalue (Class|WorldEventAction|DuplicateRuntime _array_element _array_element self))
    (bind _asbp_world_event_action (Utilities|Casting|CastToBP_WorldEventAction _returnvalue))
    (Utilities|Array|Add (Variables|Default|GetRuntimeActionSequence) _asbp_world_event_action)))