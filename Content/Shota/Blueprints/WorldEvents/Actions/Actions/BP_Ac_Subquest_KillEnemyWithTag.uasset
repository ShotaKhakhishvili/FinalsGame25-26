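; World event subquest action that tracks the killing of an enemy carrying a specific tag.
; On execute it binds to the world events actor's enemy-killed event and to its own finish event, which unbinds the kill listener.
; Each kill looks up the enemy's tag through the owner event and activates the predicate when it matches the action's Tag.
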(event Custom|OnEnemyKilled
  (params (Enemy :type BP%20Base%20Character%20Object%20Reference))
  (if (and (.HasTag (Default|FGetActorTag (stale EventExecute OwnerEvent) Enemy)) (== (.Tag (Default|FGetActorTag (stale EventExecute OwnerEvent) Enemy)) (Variables|Default|GetTag)))
    (Default|CallPredicateActivated)))

(event Custom|OnFinished
  (EventDispatchers|UnbindEventfromEnemyKilled (stale EventExecute WorldEventsActor) (delegate Custom|OnEnemyKilled)))

(event EventExecute
  (params (OwnerEvent :type BP%20Event%20Object%20Reference) (PlayerPawn :type Pawn%20Object%20Reference) (WorldEventsActor :type BP%20World%20Events%20Actor%20Object%20Reference))
  (|CallParentFunction OwnerEvent PlayerPawn WorldEventsActor)
  (EventDispatchers|BindEventtoEnemyKilled WorldEventsActor (delegate Custom|OnEnemyKilled))
  (EventDispatchers|BindEventtoActionFinished (delegate Custom|OnFinished)))