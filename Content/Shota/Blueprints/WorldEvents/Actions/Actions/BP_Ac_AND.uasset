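; World event action that acts as an AND composite, finishing only once all of its sub-actions have finished.
; On Execute it calls the parent, then binds to each sub-action's finished event before starting it, without waiting between them.
; Each completion increments a counter; when it equals the sub-action count, the action unbinds from all and signals its own completion.
; The graph never resets the counter.
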(event Custom|IncrementCounter
  (bind _result (Math|Integer|IncrementInt (Variables|Default|GetCounter))
    (:%20%20
      (if (== _result (Utilities|Array|Length (Variables|Default|GetSubActions)))
        (for _array_element (Variables|Default|GetSubActions)
          (EventDispatchers|UnbindEventfromActionFinished _array_element (delegate Custom|IncrementCounter)))
        (Default|CallActionFinished)))))

(event EventExecute
  (params (OwnerEvent :type BP%20Event%20Object%20Reference) (PlayerPawn :type BP%20Third%20Person%20Character%20Object%20Reference) (WorldEventsActor :type BP%20World%20Events%20Actor%20Object%20Reference))
  (|CallParentFunction OwnerEvent PlayerPawn WorldEventsActor)
  (for _array_element (Variables|Default|GetSubActions)
    (EventDispatchers|BindEventtoActionFinished _array_element (delegate Custom|IncrementCounter))
    (Default|Execute _array_element OwnerEvent PlayerPawn WorldEventsActor)))