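; BP_Ac_Subquest is a world event action that shows a counted subquest line in the player's quest notification widget.
; On Execute it records the widget's current child count as its line index, appends the line, and binds to predicate activations.
; Each activation increments the counter and refreshes that line, with an optional current/total display.
; Reaching the target count switches the line's state type and finishes the action.
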(event Custom|OnPredicateActivated
  (if (< (Variables|Default|GetCurrentCount) (Variables|Default|GetCount))
    (bind _result (Math|Integer|IncrementInt (Variables|Default|GetCurrentCount))
      (:%20%20
        (CallFunction|FUpdateWidget (Variables|/Game/Shota/Blueprints/Widgets/Quests/WBP_Quests.WBP_Quests_C|GetWBP_MultilineQuestText (Variables|/Game/Shota/Blueprints/Widgets/Notifiations/WGT_Notifications.WGT_Notifications_C|GetWBP_Quests (stale EventExecute _notifications))))
        (if (>= _result (Variables|Default|GetCount))
          (Default|CallActionFinished))))))

(event EventExecute
  (params (OwnerEvent :type BP%20Event%20Object%20Reference) (PlayerPawn :type Pawn%20Object%20Reference) (WorldEventsActor :type BP%20World%20Events%20Actor%20Object%20Reference))
  (|CallParentFunction OwnerEvent PlayerPawn WorldEventsActor)
  (bind _notifications (Class|BPIPlayerWorldEvents|FGetNotifications(Message) PlayerPawn))
  (Variables|Default|SetQuestLine (Class|PanelWidget|GetChildrenCount (Variables|/Game/Shota/Blueprints/Widgets/Quests/WBP_MultilineQuestText.WBP_MultilineQuestText_C|GetVerticalBoxLeft (Variables|/Game/Shota/Blueprints/Widgets/Quests/WBP_Quests.WBP_Quests_C|GetWBP_MultilineQuestText (Variables|/Game/Shota/Blueprints/Widgets/Notifiations/WGT_Notifications.WGT_Notifications_C|GetWBP_Quests _notifications)))))
  (CallFunction|FAddLine (Variables|/Game/Shota/Blueprints/Widgets/Quests/WBP_Quests.WBP_Quests_C|GetWBP_MultilineQuestText (Variables|/Game/Shota/Blueprints/Widgets/Notifiations/WGT_Notifications.WGT_Notifications_C|GetWBP_Quests _notifications)))
  (EventDispatchers|BindEventtoPredicateActivated (delegate Custom|OnPredicateActivated)))

(fn FUpdateWidget
  (params (QuestText :type WBP%20Multiline%20Quest%20Text%20Object%20Reference))
  (Default|UpdateLine QuestText (Variables|Default|GetQuestLine) (CallFunction|FGetQuestTextState)))

(fn FAddLine
  (params (QuestWidget :type WBP%20Multiline%20Quest%20Text%20Object%20Reference))
  (Default|AddLine QuestWidget (CallFunction|FGetQuestTextState)))

(fn FGetQuestTextState
  (return (Utilities|Struct|MakeS_QuestTextLine (.lefttext (Variables|Default|GetLine%20Text)) (Utilities|String|SelectText (Utilities|Text|ToText(String) (Utilities|String|Append (Utilities|String|ToString(Integer) (Variables|Default|GetCurrentCount)) "/" (Utilities|String|ToString(Integer) (Variables|Default|GetCount)))) "" (Variables|Default|GetDisplayCount)) (select (== (Variables|Default|GetCount) (Variables|Default|GetCurrentCount)) "NewEnumerator4" "NewEnumerator0"))))