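; World event action that kills the player character when a world event executes it.
; Execute runs the parent logic, calls KillCharacter on the player pawn, then immediately reports the action as finished.
; A separate helper gathers the owner's actor IDs for each configured tag as the list to destroy, though Execute does not call it directly.
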(event EventExecute
  (params (OwnerEvent :type BP%20Event%20Object%20Reference) (PlayerPawn :type BP%20Third%20Person%20Character%20Object%20Reference) (WorldEventsActor :type BP%20World%20Events%20Actor%20Object%20Reference))
  (|CallParentFunction OwnerEvent PlayerPawn WorldEventsActor)
  (Default|KillCharacter PlayerPawn)
  (Default|CallActionFinished))

(fn FGetAllIDstoDestroy
  (params (Owner :type BP%20Event%20Object%20Reference))
  (Utilities|Array|Clear (LocalVariables|GetResult))
  (for _array_element (Variables|Default|GetTag)
    (Utilities|Array|AppendArray (LocalVariables|GetResult) (Default|FGetActorIDs Owner _array_element)))
  (return (LocalVariables|GetResult)))