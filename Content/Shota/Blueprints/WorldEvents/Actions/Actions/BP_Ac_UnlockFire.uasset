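; BP_Ac_UnlockFire is a world event action that unlocks the fire element for the player.
; On Execute it calls the parent, then uses the player's ACAbilityTree to unlock the element, grant an ability point and unlock the DA_Skill_F1 node, then signals completion.
; A separate function gathers actor IDs from the owner for each configured tag, as the list to destroy.
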(event EventExecute
  (params (OwnerEvent :type BP%20Event%20Object%20Reference) (PlayerPawn :type BP%20Third%20Person%20Character%20Object%20Reference) (WorldEventsActor :type BP%20World%20Events%20Actor%20Object%20Reference))
  (bind _ac_abilitytree (Variables|/Game/Saba/Blueprints/Characters/BP_BaseCharacter.BP_BaseCharacter_C|GetAC_AbilityTree PlayerPawn))
  (|CallParentFunction OwnerEvent PlayerPawn WorldEventsActor)
  (Default|UnlockElemental _ac_abilitytree "NewEnumerator0")
  (Default|AddAbilityPoint _ac_abilitytree 1)
  (Default|UnlockNode _ac_abilitytree "/Game/Saba/Blueprints/Components/AbilityTree/DA_Skill_F1.DA_Skill_F1")
  (Default|CallActionFinished))

(fn FGetAllIDstoDestroy
  (params (Owner :type BP%20Event%20Object%20Reference))
  (Utilities|Array|Clear (LocalVariables|GetResult))
  (for _array_element (Variables|Default|GetTag)
    (Utilities|Array|AppendArray (LocalVariables|GetResult) (Default|FGetActorIDs Owner _array_element)))
  (return (LocalVariables|GetResult)))