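; World event action that unlocks a fixed set of abilities on the player.
; On execute it calls the parent, sets the player's ability tree points to four, unlocks four skill data asset nodes, then signals the action finished.
; A helper function gathers the owner's actor IDs for each entry in Tag into one list of IDs to destroy.
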(event EventExecute
  (params (OwnerEvent :type BP%20Event%20Object%20Reference) (PlayerPawn :type BP%20Third%20Person%20Character%20Object%20Reference) (WorldEventsActor :type BP%20World%20Events%20Actor%20Object%20Reference))
  (bind _ac_abilitytree (Variables|/Game/Saba/Blueprints/Characters/BP_BaseCharacter.BP_BaseCharacter_C|GetAC_AbilityTree PlayerPawn))
  (|CallParentFunction OwnerEvent PlayerPawn WorldEventsActor)
  (Variables|/Game/Saba/Blueprints/Components/AbilityTree/AC_AbilityTree.AC_AbilityTree_C|SetAvailablePoints _ac_abilitytree 4)
  (Default|UnlockNode _ac_abilitytree "/Game/Saba/Blueprints/Components/AbilityTree/DA_Skill_D1.DA_Skill_D1")
  (Default|UnlockNode _ac_abilitytree "/Game/Saba/Blueprints/Components/AbilityTree/DA_Skill_H1.DA_Skill_H1")
  (Default|UnlockNode _ac_abilitytree "/Game/Saba/Blueprints/Components/AbilityTree/DA_Skill_O1.DA_Skill_O1")
  (Default|UnlockNode _ac_abilitytree "/Game/Saba/Blueprints/Components/AbilityTree/DA_Skill_S1.DA_Skill_S1")
  (Default|CallActionFinished))

(fn FGetAllIDstoDestroy
  (params (Owner :type BP%20Event%20Object%20Reference))
  (Utilities|Array|Clear (LocalVariables|GetResult))
  (for _array_element (Variables|Default|GetTag)
    (Utilities|Array|AppendArray (LocalVariables|GetResult) (Default|FGetActorIDs Owner _array_element)))
  (return (LocalVariables|GetResult)))