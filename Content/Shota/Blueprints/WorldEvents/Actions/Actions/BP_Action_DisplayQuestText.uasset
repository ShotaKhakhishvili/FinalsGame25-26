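; BP_Action_DisplayQuestText is a world event action that, despite its name, spawns actors and registers them with the owning event; no text display appears in its graphs.
; Execute runs FExecutePart, which spawns an actor at each transform in an array and looks up its ID through the WorldEventsActor.
; The IDs it finds are added to the owner event, then the action signals that it has finished.
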(event EventExecute
  (params (OwnerEvent :type BP%20Event%20Object%20Reference) (WorldEventsActor :type BP%20World%20Events%20Actor%20Object%20Reference))
  (CallFunction|FExecutePart OwnerEvent WorldEventsActor)
  (Default|CallOnFinished))

(fn FExecutePart
  (params (Owner%20Event :type BP%20Event%20Object%20Reference) (WorldEventsActor :type BP%20World%20Events%20Actor%20Object%20Reference))
  (for _array_element 0
    (bind _returnvalue (Class|WorldEventAction|SpawnActor 0 _array_element))
    (if (.Found (Default|FGetIDfromActor WorldEventsActor _returnvalue))
      (Utilities|Array|Add (LocalVariables|GetIDs) (.ID (Default|FGetIDfromActor WorldEventsActor _returnvalue)))))
  (Default|FAddActorIDs Owner%20Event "None" (LocalVariables|GetIDs)))