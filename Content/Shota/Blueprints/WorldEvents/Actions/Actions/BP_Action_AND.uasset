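; BP_Action_AND is a composite world event action that runs several sub-actions and finishes when all have reported completion.
; Execute starts every sub-action in one loop, passing along the owner event, player pawn and world events actor, then binds to its finished event.
; Each completion increments a counter, and the action signals finished when the count equals the number of sub-actions.
; Binding follows each Execute call, and the counter is never reset here.
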(event Custom|IncrementCounter
  (bind _result (Math|Integer|IncrementInt (Variables|Default|GetCounter))
    (:%20%20
      (if (== _result (Utilities|Array|Length (Variables|Default|GetSubActions)))
        (Default|CallActionFinished)))))

(event EventExecute
  (params (OwnerEvent :type BP%20Event%20Object%20Reference) (PlayerPawn :type Pawn%20Object%20Reference) (WorldEventsActor :type BP%20World%20Events%20Actor%20Object%20Reference))
  (for _array_element (Variables|Default|GetSubActions)
    (Default|Execute _array_element OwnerEvent PlayerPawn WorldEventsActor)
    (EventDispatchers|BindEventtoActionFinished _array_element (delegate Custom|IncrementCounter))))