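; World event action that destroys the world event's actors matching a set of tags.
; On Execute it starts a two-second timer before acting.
; It then gathers actor IDs from the owner event for each configured tag and has the world events actor destroy each one by ID.
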(event Custom|SpawnSomething
  (for _array_element (CallFunction|FGetAllIDstoDestroy (stale EventExecute OwnerEvent))
    (Default|FDestroyActorwithID (stale EventExecute WorldEventsActor) _array_element)))

(event EventExecute
  (params (OwnerEvent :type BP%20Event%20Object%20Reference) (WorldEventsActor :type BP%20World%20Events%20Actor%20Object%20Reference))
  (Utilities|Time|SetTimerbyEvent (delegate Custom|SpawnSomething) 2.0))

(fn FGetAllIDstoDestroy
  (params (Owner :type BP%20Event%20Object%20Reference))
  (Utilities|Array|Clear (LocalVariables|GetResult))
  (for _array_element (Variables|Default|GetTag)
    (Utilities|Array|AppendArray (LocalVariables|GetResult) (Default|FGetActorIDs Owner _array_element)))
  (return (LocalVariables|GetResult)))