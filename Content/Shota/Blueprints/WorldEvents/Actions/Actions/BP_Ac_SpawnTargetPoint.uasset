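; World event action that spawns a BP_TargetPoint at a configured transform for the player to deal with during an event.
; On Execute it spawns the point and passes it the reach distance, reachable flag and auto-destroy-on-reach setting.
; It binds to the point's OnDestroyed and reports the action finished only when that point is destroyed.
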(event Custom|Finish
  (params (DestroyedActor :type Actor%20Object%20Reference))
  (Default|CallActionFinished))

(event EventExecute
  (params (OwnerEvent :type BP%20Event%20Object%20Reference) (PlayerPawn :type BP%20Third%20Person%20Character%20Object%20Reference) (WorldEventsActor :type BP%20World%20Events%20Actor%20Object%20Reference))
  (|CallParentFunction OwnerEvent PlayerPawn WorldEventsActor)
  (bind _returnvalue (Class|WorldEventAction|SpawnActor "/Game/Shota/Blueprints/Actors/BP_TargetPoint.BP_TargetPoint_C" (Variables|Default|GetTargetPoint)))
  (bind _asbp_target_point (Utilities|Casting|CastToBP_TargetPoint _returnvalue))
  (Variables|/Game/Shota/Blueprints/Actors/BP_TargetPoint.BP_TargetPoint_C|SetReachDistance _asbp_target_point (Variables|Default|GetReach%20Distance))
  (Variables|/Game/Shota/Blueprints/Actors/BP_TargetPoint.BP_TargetPoint_C|SetIsReachable _asbp_target_point (Variables|Default|GetIs%20Reachable))
  (Variables|/Game/Shota/Blueprints/Actors/BP_TargetPoint.BP_TargetPoint_C|SetAutoDestroyOnReach _asbp_target_point (Variables|Default|GetAuto%20Destroy%20on%20Reach))
  (Game|BindEventtoOnDestroyed _asbp_target_point (delegate Custom|Finish)))