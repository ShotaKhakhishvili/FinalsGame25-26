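; World events manager actor that runs events, tracks spawned actors by ID and keeps a registry of combat NPC controllers.
; Init binds to the world events subsystem's spawn callback, then wraps each event in a BP_Event object that executes its current action on the player pawn.
; Spawned actors get incremental IDs in two-way maps for lookup and destruction by ID.
; Tick updates the game instance's real time.
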(event Custom|Init
  (params (Events :type Array%20of%20PDA%20Event%20Definition%20Object%20References))
  (EventDispatchers|BindEventtoOnActorSpawned (Subsystems|GetWorldEventsGameInstanceSubsystem) (delegate Custom|RegisterActorID))
  (for _array_element Events
    (CallFunction|AddEvent _array_element)))

(event Custom|AddEvent
  (params (NewEvent :type PDA%20Event%20Definition%20Object%20Reference))
  (bind _self self)
  (bind _returnvalue (Game|ConstructObjectfromClass _self "/Game/Shota/Blueprints/WorldEvents/Events/BP_Event.BP_Event_C" NewEvent _self))
  (Default|FExecuteCurrentAction _returnvalue (Game|Player|GetPlayerPawn 0))
  (Utilities|Array|Add (Variables|Default|GetEvents) _returnvalue))

(event Custom|RegisterActorID
  (params (SpawnedActor :type Actor%20Object%20Reference))
  (Utilities|Map|Add (Variables|Default|GetActorFromID) (Variables|Default|GetCurrentID) SpawnedActor)
  (Utilities|Map|Add (Variables|Default|GetIDFromActor) SpawnedActor (Variables|Default|GetCurrentID))
  (Math|Integer|IncrementInt (Variables|Default|GetCurrentID)))

(event EventTick
  (params (DeltaSeconds :type Float%20%28single-precision%29))
  (Default|UpdateRealTime (CallFunction|FLGetGameInstance)))

(fn ConstructionScript)

(fn FGetActorfromID
  (params (ID :type Integer%20%28by%20ref%29))
  (bind _actorfromid (Variables|Default|GetActorFromID))
  (bind (_value _returnvalue) (Utilities|Map|Find _actorfromid ID))
  (return _value _returnvalue))

(fn FGetIDfromActor
  (params (Actor :type Actor%20Object%20Reference%20%28by%20ref%29))
  (bind _idfromactor (Variables|Default|GetIDFromActor))
  (bind (_value _returnvalue) (Utilities|Map|Find _idfromactor Actor))
  (return _value _returnvalue))

(fn FDestroyActor
  (params (Actor :type Actor%20Object%20Reference))
  (Actor|DestroyActor Actor))

(fn FDestroyActorwithID
  (params (Key :type Integer%20%28by%20ref%29))
  (CallFunction|FDestroyActor (.Value (Utilities|Map|Find (Variables|Default|GetActorFromID) Key))))

(fn FRegisterComabtNPCController
  (params (Controller :type Combat%20NPC%20Controller%20Object%20Reference))
  (Utilities|Set|Add (Variables|Default|GetEnemyControllers) Controller))

(fn FUnregisterComabtNPCController
  (params (Controller :type Combat%20NPC%20Controller%20Object%20Reference))
  (Utilities|Set|Remove (Variables|Default|GetEnemyControllers) Controller))

(fn FGetRegisteredEnemyControllers
  (bind _result (Utilities|Set|ToArray (Variables|Default|GetEnemyControllers)))
  (return _result))