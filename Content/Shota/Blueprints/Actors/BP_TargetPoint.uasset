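; BP_TargetPoint is a waypoint marker actor that displays the player's distance to it through a WBP_Target widget.
; Each tick, it turns the widget toward the player's follow camera, fetched via BPWorldEventsSubsystem, and refreshes the camera distance in whole meters.
; If the marker is reachable and that camera distance is within ReachDistance, it fires WasReached once and optionally destroys itself.
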(event EventTick
  (params (DeltaSeconds :type Float%20%28single-precision%29))
  (bind _returnvalue (Subsystems|GetBPWorldEventsSubsystem))
  (bind _widget (Variables|Default|GetWidget))
  (bind _returnvalue_2 (Transformation|GetWorldLocation _widget))
  (bind _player (Variables|/Game/Shota/Blueprints/WorldEvents/BP_WorldEventsSubsystem.BP_WorldEventsSubsystem_C|GetPlayer _returnvalue))
  (bind _followcamera (Variables|/Game/Saba/Blueprints/Characters/BP_ThirdPersonCharacter.BP_ThirdPersonCharacter_C|GetFollowCamera _player))
  (bind _returnvalue_3 (Transformation|GetWorldLocation _followcamera))
  (bind _returnvalue_4 (Math|Vector|Distance(Vector) _returnvalue_2 _returnvalue_3))
  (bind _returnvalue_5 (/ _returnvalue_4 1e+02))
  (Transformation|SetWorldRotation (Variables|Default|GetWidget) (Math|Rotator|FindLookatRotation _returnvalue_2 _returnvalue_3) false false)
  (Default|RefreshDistance (Variables|Default|GetWBP_Target) (Math|Float|Truncate _returnvalue_5))
  (if (and (<= _returnvalue_5 (Variables|Default|GetReachDistance)) (Variables|Default|GetIsReachable))
    (Utilities|FlowControl|DoOnce false
      (:Completed
        (Default|CallWasReached self)
        (if (Variables|Default|GetAutoDestroyOnReach)
          (Actor|DestroyActor))))))

(event EventBeginPlay
  (bind _aswbp_target (Utilities|Casting|CastToWBP_Target (UserInterface|GetWidget (Variables|Default|GetWidget))))
  (Variables|Default|SetWBP_Target _aswbp_target))

(fn ConstructionScript)