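; Menu pawn that sets up the menu screen on BeginPlay by showing the mouse cursor, switching to Game and UI input, and adding WBP_Menu to the viewport.
; Keys 1, 2 and 3 call CallOnCursorTypeChanged on GI_Custom, each with its own cursor type index.
; F_GetNotifications exposes the notifications widget inside the menu widget to other code.
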(event EventBeginPlay
  (bind _returnvalue (Game|GetPlayerController 0))
  (Variables|/Script/Engine.PlayerController|SetbShowMouseCursor _returnvalue true)
  (Input|SetInputModeGameandUI _returnvalue 0 "DoNotLock" false false)
  (bind _returnvalue_2 (UserInterface|CreateWidget "/Game/Shota/Blueprints/Widgets/MainMenu/WBP_Menu.WBP_Menu_C"))
  (bind _output_get (Variables|Default|SetWBP_Menu _returnvalue_2))
  (UserInterface|Viewport|AddtoViewport _output_get 0))

(event Input|KeyboardEvents|3
  (params (Key :type Key%20Structure :default "None"))
  (:Pressed
    (bind _asgi_custom (Utilities|Casting|CastToGI_Custom (Game|GetGameInstance)))
    (Default|CallOnCursorTypeChanged _asgi_custom 2)))

(event Input|KeyboardEvents|1
  (params (Key :type Key%20Structure :default "None"))
  (:Pressed
    (bind _asgi_custom (Utilities|Casting|CastToGI_Custom (Game|GetGameInstance)))
    (Default|CallOnCursorTypeChanged _asgi_custom)))

(event Input|KeyboardEvents|2
  (params (Key :type Key%20Structure :default "None"))
  (:Pressed
    (bind _asgi_custom (Utilities|Casting|CastToGI_Custom (Game|GetGameInstance)))
    (Default|CallOnCursorTypeChanged _asgi_custom 1)))

(fn ConstructionScript)

(fn FGetNotifications
  (return (Variables|/Game/Shota/Blueprints/Widgets/MainMenu/WBP_Menu.WBP_Menu_C|GetWGT_Notifications (Variables|Default|GetWBP_Menu))))