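; Custom game instance that manages saving and loading of player data, the save-slot list and options, plus level start.
; Each data type has its own SaveGame object, created fresh when loading fails; default options also reset GameUserSettings.
; Player saves share one slot name, using UserIndex as slot number, with names and dates indexed in SG_GameSaves.
; StartLevel caches the player and initialises the world events actor, while UpdateRealTime supports a real-time delta.
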(event Custom|StartLevel
  (params (PlayerPawn :type Pawn%20Object%20Reference) (WorldEventsActor :type BP%20World%20Events%20Actor%20Object%20Reference) (InitialEvents :type Array%20of%20PDA%20Event%20Definition%20Object%20References))
  (bind _asbp_third_person_character (Utilities|Casting|CastToBP_ThirdPersonCharacter PlayerPawn))
  (Variables|Default|SetPlayer _asbp_third_person_character)
  (bind _output_get (Variables|Default|SetWorldEventsActor WorldEventsActor))
  (Default|Init _output_get InitialEvents))

(event Custom|UpdateRealTime
  (bind (_seconds _partialseconds) (Class|GameplayStatics|GetAccurateRealTime))
  (Variables|Default|SetLastRealTime (Variables|Default|GetCurrentRealishTime))
  (Variables|Default|SetCurrentRealishTime (+ _seconds _partialseconds)))

(fn FLoadPlayerData
  (params (Index :type Integer))
  ;[0.15 0.15 0.15 0.5] Literal Loading
  (bind _returnvalue (SaveGame|DoesSaveGameExist "#PlayerData#" Index))
  (if _returnvalue
    (bind _returnvalue_2 (SaveGame|LoadGamefromSlot "#PlayerData#" Index))
    (bind _assg_player (Utilities|Casting|CastToSG_Player _returnvalue_2)
      (:then
        (Variables|Default|SetSG_Player _assg_player))
      (:CastFailed
        (bind _returnvalue_3 (SaveGame|CreateSaveGameObject "/Game/Shota/Blueprints/Game/SaveGame/SG_Player.SG_Player_C" :!label _label))
        (Variables|Default|SetSG_Player _returnvalue_3)))
    (else
      (goto _label))))

(fn FLoadGameSaveInfos
  ;[0.15 0.15 0.15 0.5] Literally Just Loading
  (bind _returnvalue (SaveGame|DoesSaveGameExist "#GameSaves#"))
  (if _returnvalue
    (bind _returnvalue_2 (SaveGame|LoadGamefromSlot "#GameSaves#"))
    (bind _assg_game_saves (Utilities|Casting|CastToSG_GameSaves _returnvalue_2)
      (:then
        (Variables|Default|SetSG_GameSaves _assg_game_saves))
      (:CastFailed
        (bind _returnvalue_3 (SaveGame|CreateSaveGameObject "/Game/Shota/Blueprints/Game/SaveGame/SG_GameSaves.SG_GameSaves_C" :!label _label))
        (Variables|Default|SetSG_GameSaves _returnvalue_3)))
    (else
      (goto _label))))

(fn FLoadOptions
  (bind _returnvalue (SaveGame|DoesSaveGameExist "#Options#"))
  (if _returnvalue
    (bind _returnvalue_2 (SaveGame|LoadGamefromSlot "#Options#"))
    (bind _assg_options (Utilities|Casting|CastToSG_Options _returnvalue_2)
      (:then
        (Variables|Default|SetSG_Options _assg_options))
      (:CastFailed
        (bind _returnvalue_3 (SaveGame|CreateSaveGameObject "/Game/Shota/Blueprints/Game/SaveGame/SG_Options.SG_Options_C" :!label _label))
        (Variables|Default|SetSG_Options _returnvalue_3)
        (CallFunction|FSetDefaultOptions)))
    (else
      (goto _label)))
  (return (Variables|/Game/Shota/Blueprints/Game/SaveGame/SG_Options.SG_Options_C|GetVol_Master (Variables|Default|GetSG_Options)) (Variables|/Game/Shota/Blueprints/Game/SaveGame/SG_Options.SG_Options_C|GetVol_Music (Variables|Default|GetSG_Options)) (Variables|/Game/Shota/Blueprints/Game/SaveGame/SG_Options.SG_Options_C|GetVol_SFX (Variables|Default|GetSG_Options)) (Variables|/Game/Shota/Blueprints/Game/SaveGame/SG_Options.SG_Options_C|GetVol_UI (Variables|Default|GetSG_Options)) (Variables|/Game/Shota/Blueprints/Game/SaveGame/SG_Options.SG_Options_C|GetCur_Sensitivity (Variables|Default|GetSG_Options)) (Variables|/Game/Shota/Blueprints/Game/SaveGame/SG_Options.SG_Options_C|GetCur_Icon (Variables|Default|GetSG_Options)) (Variables|/Game/Shota/Blueprints/Game/SaveGame/SG_Options.SG_Options_C|GetLandscapeQuality (Variables|Default|GetSG_Options))))

(fn FLoadGameSlotData
  (params (Index :type Integer))
  (CallFunction|FLoadPlayerData Index))

(fn FSaveOptions
  (bind _returnvalue (SaveGame|SaveGametoSlot (Variables|Default|GetSG_Options) "#Options#"))
  (return _returnvalue))

(fn FSaveGameSlot
  (params (Player :type BP%20Base%20Character%20Object%20Reference) (Slot :type Integer) (DefaultSave :type Boolean))
  (bind _output_get (LocalVariables|SetSaveSlot Slot))
  (if DefaultSave
    (bind _returnvalue (SaveGame|CreateSaveGameObject "/Game/Shota/Blueprints/Game/SaveGame/SG_Player.SG_Player_C"))
    (Variables|Default|SetSG_Player _returnvalue)
    (else
      ;[0.15 0.15 0.15 0.5] Gather Player Data
      (CallFunction|FGatherPlayerData Player _output_get)))
  ;[0.15 0.15 0.15 0.5] Save Player Data
  (SaveGame|SaveGametoSlot (Variables|Default|GetSG_Player) "#PlayerData#" (LocalVariables|GetSaveSlot))
  ;[0.15 0.15 0.15 0.5] Save Game Saves
  (CallFunction|FSaveGameSlotInfos))

(fn FSaveonNewSlot
  (params (Name :type Text) (Player :type BP%20Base%20Character%20Object%20Reference) (DefaultSave :type Boolean))
  (bind _sg_gamesaves (Variables|Default|GetSG_GameSaves))
  (bind _maxunsavedindex (Variables|/Game/Shota/Blueprints/Game/SaveGame/SG_GameSaves.SG_GameSaves_C|GetMaxUnsavedIndex _sg_gamesaves))
  (Utilities|Array|Add (Variables|/Game/Shota/Blueprints/Game/SaveGame/SG_GameSaves.SG_GameSaves_C|GetAllSaves _sg_gamesaves) (Utilities|Struct|MakeS_GameSave Name (Math|DateTime|Now) _maxunsavedindex))
  (Math|Integer|IncrementInt _maxunsavedindex
    (:%20%20
      (CallFunction|FSaveGameSlot Player (- (Variables|/Game/Shota/Blueprints/Game/SaveGame/SG_GameSaves.SG_GameSaves_C|GetMaxUnsavedIndex (Variables|Default|GetSG_GameSaves)) 1) DefaultSave)
      (return (- (Variables|/Game/Shota/Blueprints/Game/SaveGame/SG_GameSaves.SG_GameSaves_C|GetMaxUnsavedIndex (Variables|Default|GetSG_GameSaves)) 1)))))

(fn FSaveGameSlotInfos
  (SaveGame|SaveGametoSlot (Variables|Default|GetSG_GameSaves) "#GameSaves#")
  (Default|FSetTimeonSave (Variables|Default|GetSG_GameSaves) 0 (Math|DateTime|Now)))

(fn FSetDefaultOptions
  (bind _returnvalue (SaveGame|CreateSaveGameObject "/Game/Shota/Blueprints/Game/SaveGame/SG_Options.SG_Options_C"))
  (Variables|Default|SetSG_Options _returnvalue)
  (bind _returnvalue_2 (Settings|GetGameUserSettings))
  (Class|GameUserSettings|SettoDefaults _returnvalue_2)
  (Class|GameUserSettings|SaveSettings _returnvalue_2))

(fn FGetAllGameSaveInfos
  (return (Variables|/Game/Shota/Blueprints/Game/SaveGame/SG_GameSaves.SG_GameSaves_C|GetAllSaves (Variables|Default|GetSG_GameSaves))))

(fn FGatherPlayerData
  (params (Player :type BP%20Base%20Character%20Object%20Reference) (Slot :type Integer))
  (LocalVariables|SetSaveSlot Slot)
  (Default|SavaData (Variables|Default|GetSG_Player) Player))

(fn FSetGameSaveSlotasCurrent
  (params (SlotIndex :type Integer))
  (bind _returnvalue (SaveGame|DoesSaveGameExist "#PlayerData#" SlotIndex))
  (if _returnvalue
    (bind _returnvalue_2 (SaveGame|LoadGamefromSlot "#PlayerData#" SlotIndex))
    (bind _assg_player (Utilities|Casting|CastToSG_Player _returnvalue_2))
    (Variables|Default|SetSG_Player _assg_player)
    (return true)
    (else
      (return false))))

(fn FRenameGameSlot
  (params (SlotIndex :type Integer) (Name :type Text))
  (bind _success (Default|FSetNameonSave (Variables|Default|GetSG_GameSaves) SlotIndex Name))
  (if _success
    (CallFunction|FSaveGameSlotInfos))
  (return _success))

(fn FGetWorldRealDeltaTime
  (return (- (Variables|Default|GetCurrentRealishTime) (Variables|Default|GetLastRealTime))))