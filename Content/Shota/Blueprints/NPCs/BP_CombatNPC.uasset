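; Combat NPC character that uses the elemental, weapon and ability systems to fight as an ally or enemy of the player.
; On BeginPlay it applies a cooler status, grants ability points, unlocks its configured elements and skills, then switches elemental and weapon systems.
; NPC events wrap aim, charge, attack and timed retargeting, with facing taken from the controller's target.
; Abilities are picked by weighted random, and death is broadcast to the world events actor.
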(event Custom|NPC_TurnMad
  (params (Duration :type Float%20%28double-precision%29))
  (Default|CallRetargeted true)
  (Utilities|FlowControl|Delay Duration)
  (Default|CallRetargeted false))

(event Custom|NPC_EndAim
  ;[0.15 0.15 0.15 0.5] Base actions
  (if (not (Variables|Default|GetIsUsingAbility))
    (CallFunction|AimEnd)))

(event Custom|NPC_StartAim
  ;[0.15 0.15 0.15 0.5] Base actions
  (if (not (Variables|Default|GetIsUsingAbility))
    (CallFunction|AimStart)))

(event Custom|NPC_ReleaseCharge
  ;[0.15 0.15 0.15 0.5] Base actions
  (CallFunction|AttackStart))

(event Custom|NPC_StartCharge
  ;[0.15 0.15 0.15 0.5] Base actions
  (CallFunction|ChargeStart))

(event EventBeginPlay
  (|CallParentFunction)
  (Default|ApplyStatus (Variables|Default|GetAC_StatusEffectSystem) "/Game/Saba/Blueprints/Components/StatusEffectSystem/DA_CoolerMax.DA_CoolerMax")
  ;[0.15 0.15 0.15 0.5] Unlock skills
  (Default|AddAbilityPoint (Variables|Default|GetAC_AbilityTree) 100)
  (for _array_element (Variables|Default|GetUnlockedSkills)
    (if (Utilities|Enum|NotEqual(Enum) (.Elemental (Utilities|Struct|BreakS_NPCSkills _array_element)) "NewEnumerator3")
      (Default|UnlockElemental (Variables|Default|GetAC_AbilityTree) (.Elemental (Utilities|Struct|BreakS_NPCSkills _array_element))))
    (for _array_element_2 (.Skills (Utilities|Struct|BreakS_NPCSkills _array_element))
      (Default|UnlockNode (Variables|Default|GetAC_AbilityTree) _array_element_2)
      (CallFunction|SwitchElemental true)
      (CallFunction|SwitchWeaponSystem true)))
  (CallFunction|SwitchElemental true)
  (CallFunction|SwitchWeaponSystem true))

(event EventKillCharacter
  ;[0 0 0 0.5] Notify The Game That The Given Enemy Died
  (if (Variables|Default|GetIsAlive)
    (|CallParentFunction)
    (Collision|SetCollisionEnabled (Variables|Default|GetVisibleMesh) "NoCollision")
    (Default|CallDied)
    (Default|CallEnemyKilled (Variables|/Game/Shota/Blueprints/Game/GI_Custom.GI_Custom_C|GetWorldEventsActor (CallFunction|FLGetGameInstance)) self)))

(fn ConstructionScript
  (|CallParentFunction))

(fn GetFacingDirection
  (bind _returnvalue (Transformation|GetActorLocation))
  (return _returnvalue (Math|Vector|GetForwardVector (Math|Rotator|FindLookatRotation _returnvalue (+ (Transformation|GetActorLocation (Variables|/Game/Shota/Blueprints/NPCs/CombatNPC_Controller.CombatNPC_Controller_C|GetTargetedEnemy (Variables|Default|GetNPCController))) "0.000000,0.000000,50.000000")))))

(fn GetActiveSkeleton
  (return (Variables|Default|GetVisibleMesh)))

(fn GetAttachSkeleton
  (return (Variables|Default|GetVisibleMesh)))

(fn FAllytoPlayer
  (return (Variables|/Game/Shota/Blueprints/NPCs/CombatNPC_Controller.CombatNPC_Controller_C|GetAllyToPlayer (Variables|Default|GetNPCController))))

(fn FRandomAbilityIndex
  (for _array_element (Variables|Default|GetAbilities)
    (LocalVariables|SetTotalWeights (+ (LocalVariables|GetTotalWeights) (.Weight (Utilities|Struct|BreakS_NPCAbilityData _array_element)))))
  (LocalVariables|SetRandomFloat (Math|Random|RandomFloatinRange 0.0 (LocalVariables|GetTotalWeights)))
  (for (_array_element_2 _array_index) (Variables|Default|GetAbilities)
    (bind _output_get (LocalVariables|SetAcc (+ (LocalVariables|GetAcc) (.Weight (Utilities|Struct|BreakS_NPCAbilityData _array_element_2)))))
    (if (>= _output_get (LocalVariables|GetRandomFloat))
      (return _array_index)))
  (return (Utilities|Array|LastIndex (Variables|Default|GetAbilities))))