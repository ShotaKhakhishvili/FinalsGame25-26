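; Orc bowman NPC that configures a parent NPC class as a bow-wielding enemy variant with its own stats and elemental type.
; On parameter initialization it sets health, mana and element, registers the bow component as its only weapon system and switches to it.
; It also picks one of three armor skin materials at random for the visible mesh, so individual bowmen vary in look.
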(event EventInitParams
  ;[0.15 0.15 0.15 0.5] Initialize Parameters
  (CallFunction|UpdateStats 3e+01 1e+02 0.0 "NewEnumerator3")
  (Variables|Default|SetWeaponSystems (Utilities|Array|MakeArray (Variables|Default|GetAC_BowSystem)))
  (CallFunction|SwitchWeaponSystem true)
  (Rendering|Material|SetMaterial (Variables|Default|GetVisibleMesh) 0 (Utilities|Select :Index (Math|Random|RandomInteger 3) :Option%200 "/Game/Saba/Meshes/Orc_2/Materials/Skin_1/M_Armor_Skin_1.M_Armor_Skin_1" :Option%201 "/Game/Saba/Meshes/Orc_2/Materials/Skin_2/M_Armor_Skin_2.M_Armor_Skin_2" :Option%202 "/Game/Saba/Meshes/Orc_2/Materials/Skin_3/M_Armor_Skin_3.M_Armor_Skin_3")))

(fn ConstructionScript
  (|CallParentFunction))