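; Bull NPC Blueprint: a sword-wielding, damage-resistant character built on a parent NPC class.
; InitParams seeds health, mana and element, then registers the sword system as its only weapon and force-switches to it.
; The UpdateStats override scales negative health changes to a tenth before calling the parent, giving roughly tenfold effective health, and prints current HP.
; GetActiveSkeleton returns VisibleMesh as the active skeleton.
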(event EventUpdateStats
  (params (Hp :type Float%20%28double-precision%29) (Mana :type Float%20%28double-precision%29) (Xp :type Float%20%28double-precision%29) (Elemental :type E_ElementalType%20Enum :default "NewEnumerator0"))
  ;[0.15 0.15 0.15 0.5] Add damage resistance (1000 hp)
  (|CallParentFunction (Utilities|ScaleNegativeValue Hp 0.1) Mana Xp Elemental)
  (Development|PrintString (Utilities|String|ToString(Float) (Variables|/Game/Saba/Blueprints/Components/StatsSystem/AC_StatsSystem.AC_StatsSystem_C|GetHp (Variables|Default|GetAC_StatsSystem)))))

(event EventInitParams
  ;[0.15 0.15 0.15 0.5] Initialize Parameters
  (CallFunction|UpdateStats 1e+02 1e+02 0.0 "NewEnumerator3")
  (Variables|Default|SetWeaponSystems (Utilities|Array|MakeArray (Variables|Default|GetAC_SwordSystem)))
  (CallFunction|SwitchWeaponSystem true true))

(fn ConstructionScript
  (|CallParentFunction))

(fn GetActiveSkeleton
  (return (Variables|Default|GetVisibleMesh)))