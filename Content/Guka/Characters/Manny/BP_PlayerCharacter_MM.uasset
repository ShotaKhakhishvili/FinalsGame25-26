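; Player character Blueprint that adds dash, roll, slide, crouch and vault/climb traversal to its parent, using Enhanced Input.
; ShouldCheck gates actions on state flags; dash and roll pick directional montages from movement input angle.
; Jump launches out of slides or tries Vault, whose line traces choose climb, mantle or vault by wall height and thickness.
; Vaults run in Flying mode without capsule collision, and a sphere trace guards uncrouching.
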(event Custom|ToggleCrouch
  ;[0.15 0.15 0.15 0.5] Crouch State
  (bind _result (CallFunction|CanMove))
  (if _result
    (if (or (Variables|Default|GetForcedCrouchFallback%20) (Variables|Default|GetIsCrouched))
      (bind _canuncrouch (CallFunction|CanUncrouch))
      (if _canuncrouch
        (Character|UnCrouch)
        (Variables|Default|SetForcedCrouchFallback%20 false)
        (Variables|Default|SetIsCrouched false))
      (else
        (bind _result_2 (CallFunction|ShouldCheck false true true false true false true true))
        (if _result_2
          (Character|Crouch)
          (Variables|Default|SetIsCrouched true))))))

(event Input|EnhancedActionEvents|EnhancedInputActionIA_Crouch
  (params (ActionValue :type Boolean) (ElapsedSeconds :type Float%20%28double-precision%29) (TriggeredSeconds :type Float%20%28double-precision%29) (InputAction :type Input%20Action%20Object%20Reference :default "/Game/Guka/Input/IA_Crouch.IA_Crouch"))
  ;[0.15 0.15 0.15 0.5] Crouch State
  (:Started
    (CallFunction|ToggleCrouch)))

(event Input|EnhancedActionEvents|EnhancedInputActionIA_Slide
  (params (ActionValue :type Boolean) (ElapsedSeconds :type Float%20%28double-precision%29) (TriggeredSeconds :type Float%20%28double-precision%29) (InputAction :type Input%20Action%20Object%20Reference :default "/Game/Guka/Input/IA_Slide.IA_Slide"))
  ;[0.15 0.15 0.15 0.5] Traversal Abilities
  ;;[0.15 0.15 0.15 0.5] Slide
  (:Started
    (bind _result (CallFunction|ShouldCheck true true true true true true true true))
    (if (and _result (Variables|Default|GetCanSlide))
      (CallFunction|ToggleCrouch)
      (Variables|Default|SetIsSliding true)
      (Variables|Default|SetCanSlide false)
      (Animation|Montage|PlayMontage (Variables|Character|GetMesh) "/Game/Guka/Animation/Slide/Montages/UEFNManny_threepeat_runningslide_v4_moreRealistic_Montage.UEFNManny_threepeat_runningslide_v4_moreRealistic_Montage"
        (:OnBlendOut
          _)
        (:OnInterrupted
          _))
      (CallFunction|ToggleCrouch)
      (Variables|Default|SetIsSliding false)
      (Utilities|FlowControl|Delay (Variables|Default|GetSlideCooldown))
      (Variables|Default|SetCanSlide true))))

(event Input|EnhancedActionEvents|EnhancedInputActionIA_Dash
  (params (ActionValue :type Boolean) (ElapsedSeconds :type Float%20%28double-precision%29) (TriggeredSeconds :type Float%20%28double-precision%29) (InputAction :type Input%20Action%20Object%20Reference :default "/Game/Guka/Input/IA_Dash.IA_Dash"))
  ;[0.15 0.15 0.15 0.5] Traversal Abilities
  ;;[0.15 0.15 0.15 0.5] Dash
  (:Started
    (bind _result (CallFunction|ShouldCheck true true true true true true true true))
    (if (and _result (not (Variables|Default|GetDashOnCooldown)))
      (CallFunction|AimEnd)
      (Variables|Default|SetIsDashing true)
      (Variables|Default|SetDashOnCooldown true)
      (bind (_angle _direction) (CallFunction|GetActorDirectionAngle (Transformation|GetActorForwardVector)))
      (Character|LaunchCharacter (* (Variables|Default|GetDashStrength) _direction) true false)
      (bind _direction_2 (CallFunction|GetDashDirectionfromAngle _angle))
      (Animation|Montage|PlayMontage (Variables|Character|GetMesh) (.Value (Utilities|Map|Find (Variables|Default|GetDashMontages) _direction_2))
        (:then
          (Components|Activation|SetActive (Variables|Default|GetDashEffect) true true)
          (Utilities|FlowControl|Delay (Variables|Default|GetDashDuration))
          (Components|Activation|SetActive (Variables|Default|GetDashEffect) false false)
          (Variables|Default|SetIsDashing false)
          (Utilities|FlowControl|Delay (Variables|Default|GetDashCooldownTime))
          (Variables|Default|SetDashOnCooldown false))))))

(event Input|EnhancedActionEvents|EnhancedInputActionIA_Roll
  (params (ActionValue :type Boolean) (ElapsedSeconds :type Float%20%28double-precision%29) (TriggeredSeconds :type Float%20%28double-precision%29) (InputAction :type Input%20Action%20Object%20Reference :default "/Game/Guka/Input/IA_Roll.IA_Roll"))
  ;[0.15 0.15 0.15 0.5] Traversal Abilities
  ;;[0.15 0.15 0.15 0.5] Roll
  (:Started
    (bind _result (CallFunction|ShouldCheck true true true true true true true true))
    (if _result
      (CallFunction|ToggleCrouch)
      (Variables|Default|SetIsRolling true)
      (bind _angle (CallFunction|GetActorDirectionAngle (Math|Vector|NegateVector (Transformation|GetActorForwardVector))))
      (bind _direction (CallFunction|GetRollDirectionfromAngle _angle))
      (Animation|Montage|PlayMontage (Variables|Character|GetMesh) (.Value (Utilities|Map|Find (Variables|Default|GetRollMontages) _direction)) 1.5
        (:OnBlendOut
          _)
        (:OnInterrupted
          _))
      (CallFunction|ToggleCrouch)
      (Variables|Default|SetIsRolling false))))

(event EventBeginPlay
  (bind _returnvalue (Game|GetPlayerCameraManager 0))
  ;[0.15 0.15 0.15 0.5] Begin Play
  (|CallParentFunction)
  ;;[0.15 0.15 0.15 0.5] Caching standing half height
  (Variables|Default|SetStandingHalfHeight (Components|Capsule|GetUnscaledCapsuleHalfHeight (Variables|Default|GetCapsuleComponent)))
  ;;[0.15 0.15 0.15 0.5] Camera Pitch
  (Variables|/Script/Engine.PlayerCameraManager|SetViewPitchMax _returnvalue 75.0)
  (Variables|/Script/Engine.PlayerCameraManager|SetViewPitchMin _returnvalue -75.0)
  (bind _asplayer_controller (Utilities|Casting|CastToPlayerController (Pawn|GetController)))
  (Utilities|IsValid (PlayerController|LocalPlayerSubsystems|GetEnhancedInputLocalPlayerSubsystem _asplayer_controller)
    (:Is%20Valid
      (Input|AddMappingContext (PlayerController|LocalPlayerSubsystems|GetEnhancedInputLocalPlayerSubsystem _asplayer_controller) "/Game/Guka/Input/IMC_Player.IMC_Player" 1 "(bIgnoreAllPressedKeysUntilRelease=True,bForceImmediately=False,bNotifyUserSettings=False)"))))

(event EventSprintStart
  ;[0.15 0.15 0.15 0.5] Sprint State
  (if (Variables|Default|GetIsCrouched)
    (CallFunction|ToggleCrouch)
    (if (not (Variables|Default|GetIsCrouched))
      (|CallParentFunction :!label _label))
    (else
      (goto _label))))

(event EventJumpStart
  ;[0.15 0.15 0.15 0.5] Jump/Vault
  (if (Variables|Default|GetIsSliding)
    (bind _canuncrouch (CallFunction|CanUncrouch))
    (if _canuncrouch
      (Character|LaunchCharacter (+ (* (Transformation|GetActorForwardVector) (Math|Float|Clamp(Float) (* (Math|Vector|VectorLength (Variables|/Script/Engine.MovementComponent|GetVelocity (Variables|Character|GetCharacterMovement))) 0.6) 2.5e+02 4.4e+02)) "0.000000,0.000000,850.000000") true true)
      (|CallParentFunction))
    (else
      ;;[0.15 0.15 0.15 0.5] Vault
      (bind _result (CallFunction|ShouldCheck true true true true false false false true))
      (if _result
        (Utilities|Vault
          (:NotVaulted
            (if (not (Variables|Default|GetIsRolling))
              (|CallParentFunction))))))))

(fn ConstructionScript
  (|CallParentFunction))

(fn GetActorDirectionAngle
  (params (DefaultDirection :type Vector))
  (bind _returnvalue (Class|Pawn|GetLastMovementInputVector))
  (bind _returnvalue_2 (Math|Vector|VectorLength _returnvalue))
  (bind _returnvalue_3 (Math|Vector|Normalize _returnvalue))
  (bind _returnvalue_4 (> _returnvalue_2 0.1))
  (bind _returnvalue_5 (select _returnvalue_4 _returnvalue_3 DefaultDirection))
  (return (Class|KismetMathLibrary|DegAtan2 (Math|Vector|DotProduct (Transformation|GetActorRightVector) _returnvalue_5) (Math|Vector|DotProduct (Transformation|GetActorForwardVector) _returnvalue_5)) _returnvalue_5))

(fn GetDashDirectionfromAngle
  (params (Angle :type Float%20%28double-precision%29))
  (if (and (>= Angle -22.5) (< Angle 22.5))
    (return "NewEnumerator0")
    (elif (and (>= Angle 22.5) (< Angle 67.5))
      (return "NewEnumerator1")
      (elif (and (>= Angle 67.5) (< Angle 112.5))
        (return "NewEnumerator2")
        (elif (and (>= Angle 112.5) (< Angle 157.5))
          (return "NewEnumerator3")
          (elif (or (>= Angle 157.5) (< Angle -157.5))
            (return "NewEnumerator4")
            (elif (and (>= Angle -157.5) (< Angle -112.5))
              (return "NewEnumerator5")
              (elif (and (>= Angle -112.5) (< Angle -67.5))
                (return "NewEnumerator6")
                (else
                  (return "NewEnumerator7"))))))))))

(fn GetRollDirectionfromAngle
  (params (Angle :type Float%20%28double-precision%29))
  (if (and (>= Angle -46.0) (< Angle 46.0))
    (return "NewEnumerator0")
    (elif (and (>= Angle 46.0) (< Angle 134.0))
      (return "NewEnumerator2")
      (elif (or (>= Angle 134.0) (< Angle -134.0))
        (return "NewEnumerator4")
        (else
          (return "NewEnumerator6"))))))

(fn CanUncrouch
  (bind _returnvalue (Transformation|GetActorLocation))
  (bind _charactermovement (Variables|Character|GetCharacterMovement))
  (bind _crouchedhalfheight (Variables|/Script/Engine.CharacterMovementComponent|GetCrouchedHalfHeight _charactermovement))
  (bind _returnvalue_2 (+ _returnvalue (Math|Vector|MakeVector 0.0 0.0 _crouchedhalfheight)))
  (bind _returnvalue_3 (Collision|MultiSphereTraceByChannel _returnvalue_2 (+ _returnvalue_2 (Math|Vector|MakeVector 0.0 0.0 (- (Variables|Default|GetStandingHalfHeight) _crouchedhalfheight))) 34.0 "TraceTypeQuery1" false 0 "ForDuration"))
  (if (not _returnvalue_3)
    (return true)
    (else
      (return false))))

(fn ShouldCheck
  (params (Dashing :type Boolean) (Sliding :type Boolean) (Rolling :type Boolean) (Crouched :type Boolean) (Vaulting :type Boolean) (Forced%20Crouch :type Boolean) (Falling :type Boolean) (Moving :type Boolean))
  (LocalVariables|SetFinalResult true)
  (Utilities|FlowControl|Sequence
    (:then_0
      (if Dashing
        (LocalVariables|SetFinalResult (and (not (Variables|Default|GetIsDashing)) (LocalVariables|GetFinalResult)))))
    (:then_1
      (if Sliding
        (LocalVariables|SetFinalResult (and (not (Variables|Default|GetIsSliding)) (LocalVariables|GetFinalResult)))))
    (:then_2
      (if Rolling
        (LocalVariables|SetFinalResult (and (not (Variables|Default|GetIsRolling)) (LocalVariables|GetFinalResult)))))
    (:then_3
      (if Crouched
        (LocalVariables|SetFinalResult (and (not (Variables|Default|GetIsCrouched)) (LocalVariables|GetFinalResult)))))
    (:then_4
      (if Vaulting
        (LocalVariables|SetFinalResult (and (not (Variables|Default|GetIsVaulting)) (LocalVariables|GetFinalResult)))))
    (:then_5
      (if Forced%20Crouch
        (LocalVariables|SetFinalResult (and (not (Variables|Default|GetForcedCrouchFallback%20)) (LocalVariables|GetFinalResult)))))
    (:then_6
      (if Falling
        (LocalVariables|SetFinalResult (and (not (AI|Components|NavMovement|IsFalling (Variables|Character|GetCharacterMovement))) (LocalVariables|GetFinalResult)))))
    (:then_7
      (if Moving
        (bind _result (CallFunction|CanMove))
        (LocalVariables|SetFinalResult (and _result (LocalVariables|GetFinalResult)))))
    (:then_8
      (return (LocalVariables|GetFinalResult)))))

(fn CanSwitchSetting
  (bind _result (CallFunction|ShouldCheck true true true false true false false false))
  (bind (_ability _elemental _weapon _attack) (|CallParentFunction))
  (return _ability _elemental _weapon (and _attack _result)))

(fn CanMove
  (bind _result (|CallParentFunction))
  (return (and _result (not (Variables|Default|GetIsVaulting)))))